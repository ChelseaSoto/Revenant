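; Save data container that holds the player's quest log, collected items and four ability unlock states.
; Quest stage and objective progress are stored in a map by quest ID, and loading re-adds each active quest to the quest log and restores those values.
; Collectables are recorded by ID for lookup, alongside a running count.
; Clearing empties quest and collected-ID data but leaves the count and ability unlocks untouched.
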(event EventAddCollectable
  (params (Collected%20Actor :type BP%20Collectable%20Base%20Object%20Reference))
  (Utilities|Array|Add (Variables|Collectables|GetIDs%20Collected) (Variables|/Game/Blueprints/GameSystems/Collectables/BP_CollectableBase.BP_CollectableBase_C|GetCollectableID Collected%20Actor))
  (Math|Integer|IncrementInt (Variables|Collectables|GetCollectable%20Amount)
    (:%20%20
      (Development|PrintString 0 "adding!!"))))

(event EventReturnAllCollected
  (CallFunction|ReturnCollectables))

(fn SaveQuestDetails
  (params (Quest :type BP%20Quest%20Base%20Object%20Reference))
  (Utilities|Map|Add (Variables|Quest|GetQuestProgress) (Variables|/Game/Blueprints/GameSystems/QuestSystems/BP_QuestBase.BP_QuestBase_C|GetQuestID Quest) (Utilities|Struct|MakeST_QuestSaveData (Variables|/Game/Blueprints/GameSystems/QuestSystems/BP_QuestBase.BP_QuestBase_C|GetCurrentObjectiveProgress Quest) (Variables|/Game/Blueprints/GameSystems/QuestSystems/BP_QuestBase.BP_QuestBase_C|GetCurrentStage Quest))))

(fn LoadQuests
  (params (Quest%20Log :type BPC%20Quest%20Log%20Component%20Object%20Reference))
  (for _array_element (Variables|Quest|GetCurrentActiveQuests)
    (bind _returnvalue (Default|AddNewQuest Quest%20Log _array_element))
    (Variables|/Game/Blueprints/GameSystems/QuestSystems/BP_QuestBase.BP_QuestBase_C|SetCurrentObjectiveProgress _returnvalue (.Progress (Utilities|Struct|BreakST_QuestSaveData (.Value (Utilities|Map|Find (Variables|Quest|GetQuestProgress) _array_element)))))
    (Variables|/Game/Blueprints/GameSystems/QuestSystems/BP_QuestBase.BP_QuestBase_C|SetCurrentStage _returnvalue (.CurrentStage (Utilities|Struct|BreakST_QuestSaveData (.Value (Utilities|Map|Find (Variables|Quest|GetQuestProgress) _array_element))))))
  (Variables|/Game/Blueprints/GameSystems/QuestSystems/BPC_QuestLogComponent.BPC_QuestLogComponent_C|SetCurrentActiveQuests Quest%20Log (Variables|Quest|GetCurrentActiveQuests))
  (Variables|/Game/Blueprints/GameSystems/QuestSystems/BPC_QuestLogComponent.BPC_QuestLogComponent_C|SetCompletedQuests Quest%20Log (Variables|Quest|GetCompletedQuests)))

(fn SaveQuestLog
  (params (QuestLog :type BPC%20Quest%20Log%20Component%20Object%20Reference))
  (Variables|Quest|SetCurrentActiveQuests (Variables|/Game/Blueprints/GameSystems/QuestSystems/BPC_QuestLogComponent.BPC_QuestLogComponent_C|GetCurrentActiveQuests QuestLog))
  (Variables|Quest|SetCompletedQuests (Variables|/Game/Blueprints/GameSystems/QuestSystems/BPC_QuestLogComponent.BPC_QuestLogComponent_C|GetCompletedQuests QuestLog)))

(fn ChangeAbilityDetails
  (params (Ability1 :type Boolean) (Ability2 :type Boolean) (Ability3 :type Boolean) (Ability4 :type Boolean))
  (Variables|Ability|SetAbilityUnlocked_1 Ability1)
  (Variables|Ability|SetAbilityUnlocked_2 Ability2)
  (Variables|Ability|SetAbilityUnlocked_3 Ability3)
  (Variables|Ability|SetAbilityUnlocked_4 Ability4))

(fn ClearSaveData
  (Utilities|Array|Clear (Variables|Quest|GetCurrentActiveQuests))
  (Utilities|Array|Clear (Variables|Quest|GetCompletedQuests))
  (Utilities|Map|Clear (Variables|Quest|GetQuestProgress))
  (Utilities|Array|Clear (Variables|Collectables|GetIDs%20Collected)))

(fn ReturnCollectables
  (return (Variables|Collectables|GetIDs%20Collected)))

(fn CheckCollectables
  (params (Actor :type BP%20Collectable%20Base%20Object%20Reference))
  (return (Utilities|Array|ContainsItem (Variables|Collectables|GetIDs%20Collected) (Variables|/Game/Blueprints/GameSystems/Collectables/BP_CollectableBase.BP_CollectableBase_C|GetCollectableID Actor))))