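; B_RollingBall is a rolling-ball trap that releases a physics sphere when the player enters its activation trigger.
; The trigger enables gravity on the sphere, whose starting transform is cached at BeginPlay.
; When the HitSphere overlaps the player, after a short delay it damages the character and teleports them to a safe position.
; It then zeroes the ball's velocity, disables gravity and teleports it back to its start, re-arming the trap.
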(event OnComponentBeginOverlap(ActivationTrigger)
  (params (OverlappedComponent :type Primitive%20Component%20Object%20Reference) (OtherActor :type Actor%20Object%20Reference) (OtherComp :type Primitive%20Component%20Object%20Reference) (OtherBodyIndex :type Integer) (bFromSweep :type Boolean) (SweepResult :type Hit%20Result%20Structure%20%28by%20ref%29))
  ;[1 1 1] When player overlaps with activation trigger enable gravity on the ball
  (if (== OtherActor (Game|Player|GetPlayerPawn 0))
    (Physics|SetEnableGravity (Variables|Default|GetSphere) true)
    (Development|PrintString "ball rolling!" true true "(R=1.000000,G=0.000000,B=0.016322,A=1.000000)")))

(event OnComponentBeginOverlap(HitSphere)
  (params (OverlappedComponent :type Primitive%20Component%20Object%20Reference) (OtherActor :type Actor%20Object%20Reference) (OtherComp :type Primitive%20Component%20Object%20Reference) (OtherBodyIndex :type Integer) (bFromSweep :type Boolean) (SweepResult :type Hit%20Result%20Structure%20%28by%20ref%29))
  (bind _sphere (Variables|Default|GetSphere))
  ;[1 1 1] If player overlaps ball's collider call the player's ragdoll event
  (if (== OtherActor (Game|Player|GetPlayerPawn 0))
    (Utilities|Casting|CastToBP_ThirdPersonCharacter OtherActor)
    (Utilities|FlowControl|Delay 0.2)
    (bind _asbp_third_person_character (Utilities|Casting|CastToBP_ThirdPersonCharacter OtherActor))
    (Default|PlayerTakeDamage _asbp_third_person_character (Variables|Default|GetDamage))
    (Default|TeleporttoSafePos _asbp_third_person_character)
    ;;[1 1 1] this is overengineered just add 3 walls
    (Class|PrimitiveComponent|SetAllPhysicsLinearVelocity _sphere "0, 0, 0" false)
    (Physics|SetEnableGravity _sphere false)
    (Transformation|SetWorldTransform _sphere (Variables|Default|GetStartingPosition) false true)))

(event EventBeginPlay
  ;[1 1 1] Ball origin point
  (Variables|Default|SetStartingPosition (Transformation|GetWorldTransform (Variables|Default|GetSphere))))

(fn ConstructionScript)