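; Spike pit trap that rises once when the player enters its activation trigger and sends the player back to a safe position on contact.
; A one-shot gate starts a timeline that lerps the whole actor upward from its BeginPlay transform.
; The hitbox calls TeleportToSafePos on the third-person character after a short delay, standing in for a ragdoll death that is not connected.
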(event OnComponentBeginOverlap(HitBox)
  (params (OverlappedComponent :type Primitive%20Component%20Object%20Reference) (OtherActor :type Actor%20Object%20Reference) (OtherComp :type Primitive%20Component%20Object%20Reference) (OtherBodyIndex :type Integer) (bFromSweep :type Boolean) (SweepResult :type Hit%20Result%20Structure%20%28by%20ref%29))
  ;[1 1 1] If player overlaps with the spike call the player's ragdoll event (currently no ragdoll, just teleport player to spawn point)
  (if (== OtherActor (Game|Player|GetPlayerPawn 0))
    (Utilities|Casting|CastToBP_ThirdPersonCharacter OtherActor)
    (Development|PrintString "Player hit a spike" true true "(R=1.000000,G=0.041135,B=0.000000,A=1.000000)" 5.0)
    (Utilities|FlowControl|Delay 0.2)
    (bind _asbp_third_person_character (Utilities|Casting|CastToBP_ThirdPersonCharacter OtherActor))
    (Default|TeleporttoSafePos _asbp_third_person_character)
    (else
      (Development|PrintString "non-player overlapping a spike" true true "(R=1.000000,G=0.000000,B=0.976581,A=1.000000)" 5.0))))

(event OnComponentBeginOverlap(ActivationTrigger)
  (params (OverlappedComponent :type Primitive%20Component%20Object%20Reference) (OtherActor :type Actor%20Object%20Reference) (OtherComp :type Primitive%20Component%20Object%20Reference) (OtherBodyIndex :type Integer) (bFromSweep :type Boolean) (SweepResult :type Hit%20Result%20Structure%20%28by%20ref%29))
  ;[1 1 1] If player overlaps trigger begin raising spike
  (if (== OtherActor (Game|Player|GetPlayerPawn 0))
    (Utilities|FlowControl|DoOnce false
      (:Completed
        (CallFunction|RaiseSpike)
        (Development|PrintString "Spike raising")))))

(event Custom|Raise%20Spike
  (bind _starttransform (Variables|Default|GetStartTransform))
  (bind _starttransform_2 (Variables|Default|GetStartTransform))
  ;[1 1 1] Raises spike on the Z-axis over 5 seconds while maintaining scale / rotation
  (bind _spikeraisetimeline (Timeline|Spike%20Raise%20Timeline Play)
    (:Update
      (Transformation|SetActorTransform (Math|Transform|MakeTransform (Math|Vector|Lerp(Vector) (.location _starttransform) (Math|Vector|MakeVector (.x (.location _starttransform_2)) (.y (.location _starttransform_2)) (+ (.z (.location _starttransform_2)) 1.5e+02)) _spikeraisetimeline) (.rotation _starttransform) (.scale _starttransform))))))

(event EventBeginPlay
  ;[1 1 1] Get the starting transform of the spike
  (Variables|Default|SetStartTransform (Transformation|GetActorTransform)))

(fn ConstructionScript)