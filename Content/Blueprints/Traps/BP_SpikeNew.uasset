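; BP_SpikeNew is a spike trap that hurts the player on contact and returns them to their last safe position.
; When the player pawn overlaps its HitBox, it ragdolls the third-person character, waits briefly, then applies its Damage value.
; If the player survives, it teleports them to the safe position and ends the ragdoll; if health is depleted, it does neither.
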(event OnComponentBeginOverlap(HitBox)
  (params (OverlappedComponent :type Primitive%20Component%20Object%20Reference) (OtherActor :type Actor%20Object%20Reference) (OtherComp :type Primitive%20Component%20Object%20Reference) (OtherBodyIndex :type Integer) (bFromSweep :type Boolean) (SweepResult :type Hit%20Result%20Structure%20%28by%20ref%29))
  ;[1 1 1] If player overlaps with the spike, deal damage to the player and teleport them to last safe point
  (if (== OtherActor (Game|Player|GetPlayerPawn 0))
    (bind _asbp_third_person_character (Utilities|Casting|CastToBP_ThirdPersonCharacter OtherActor))
    (Default|Ragdoll _asbp_third_person_character)
    (Utilities|FlowControl|Delay 1.0)
    (Default|PlayerTakeDamage _asbp_third_person_character (Variables|Default|GetDamage))
    (if (not (<= (Variables|/Game/ThirdPerson/Blueprints/BP_ThirdPersonCharacter.BP_ThirdPersonCharacter_C|GetHealth _asbp_third_person_character) 0.0))
      (Default|TeleporttoSafePos _asbp_third_person_character)
      (Default|UnRagdoll _asbp_third_person_character))))

(fn ConstructionScript)