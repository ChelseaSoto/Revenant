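; BP_AmbientSound is a placeable ambient sound trigger that plays audio when overlap begins on its radius sphere.
; Its construction script picks a random sound, applies attenuation and sets the sphere radius.
; AlwaysPlay plays on any overlap; otherwise only the player can trigger it, with a chance that grows after each failed attempt and resets on playback.
; Any end overlap fades the sound out.
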(event OnComponentBeginOverlap(SoundRadius)
  (params (OverlappedComponent :type Primitive%20Component%20Object%20Reference) (OtherActor :type Actor%20Object%20Reference) (OtherComp :type Primitive%20Component%20Object%20Reference) (OtherBodyIndex :type Integer) (bFromSweep :type Boolean) (SweepResult :type Hit%20Result%20Structure%20%28by%20ref%29))
  (if (Variables|Default|GetAlwaysPlay?)
    (Audio|Components|Audio|Play (Variables|Default|GetAmbientSound) 0.0 :!label _label)
    (Variables|Default|SetPlayChance 0.2)
    (elif (and (== OtherActor (Game|Player|GetPlayerPawn 0)) (Math|Random|RandomBoolwithWeight (Variables|Default|GetPlayChance)))
      (goto _label)
      (else
        (Variables|Default|SetPlayChance (+ (Variables|Default|GetPlayChance) 0.1))))))

(event OnComponentEndOverlap(SoundRadius)
  (params (OverlappedComponent :type Primitive%20Component%20Object%20Reference) (OtherActor :type Actor%20Object%20Reference) (OtherComp :type Primitive%20Component%20Object%20Reference) (OtherBodyIndex :type Integer))
  (if true
    (Audio|Components|Audio|FadeOut (Variables|Default|GetAmbientSound) 1.0 0.0 "Linear" :!class /Script/Engine.AudioComponent)))

(fn ConstructionScript
  (Audio|Components|Audio|SetSound (Variables|Default|GetAmbientSound) (.OutItem (Utilities|Array|Random (Variables|Default|GetSound))))
  (Variables|/Script/Engine.AudioComponent|SetAttenuationSettings (Variables|Default|GetAmbientSound) (Variables|Default|GetAmbiendSoundAttenuation))
  (Components|Sphere|SetSphereRadius (Variables|Default|GetSoundRadius) (Math|Conversions|ToFloat(Integer) (Variables|Default|GetSphereRad)) true))