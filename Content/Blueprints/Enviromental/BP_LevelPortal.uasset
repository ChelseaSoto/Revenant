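; Level portal actor that sends the player to another level when they overlap its trigger while it is active.
; Construction script copies target level, fade duration and quest data into a child BP_LevelTransitions actor, which handles the transition and mission.
; Activate gives the mission, starts VFX, light and aura sound.
; Deactivate clears the flag, but re-calls VFX Activate after a delay; both light interpolations are single-step, not ticked.
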(event OnComponentBeginOverlap(Trigger)
  (params (OverlappedComponent :type Primitive%20Component%20Object%20Reference) (OtherActor :type Actor%20Object%20Reference) (OtherComp :type Primitive%20Component%20Object%20Reference) (OtherBodyIndex :type Integer) (bFromSweep :type Boolean) (SweepResult :type Hit%20Result%20Structure%20%28by%20ref%29))
  (if (and (== OtherActor (Game|Player|GetPlayerPawn 0)) (Variables|Default|GetisActive?))
    (Default|LevelTransition (Variables|Default|GetAs%20BP%20Level%20Transitions))))

(event Custom|Activate
  (Default|GiveMission (Variables|Default|GetAs%20BP%20Level%20Transitions))
  (Variables|Default|SetisActive? true)
  (Components|Activation|Activate (Variables|Default|GetPortalVFX) false)
  (Rendering|Components|Light|SetIntensity (Variables|Default|GetPointLight) (Math|Interpolation|FInterpTo 0.0 0.5 (Utilities|Time|GetWorldDeltaSeconds) 1.0))
  (Audio|SpawnSoundatLocation "/Game/Audio/SFX/WorldSFX/SQ_Aura.SQ_Aura" (Transformation|GetActorLocation) "0, 0, 0" 1.0 1.0 0.0 0 0))

(event Custom|Deactivate
  (Variables|Default|SetisActive? false)
  (Rendering|Components|Light|SetIntensity (Variables|Default|GetPointLight) (Math|Interpolation|FInterpTo 0.5 0.0 (Utilities|Time|GetWorldDeltaSeconds) 0.2))
  (Utilities|FlowControl|Delay 5.0)
  (Components|Activation|Activate (Variables|Default|GetPortalVFX) false))

(event EventBeginPlay)

(fn ConstructionScript
  (bind _asbp_level_transitions (Utilities|Casting|CastToBP_LevelTransitions (Variables|/Script/Engine.ChildActorComponent|GetChildActor (Variables|Default|GetLevelTransition))))
  (bind _output_get (Variables|Default|SetAs%20BP%20Level%20Transitions _asbp_level_transitions))
  (Variables|/Game/Blueprints/Interactables/BP_LevelTransitions.BP_LevelTransitions_C|SetLevel%20To%20Transition%20To _output_get (Variables|Default|GetLevel%20to%20Transition%20To))
  (Variables|/Game/Blueprints/Interactables/BP_LevelTransitions.BP_LevelTransitions_C|SetDuration _output_get (Variables|Default|GetFade%20Duration))
  (Variables|/Game/Blueprints/GameSystems/QuestSystems/BPC_QuestGiver.BPC_QuestGiver_C|SetQuestData (Variables|/Game/Blueprints/Interactables/BP_LevelTransitions.BP_LevelTransitions_C|GetBPC_QuestGiver _output_get) (Utilities|Struct|MakeDataTableRowHandle (Variables|Default|GetQuest%20Data%20Data%20Table) (Variables|Default|GetQuest%20Data%20Row%20Name))))