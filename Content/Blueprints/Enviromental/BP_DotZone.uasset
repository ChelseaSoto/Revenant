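; BP_DotZone is a damage-over-time zone that hurts the player character while they overlap it.
; Entering starts a looping 0.75-second timer that subtracts Health directly, then triggers camera shake and the damage indicator.
; Damage scales with the tick count up to a clamp, so the first tick deals none.
; Leaving clears the timer and resets the ramp; ShouldTakeDamage is set but never read here.
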(event Custom|Deal%20Damage
  (Variables|/Game/ThirdPerson/Blueprints/BP_ThirdPersonCharacter.BP_ThirdPersonCharacter_C|SetHealth (stale EventBeginPlay _asbp_third_person_character) (- (Variables|/Game/ThirdPerson/Blueprints/BP_ThirdPersonCharacter.BP_ThirdPersonCharacter_C|GetHealth (stale EventBeginPlay _asbp_third_person_character)) (Math|Float|Clamp(Float) (* (Variables|Default|GetDamageToDeal) (Variables|Default|GetDamageTicksDone)) 0.0 15.0)))
  (Math|Integer|IncrementInt (Variables|Default|GetDamageTicksDone)
    (:%20%20
      (Default|CameraShake (stale EventBeginPlay _asbp_third_person_character) false)
      (Default|ShowDamageIndicator (stale EventBeginPlay _asbp_third_person_character)))))

(event Collision|EventActorBeginOverlap
  (params (OtherActor :type Actor%20Object%20Reference))
  (if (== OtherActor (Game|GetPlayerCharacter 0))
    (Variables|Default|SetShouldTakeDamage true)
    (bind _returnvalue (Utilities|Time|SetTimerbyEvent (delegate Custom|Deal%20Damage) 0.75 true))))

(event Collision|EventActorEndOverlap
  (params (OtherActor :type Actor%20Object%20Reference))
  (if (== (Game|GetPlayerCharacter 0) OtherActor)
    (Variables|Default|SetShouldTakeDamage false)
    (Variables|Default|SetDamageTicksDone 0)
    (Utilities|Time|ClearandInvalidateTimerbyHandle (stale Collision|EventActorBeginOverlap _returnvalue))))

(event EventBeginPlay
  (bind _asbp_third_person_character (Utilities|Casting|CastToBP_ThirdPersonCharacter (Game|GetPlayerCharacter 0))))

(fn ConstructionScript)