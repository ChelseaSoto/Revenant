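; JumpBoost is an environmental pad that launches the player forward and up when they run into it fast enough.
; BeginPlay caches the third-person player character, and the Box overlap fires LaunchPlayer only for that character moving above a speed threshold, effectively a sprint.
; LaunchPlayer sends the character along its own facing with a fixed lift and attaches a short-lived Niagara aura to its capsule.
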(event OnComponentBeginOverlap(Box)
  (params (OverlappedComponent :type Primitive%20Component%20Object%20Reference) (OtherActor :type Actor%20Object%20Reference) (OtherComp :type Primitive%20Component%20Object%20Reference) (OtherBodyIndex :type Integer) (bFromSweep :type Boolean) (SweepResult :type Hit%20Result%20Structure%20%28by%20ref%29))
  (bind _returnvalue (Game|GetPlayerCharacter 0))
  ;[1 1 1] Launch the player forward & up when they sprint into this
  (bind _output_get (Variables|Default|Setspeed (Math|Vector|VectorLength (Transformation|GetVelocity _returnvalue))))
  (if (and (> _output_get 4.5e+02) (== OtherActor _returnvalue))
    (CallFunction|LaunchPlayer)))

(event Custom|LaunchPlayer
  (bind _playerref (Variables|Default|GetPlayerRef))
  (bind _returnvalue (Transformation|GetActorForwardVector _playerref))
  ;[1 1 1] Launch the player forward & up when they sprint into this
  (Character|LaunchCharacter _playerref (Math|Vector|MakeVector (* (.x _returnvalue) 1.25e+03) (* (.y _returnvalue) 1.25e+03) 5e+02) false false)
  (bind _returnvalue_2 (Niagara|SpawnSystemAttached "/Game/VFX/Particles/ItemAura/NS_CampfireAura.NS_CampfireAura" (Variables|/Script/Engine.Character|GetCapsuleComponent _playerref) "None" "0, 0, 0" "0, 0, 0" "KeepRelativeOffset" false))
  (Utilities|FlowControl|Delay 0.85)
  (Components|DestroyComponent _returnvalue_2))

(event EventBeginPlay
  ;[1 1 1] Launch the player forward & up when they sprint into this
  (bind _asbp_third_person_character (Utilities|Casting|CastToBP_ThirdPersonCharacter (Game|GetPlayerCharacter 0)))
  (Variables|Default|SetPlayerRef _asbp_third_person_character))

(fn ConstructionScript)