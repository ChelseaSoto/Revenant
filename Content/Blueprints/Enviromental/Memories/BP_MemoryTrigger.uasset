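; BP_MemoryTrigger is a trigger volume that reveals a set of memory objects when the player enters it.
; On BeginPlay it hides every actor in its HiddenActors array and disables their collision.
; When the player character overlaps TriggerZone, it unhides those actors and restores their collision, with no logic to hide them again on exit.
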(event OnComponentBeginOverlap(TriggerZone)
  (params (OverlappedComponent :type Primitive%20Component%20Object%20Reference) (OtherActor :type Actor%20Object%20Reference) (OtherComp :type Primitive%20Component%20Object%20Reference) (OtherBodyIndex :type Integer) (bFromSweep :type Boolean) (SweepResult :type Hit%20Result%20Structure%20%28by%20ref%29))
  ;[1 1 1] When player enters trigger show all memory objects and enable their collision
  (if (== OtherActor (Game|GetPlayerCharacter 0))
    (for _array_element (Variables|Default|GetHiddenActors)
      (Rendering|SetActorHiddenInGame _array_element false)
      (Collision|SetActorEnableCollision _array_element true))))

(event EventBeginPlay
  ;[1 1 1] On start hide all objects in memory and disable their collision
  (for _array_element (Variables|Default|GetHiddenActors)
    (Rendering|SetActorHiddenInGame _array_element true)
    (Collision|SetActorEnableCollision _array_element false)))

(fn ConstructionScript)