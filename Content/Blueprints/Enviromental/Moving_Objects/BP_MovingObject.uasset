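; BP_MovingObject is an environmental actor that moves along the spline of a referenced PathToFollow.
; BeginPlay starts a timeline with play rate set from TimeToComplete, whose track maps to spline distance to update position and rotation, preserving scale.
; With DoesPingPong, looping is disabled and a FlipFlop alternates play and reverse each time the timeline finishes; otherwise the timeline simply plays.
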(event Custom|Move%20Object
  (bind _pathtofollow (Variables|Default|GetPathToFollow))
  (bind _spline (Variables|/Game/Blueprints/Enviromental/Moving_Objects/BP_SplinePath.BP_SplinePath_C|GetSpline _pathtofollow))
  ;[1 1 1] Sets the play rate of timeline //Omar
  (Components|Timeline|SetPlayRate (Variables|Default|GetMove%20Object%20T) (/ 1.0 (Variables|Default|GetTime%20To%20Complete)))
  ;[1 1 1] if it pingpongs then disable the loop //Omar
  (if (Variables|Default|Getdoes%20PingPong?)
    (Components|Timeline|SetLooping (Variables|Default|GetMove%20Object%20T) false)
    (Utilities|FlowControl|FlipFlop
      (:A
        (bind _move_track (Timeline|Move%20Object%20T Play)
          (:Update
            ;[1 1 1] Get split pos then do that for the object //Omar
            (Transformation|SetActorTransform (Math|Transform|MakeTransform (Spline|GetLocationatDistanceAlongSpline _spline (Math|Float|Lerp 0.0 (Spline|GetSplineLength (Variables|/Game/Blueprints/Enviromental/Moving_Objects/BP_SplinePath.BP_SplinePath_C|GetSpline (Variables|Default|GetPathToFollow))) _move_track) "World") (Spline|GetRotationatDistanceAlongSpline _spline (Math|Float|Lerp 0.0 (Spline|GetSplineLength (Variables|/Game/Blueprints/Enviromental/Moving_Objects/BP_SplinePath.BP_SplinePath_C|GetSpline (Variables|Default|GetPathToFollow))) _move_track) "Local") (Transformation|GetActorScale3D self))))
          (:Finished
            (CallFunction|MoveObject))))
      (:B
        (Timeline|Move%20Object%20T Reverse)))
    (else
      (Timeline|Move%20Object%20T Play))))

(event EventBeginPlay
  ;[1 1 1] Get Spline Path //Omar
  (CallFunction|MoveObject))

(fn ConstructionScript)