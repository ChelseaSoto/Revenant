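; BP_MazeBrazier is an environmental brazier whose light turns on when a linked puzzle is finished.
; On BeginPlay it hides its PointLight and binds TurnOnLight to the puzzle's finished event.
; TurnOnLight reveals the light, sets IsActive, calls IsCompleted, and eases the light to a fixed relative position over a short time.
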(event Custom|TurnOnLight
  (Development|SetHiddeninGame (Variables|Default|GetPointLight) false true)
  (Variables|Default|SetisActive? true)
  (Default|CallIsCompleted)
  (Components|MoveComponentTo (Variables|Default|GetPointLight) "0.000000,0.000000,130.000000" "0, 0, 0" false true 2.0 false))

(event EventBeginPlay
  (Development|SetHiddeninGame (Variables|Default|GetPointLight) true true)
  (EventDispatchers|BindEventtoPuzzleFinished (Variables|Default|GetPuzzle%20I%20need%20done) (delegate Custom|TurnOnLight)))

(fn ConstructionScript)