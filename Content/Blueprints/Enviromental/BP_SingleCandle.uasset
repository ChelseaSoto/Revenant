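; BP_SingleCandle is an environmental candle that puts itself out by destroying its Niagara effect and point light.
; BeginPlay picks a random delay, and Tick watches IsCandleActive, which is not set in these graphs.
; While inactive, Tick restarts a Retriggerable Delay every frame, so removal and the IsDestroyed latch wait until those retriggers stop.
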(event EventBeginPlay
  (Variables|Default|SetRandomDelay (Math|Random|RandomFloatinRange 2.0 4.0)))

(event Collision|EventActorBeginOverlap
  (params (OtherActor :type Actor%20Object%20Reference)))

(event EventTick
  (params (DeltaSeconds :type Float%20%28single-precision%29))
  (if (not (Variables|Default|GetIsDestroyed?))
    (if (not (Variables|Default|GetIsCandleActive?))
      (Utilities|FlowControl|RetriggerableDelay (Variables|Default|GetRandomDelay))
      (Components|DestroyComponent (Variables|Default|GetNiagara1))
      (Components|DestroyComponent (Variables|Default|GetPointLight))
      (Variables|Default|SetIsDestroyed? true))))

(fn ConstructionScript)