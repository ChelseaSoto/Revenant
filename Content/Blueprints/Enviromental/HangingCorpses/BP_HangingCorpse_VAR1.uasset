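; Hanging corpse prop variant that slowly twists back and forth around its local yaw axis as environmental dressing.
; BeginPlay randomizes speed, swing duration and damping factor per instance so the motion varies.
; Tick rotates the actor and flips direction whenever the timer reaches the swing duration.
; The damping factor only scales the constant speed, so the motion never decays.
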(event EventBeginPlay
  (Variables|Default|SetSwingSpeed (Math|Random|RandomFloatinRange 2.0 5.0))
  (Variables|Default|SetSwingDuration (Math|Random|RandomFloatinRange 6.0 9.0))
  (Variables|Default|SetDampingFactor (Math|Random|RandomFloatinRange 0.96 0.99)))

(event Collision|EventActorBeginOverlap
  (params (OtherActor :type Actor%20Object%20Reference)))

(event EventTick
  (params (DeltaSeconds :type Float%20%28single-precision%29))
  (Variables|Default|SetCurrentTime (+ DeltaSeconds (Variables|Default|GetCurrentTime)))
  (Variables|Default|SetNewSwingSpeed (* (Variables|Default|GetSwingSpeed) (Variables|Default|GetDampingFactor)))
  (Transformation|AddActorLocalRotation (Math|Rotator|MakeRotator 0.0 0.0 (* (Variables|Default|GetRotationDirection) (Variables|Default|GetNewSwingSpeed) DeltaSeconds)) false false)
  (if (>= (Variables|Default|GetCurrentTime) (Variables|Default|GetSwingDuration))
    (Variables|Default|SetCurrentTime 0.0)
    (Variables|Default|SetRotationDirection (* (Variables|Default|GetRotationDirection) -1.0))))

(fn ConstructionScript)