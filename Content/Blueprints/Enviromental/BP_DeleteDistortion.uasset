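; BP_DeleteDistortion is an environmental actor apparently meant to clear a distortion once tracked enemies die, but that logic is unwired.
; BeginPlay only caches a ShadowMage and ShadowMelee reference, redundantly repeating the class lookup for each EnemiesToTrack entry.
; Disconnected nodes would count down deaths, bind a melee death dispatcher, and destroy a set of actors plus itself at zero.
; Tick and the DeleteDistortion event are empty.
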(event Custom|DeleteDistortion)

(event EventBeginPlay
  (for _array_element (Variables|Default|GetEnemiesToTrack)
    (bind _returnvalue (Actor|GetActorOfClass "/Game/Blueprints/Enemies/Blueprints/BP_ShadowMage.BP_ShadowMage_C"))
    (Variables|Default|SetShadowMage _returnvalue)
    (bind _returnvalue_2 (Actor|GetActorOfClass "/Game/Blueprints/Enemies/Blueprints/BP_ShadowMelee.BP_ShadowMelee_C"))
    (Variables|Default|SetShadowMelee _returnvalue_2)))

(event Collision|EventActorBeginOverlap
  (params (OtherActor :type Actor%20Object%20Reference)))

(event EventTick
  (params (DeltaSeconds :type Float%20%28single-precision%29)))

(fn ConstructionScript)