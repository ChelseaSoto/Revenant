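; BP_Noura is an environmental actor that jumps to the next preset transform each time the player character overlaps it.
; Begin overlap teleports it to the current entry in its Positions array and advances Index, until the list runs out.
; A DoOnce gate, reset after a short delay, keeps repeated overlaps from skipping through positions.
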(event Collision|EventActorBeginOverlap
  (params (OtherActor :type Actor%20Object%20Reference))
  (if (== OtherActor (Game|GetPlayerCharacter 0))
    (if (< (Variables|Default|Getindex) (Utilities|Array|Length (Variables|Default|GetPositions)))
      (Utilities|FlowControl|DoOnce false :!label _label
        (:Completed
          (Transformation|SetActorTransform (Utilities|Array|Get(acopy) (Variables|Default|GetPositions) (Variables|Default|Getindex)) false true)
          (Math|Integer|IncrementInt (Variables|Default|Getindex)
            (:%20%20
              (Utilities|FlowControl|Delay 0.2)
              (goto _label Reset))))))))

(fn ConstructionScript)