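; BP_MovingWall is an environmental wall actor that slides to a marked location when the player enters its trigger.
; On overlap by player pawn 0, it moves its root component to the MoveLocation component's world X and Y over TimeToMove using MoveComponentTo.
; The root keeps its current height and rotation, and the graph has no return movement.
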(event OnComponentBeginOverlap(Trigger)
  (params (OverlappedComponent :type Primitive%20Component%20Object%20Reference) (OtherActor :type Actor%20Object%20Reference) (OtherComp :type Primitive%20Component%20Object%20Reference) (OtherBodyIndex :type Integer) (bFromSweep :type Boolean) (SweepResult :type Hit%20Result%20Structure%20%28by%20ref%29))
  (bind _defaultsceneroot (Variables|Default|GetDefaultSceneRoot))
  (Variables|Default|SetMove%20To (Transformation|GetWorldLocation (Variables|Default|GetMove%20Location)))
  (if (== OtherActor (Game|Player|GetPlayerPawn 0))
    (Components|MoveComponentTo _defaultsceneroot (Math|Vector|MakeVector (.x (Variables|Default|GetMove%20To)) (.y (Variables|Default|GetMove%20To)) (.z (Transformation|GetWorldLocation _defaultsceneroot))) (Variables|/Script/Engine.SceneComponent|GetRelativeRotation _defaultsceneroot) false false (Variables|Default|GetTime%20to%20Move) false)))

(fn ConstructionScript)