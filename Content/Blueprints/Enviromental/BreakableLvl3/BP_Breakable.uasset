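; Breakable level actor linked to a target object, which it notifies when broken.
; On BeginPlay it runs a projectile path prediction toward ObjectToDestroy with overridden gravity, turns the path points into a spline, and builds spline meshes along it as a connection between the two.
; Broken fires once, calling DestryInc on the target and then destroying this actor.
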(event EventBeginPlay
  (bind _returnvalue (Transformation|GetActorLocation))
  (bind _splinetoobject (Variables|Default|GetSplineToObject))
  (bind _predictresult (Class|GameplayStatics|BlueprintPredictProjectilePathAdvanced (Utilities|Struct|MakePredictProjectilePathParams _returnvalue (- (Transformation|GetActorLocation (Variables|Default|GetObjectToDestroy)) _returnvalue) false 0.0 1.0 false "ECC_WorldStatic" "ObjectTypeQuery1" 0 2e+01 -1.0 "None" 0.0 false)))
  (for _array_element (.pathdata _predictresult)
    (Spline|AddSplinePoint (Variables|Default|GetSplineToObject) (.Location (Utilities|Struct|BreakPredictProjectilePathPointData _array_element)) "World" true))
  (for _index (range 0 (- (Spline|GetNumberOfSplinePoints (Variables|Default|GetSplineToObject)) 2))
    (bind _returnvalue_2 (AddComponent|AddSplineMeshComponent true))
    (SplineMesh|SetStartandEnd _returnvalue_2 (.Location (Spline|GetLocationandTangentatSplinePoint _splinetoobject _index "World")) (.Tangent (Spline|GetLocationandTangentatSplinePoint _splinetoobject _index "World")) (.Location (Spline|GetLocationandTangentatSplinePoint _splinetoobject (+ _index 1) "World")) (.Tangent (Spline|GetLocationandTangentatSplinePoint _splinetoobject (+ _index 1) "World")) true :!class /Script/Engine.SplineMeshComponent)))

(fn ConstructionScript)

(fn Broken!
  (Utilities|FlowControl|DoOnce false
    (:Completed
      (Default|DestryInc (Variables|Default|GetObjectToDestroy))
      (Actor|DestroyActor)
      (return false))))