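; VanishText is an actor with a 3D text component that is visible only while the player character overlaps it.
; It hides the text on BeginPlay, shows it on begin overlap and hides it again on end overlap, printing a message on each overlap change.
; The unhide call also targets the player's root component, while the hide calls affect only the text.
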(event EventBeginPlay
  (Development|SetHiddeninGame (Variables|Default|GetText3D) true false))

(event Collision|EventActorBeginOverlap
  (params (OtherActor :type Actor%20Object%20Reference))
  (if (== OtherActor (Game|GetPlayerCharacter 0))
    (Development|PrintString "Time to be visible!")
    (Development|SetHiddeninGame (Variables|Default|GetText3D) false false)))

(event EventTick
  (params (DeltaSeconds :type Float%20%28single-precision%29)))

(event Collision|EventActorEndOverlap
  (params (OtherActor :type Actor%20Object%20Reference))
  (if (== OtherActor (Game|GetPlayerCharacter 0))
    (Development|PrintString "Time to hide!")
    (Development|SetHiddeninGame (Variables|Default|GetText3D) true false)))

(fn ConstructionScript)