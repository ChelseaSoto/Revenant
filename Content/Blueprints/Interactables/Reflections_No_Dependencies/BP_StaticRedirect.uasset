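; BP_StaticRedirect is an interactable block that the player character pushes a set distance by running into it.
; On hit, it rounds the player's forward vector into a push direction, then CanPush line-traces that the player faces it and box-traces that the way is clear.
; Push disables player movement, attaches the player to the block and slides both along the MoveBlock timeline; EndPush restores walking and detaches.
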(event Custom|Push
  ;[1 1 1] Push Distance
  (Variables|Default|SetCurrent%20Location (Transformation|GetActorLocation))
  (bind _position (Timeline|Move%20Block PlayFromStart)
    (:Update
      (Transformation|SetActorRelativeLocation (+ (* _position (Variables|Default|GetPushable%20Direction) (Variables|Default|GetTravel%20Distance)) (Variables|Default|GetCurrent%20Location))))
    (:Finished
      (CallFunction|EndPush))))

(event Custom|End%20Push
  (bind _returnvalue (Game|GetPlayerCharacter 0))
  ;[1 1 1] end push anim//Omar
  (Pawn|Components|CharacterMovement|SetMovementMode (Variables|/Script/Engine.Character|GetCharacterMovement _returnvalue) "MOVE_Walking" 0)
  (Transformation|DetachFromActor _returnvalue "KeepWorld" "KeepWorld" "KeepWorld"))

(event EventBeginPlay
  (|CallParentFunction) ; This node is disabled and will not be called.\nDrag off pins to build functionality.
)

(event Collision|EventActorBeginOverlap
  (params (OtherActor :type Actor%20Object%20Reference))
  (|CallParentFunction OtherActor) ; This node is disabled and will not be called.\nDrag off pins to build functionality.
)

(event EventTick
  (params (DeltaSeconds :type Float%20%28single-precision%29))
  (|CallParentFunction DeltaSeconds) ; This node is disabled and will not be called.\nDrag off pins to build functionality.
)

(event Collision|EventHit
  (params (MyComp :type Primitive%20Component%20Object%20Reference) (Other :type Actor%20Object%20Reference) (OtherComp :type Primitive%20Component%20Object%20Reference) (bSelfMoved :type Boolean) (HitLocation :type Vector :default "0, 0, 0") (HitNormal :type Vector :default "0, 0, 0") (NormalImpulse :type Vector :default "0, 0, 0") (Hit :type Hit%20Result%20Structure%20%28by%20ref%29))
  (bind _returnvalue (Transformation|GetActorForwardVector Other))
  (bind _returnvalue_2 (Game|GetPlayerCharacter 0))
  (if (== Other (Game|GetPlayerCharacter 0))
    ;[1 1 1] Get the direction I should be pushed //Omar
    (Variables|Default|SetPushable%20Direction (Math|Vector|MakeVector (Math|Conversions|ToFloat(Integer) (Math|Float|Round (.x _returnvalue))) (Math|Conversions|ToFloat(Integer) (Math|Float|Round (.y _returnvalue))) (Math|Conversions|ToFloat(Integer) (Math|Float|Round (.z _returnvalue)))))
    (bind _canpush (CallFunction|CanPush))
    (if _canpush
      (Development|PrintString "pushing")
      (Pawn|Components|CharacterMovement|DisableMovement (Variables|/Script/Engine.Character|GetCharacterMovement _returnvalue_2))
      (Transformation|AttachActorToActor _returnvalue_2 self "None" "KeepWorld" "KeepWorld" "KeepWorld" true)
      (CallFunction|Push)
      (else
        (Development|PrintString "no push")))))

(fn ConstructionScript
  (|CallParentFunction))

(fn CanPush
  (bind _returnvalue (Game|GetPlayerCharacter 0))
  (bind _self self)
  (bind _returnvalue_2 (Transformation|GetActorLocation _returnvalue))
  (bind _returnvalue_3 (Transformation|GetActorLocation _self))
  ;[1 1 1] Check if i can be pushed //Omar
  (bind (_outhit _returnvalue_4) (Collision|LineTraceByChannel _returnvalue_2 (+ _returnvalue_2 (* (Transformation|GetActorForwardVector _returnvalue) 1e+02)) "TraceTypeQuery1" false (Utilities|Array|MakeArray _returnvalue) "None" false))
  (if _returnvalue_4
    (if (== (.HitActor (Collision|BreakHitResult _outhit)) self)
      (bind _returnvalue_5 (Collision|BoxTraceByChannel _returnvalue_3 (+ _returnvalue_3 (* (Transformation|GetActorForwardVector (Game|GetPlayerCharacter 0)) 1.5e+02)) "20.000000,10.000000,90.000000" "0, 0, 0" "TraceTypeQuery1" false 0 "ForDuration"))
      (if _returnvalue_5
        (return false)
        (else
          (return true)))
      (else
        (return false)))
    (else
      (return false))))