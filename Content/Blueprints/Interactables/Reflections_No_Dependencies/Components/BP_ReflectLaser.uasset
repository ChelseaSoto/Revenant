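; Reflection Blueprint that makes lasers bounce off a surface by spawning a BP_LaserChild at the impact point.
; On a hit, it mirrors the incoming direction around the impact normal and passes color, spawn reference and an extended ID to the child.
; Children register both locally and with the originating SpawnRef.
; When the hit ends, it destroys attached lasers whose IDs contain the incoming laser's ID, clearing downstream bounces it holds.
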(fn ConstructionScript
  (|CallParentFunction))

(fn CalcRotation
  (params (impact%20point :type Vector) (Impact%20Normal :type Vector) (Trace%20Start :type Vector))
  ;[1 1 1] Calculates Reflection watch video for explantion tbh //Omar https://www.youtube.com/watch?v=74TRpvuaKfs
  (return (Math|Rotator|MakeRotfromZ (Math|Vector|MirrorVectorbyNormal (- impact%20point Trace%20Start) Impact%20Normal))))

(fn ClearAttachedLasers
  (params (ID_Clear :type String))
  ;[1 1 1] Check Every ID for similar ones to mine then destroy them and remove from list
  (bind _arrayelement (Utilities|Array|ReverseforEachLoop (Variables|Default|GetLasersAttached))
    (:LoopBody
      (Utilities|IsValid _arrayelement
        (:Is%20Valid
          (if (Utilities|String|Contains (Variables|/Game/Blueprints/Laser/BP_LaserChild.BP_LaserChild_C|GetLaser_ID _arrayelement) ID_Clear)
            (Actor|DestroyActor _arrayelement)
            (Utilities|Array|RemoveItem (Variables|Default|GetLasersAttached) _arrayelement)))))))

(fn LaserBounce
  (params (LaserThatHit :type BP%20Laser%20Child%20Object%20Reference) (HitResponse :type Boolean) (HitResult :type Hit%20Result%20Structure))
  (bind (_bblockinghit _binitialoverlap _time _distance _location _impactpoint _normal _impactnormal _physmat _hitactor _hitcomponent _hitbonename _bonename _hititem _elementindex _faceindex _tracestart) (Collision|BreakHitResult HitResult))
  (if HitResponse
    ;[1 1 1] Sets refrences for new Laser //Omar
    (bind _returnvalue (Game|SpawnActorfromClass "/Game/Blueprints/Laser/BP_LaserChild.BP_LaserChild_C" (Math|Transform|MakeTransform _impactpoint (CallFunction|CalcRotation _impactpoint _impactnormal _tracestart) "1.000000,1.000000,1.000000") "Undefined" "MultiplyWithRoot" 0 (Default|UpdateID LaserThatHit "B") LaserThatHit (Variables|/Game/Blueprints/Laser/BP_LaserParent.BP_LaserParent_C|GetLinearColor LaserThatHit) (Variables|/Game/Blueprints/Laser/BP_LaserParent.BP_LaserParent_C|GetSpawnRef LaserThatHit) 0))
    (Utilities|Array|Add (Variables|Default|GetLasersAttached) _returnvalue)
    (Utilities|Array|Add (Variables|/Game/Blueprints/Laser/BP_LaserSpawn.BP_LaserSpawn_C|GetChild%20Lasers (Variables|/Game/Blueprints/Laser/BP_LaserParent.BP_LaserParent_C|GetSpawnRef LaserThatHit)) _returnvalue)
    (return _returnvalue)
    (else
      ;[1 1 1] Gets hit info from parent laser for reflection calc //Omar
      ;;[1 1 1] If im not being hit clear any lasers I've made
      (CallFunction|ClearAttachedLasers (Variables|/Game/Blueprints/Laser/BP_LaserChild.BP_LaserChild_C|GetLaser_ID LaserThatHit)))))