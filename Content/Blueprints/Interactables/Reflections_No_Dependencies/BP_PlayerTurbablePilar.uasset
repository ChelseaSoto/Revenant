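; Interactable pillar the player rotates in 90-degree steps, apparently for mirror/reflection puzzles.
; Interact calls Turn, which faces the player toward the pillar, plays a montage and sound, then lerps the mesh yaw on a timeline.
; A CanTurn flag blocks re-triggering until the timeline finishes and saves the new yaw.
; Box overlap toggles a gamepad-aware interact prompt and an overlay highlight material.
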(event OnComponentBeginOverlap(Box)
  (params (OverlappedComponent :type Primitive%20Component%20Object%20Reference) (OtherActor :type Actor%20Object%20Reference) (OtherComp :type Primitive%20Component%20Object%20Reference) (OtherBodyIndex :type Integer) (bFromSweep :type Boolean) (SweepResult :type Hit%20Result%20Structure%20%28by%20ref%29))
  ;[1 1 1] Player Interaction pop up
  (bind _asbp_third_person_character (Utilities|Casting|CastToBP_ThirdPersonCharacter OtherActor))
  (bind _returnvalue (UserInterface|CreateWidget "/Game/UI/P_Interact.P_Interact_C" 0 (Variables|/Game/ThirdPerson/Blueprints/BP_ThirdPersonCharacter.BP_ThirdPersonCharacter_C|GetUsingGamepad _asbp_third_person_character)))
  (Variables|Default|SetInteractPrompt _returnvalue)
  (if (== OtherActor (Game|GetPlayerCharacter 0))
    (UserInterface|Viewport|AddtoViewport (Variables|Default|GetInteractPrompt) 0)
    (Rendering|Material|SetOverlayMaterial (Variables|Default|GetSM_Visual) "/Game/Materials/M_OverlayMat.M_OverlayMat" :!class /Script/Engine.MeshComponent)))

(event OnComponentEndOverlap(Box)
  (params (OverlappedComponent :type Primitive%20Component%20Object%20Reference) (OtherActor :type Actor%20Object%20Reference) (OtherComp :type Primitive%20Component%20Object%20Reference) (OtherBodyIndex :type Integer))
  ;[1 1 1] Player Interaction pop up
  (if (== (Game|GetPlayerCharacter 0) OtherActor)
    (Widget|RemovefromParent (Variables|Default|GetInteractPrompt))
    (Rendering|Material|SetOverlayMaterial (Variables|Default|GetSM_Visual) 0 :!class /Script/Engine.MeshComponent)))

(event Custom|Turn
  (if (Variables|Default|GetCanTurn)
    ;[1 1 1] Turns 90 degrees then saves rotation
    (CallFunction|ANIMATION)
    (Audio|PlaySoundatLocation "/Game/Audio/SFX/WorldSFX/Pillars/SQ_Mirror.SQ_Mirror" (Transformation|GetActorLocation) "0, 0, 0" 1.0 1.0 0.0 0 0 0 0)
    (Variables|Default|SetCanTurn false)
    (bind _newtrack_0 (Timeline|TurnPillar PlayFromStart)
      (:Update
        (Transformation|SetRelativeRotation (Variables|Default|GetSM_Visual) (Math|Rotator|MakeRotator 0.0 0.0 (Math|Float|Lerp (Variables|Default|GetCurrentRotation) (+ (Variables|Default|GetCurrentRotation) 9e+01) _newtrack_0)) false false))
      (:Finished
        (Variables|Default|SetCurrentRotation (.yaw (Variables|/Script/Engine.SceneComponent|GetRelativeRotation (Variables|Default|GetSM_Visual))))
        (Variables|Default|SetCanTurn true)))))

(event Custom|ANIMATION
  (bind _my_player_character (CallFunction|GetMyPlayerCharacter))
  (Transformation|SetActorRotation _my_player_character (Math|Rotator|FindLookatRotation (.location (Transformation|GetActorTransform _my_player_character)) (Transformation|GetActorLocation)))
  (Animation|Montage|PlayMontage (Variables|/Script/Engine.Character|GetMesh _my_player_character) "/Game/ArtPrototype/Rigs/Hossam/Animations/New/TurnMirror_Montage.TurnMirror_Montage" 1.2))

(event EventBeginPlay
  (Variables|Default|SetCurrentRotation (.yaw (Variables|/Script/Engine.SceneComponent|GetRelativeRotation (Variables|Default|GetSM_Visual)))))

(event Collision|EventActorBeginOverlap
  (params (OtherActor :type Actor%20Object%20Reference))
  (|CallParentFunction OtherActor))

(fn ConstructionScript
  (|CallParentFunction))

(fn Interact
  (CallFunction|Turn)
  (return ""))