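; BP_LevelTransitions_Level2 is an overlap trigger that updates level-lock progress in the save game, commented as unlocking level 3.
; When BP_ThirdPersonCharacter overlaps it, it loads BPC_levellock from a fixed save slot, sets Level2Unlock to false and saves it back.
; Despite the name, it performs no level load, and it does nothing if that save cannot be loaded and cast.
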(event EventBeginPlay
  (|CallParentFunction) ; This node is disabled and will not be called.\nDrag off pins to build functionality.
)

(event Collision|EventActorBeginOverlap
  (params (OtherActor :type Actor%20Object%20Reference))
  ;[1 1 1] unlocks level 3/Omar
  (Utilities|Casting|CastToBP_ThirdPersonCharacter OtherActor)
  (bind _returnvalue (SaveGame|LoadGamefromSlot "slot1"))
  (bind _asbpc_levellock (Utilities|Casting|CastToBPC_levellock _returnvalue))
  (Variables|/Game/Savegame/BPC_levellock.BPC_levellock_C|SetLevel2%20Unlock _asbpc_levellock false)
  (SaveGame|SaveGametoSlot _asbpc_levellock "slot1"))

(event EventTick
  (params (DeltaSeconds :type Float%20%28single-precision%29))
  (|CallParentFunction DeltaSeconds) ; This node is disabled and will not be called.\nDrag off pins to build functionality.
)

(fn ConstructionScript
  (|CallParentFunction))