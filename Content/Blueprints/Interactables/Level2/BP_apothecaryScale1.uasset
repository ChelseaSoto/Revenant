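; Interactable apothecary balance scale for Level 2 that fires a dispatcher when both pans hold actors and the net mass is zero.
; Pan overlap events track actors and adjust a signed total using BP_ScaleItem mass, or one for other actors.
; AddMass maps that total to clamped spline distances, and a timeline lerps both cubes there.
; On BeginPlay, cubes start at spline midpoints and a timeline lowers the whole scale.
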(event OnComponentBeginOverlap(rightbox)
  (params (OverlappedComponent :type Primitive%20Component%20Object%20Reference) (OtherActor :type Actor%20Object%20Reference) (OtherComp :type Primitive%20Component%20Object%20Reference) (OtherBodyIndex :type Integer) (bFromSweep :type Boolean) (SweepResult :type Hit%20Result%20Structure%20%28by%20ref%29))
  (bind _rightcube (Variables|Default|GetRightCube))
  (bind _leftcube (Variables|Default|GetLeftCube))
  (bind _returnvalue (Transformation|GetWorldTransform _rightcube))
  (bind _returnvalue_2 (Transformation|GetWorldTransform _leftcube))
  (Utilities|Array|AddUnique (Variables|Default|GetRightActors) OtherActor)
  (bind _asbp_scale_item (Utilities|Casting|CastToBP_ScaleItem OtherActor)
    (:then
      (CallFunction|+Mass _asbp_scale_item))
    (:CastFailed
      (Math|Integer|IncrementInt (Variables|Default|GetTotalMass)
        (:%20%20
          _))))
  (CallFunction|AddMass)
  (bind _alpha (Timeline|Timeline PlayFromStart)
    (:Update
      (Transformation|SetWorldTransform _leftcube (Math|Transform|MakeTransform (Math|Vector|Lerp(Vector) (.location _returnvalue_2) (Spline|GetLocationatDistanceAlongSpline (Variables|Default|GetLeft%20Spline) (Variables|Default|GetCurrentLeftLength) "World") _alpha) (.rotation _returnvalue_2) (.scale _returnvalue_2)) false false)
      (Transformation|SetWorldTransform _rightcube (Math|Transform|MakeTransform (Math|Vector|Lerp(Vector) (.location _returnvalue) (Spline|GetLocationatDistanceAlongSpline (Variables|Default|GetRight%20Spline) (Variables|Default|GetCurrentRightLength) "World") _alpha) (.rotation _returnvalue) (.scale _returnvalue)) false false))))

(event OnComponentEndOverlap(rightbox)
  (params (OverlappedComponent :type Primitive%20Component%20Object%20Reference) (OtherActor :type Actor%20Object%20Reference) (OtherComp :type Primitive%20Component%20Object%20Reference) (OtherBodyIndex :type Integer))
  (bind _rightcube (Variables|Default|GetRightCube))
  (bind _leftcube (Variables|Default|GetLeftCube))
  (bind _returnvalue (Transformation|GetWorldTransform _rightcube))
  (bind _returnvalue_2 (Transformation|GetWorldTransform _leftcube))
  (Utilities|Array|RemoveItem (Variables|Default|GetRightActors) OtherActor)
  (bind _asbp_scale_item (Utilities|Casting|CastToBP_ScaleItem OtherActor)
    (:then
      (CallFunction|-Mass _asbp_scale_item))
    (:CastFailed
      (Math|Integer|DecrementInt (Variables|Default|GetTotalMass)
        (:%20%20
          _))))
  (CallFunction|AddMass)
  (bind _alpha (Timeline|Timeline PlayFromStart)
    (:Update
      (Transformation|SetWorldTransform _leftcube (Math|Transform|MakeTransform (Math|Vector|Lerp(Vector) (.location _returnvalue_2) (Spline|GetLocationatDistanceAlongSpline (Variables|Default|GetLeft%20Spline) (Variables|Default|GetCurrentLeftLength) "World") _alpha) (.rotation _returnvalue_2) (.scale _returnvalue_2)) false false)
      (Transformation|SetWorldTransform _rightcube (Math|Transform|MakeTransform (Math|Vector|Lerp(Vector) (.location _returnvalue) (Spline|GetLocationatDistanceAlongSpline (Variables|Default|GetRight%20Spline) (Variables|Default|GetCurrentRightLength) "World") _alpha) (.rotation _returnvalue) (.scale _returnvalue)) false false))))

(event OnComponentBeginOverlap(leftbox)
  (params (OverlappedComponent :type Primitive%20Component%20Object%20Reference) (OtherActor :type Actor%20Object%20Reference) (OtherComp :type Primitive%20Component%20Object%20Reference) (OtherBodyIndex :type Integer) (bFromSweep :type Boolean) (SweepResult :type Hit%20Result%20Structure%20%28by%20ref%29))
  (bind _rightcube (Variables|Default|GetRightCube))
  (bind _leftcube (Variables|Default|GetLeftCube))
  (bind _returnvalue (Transformation|GetWorldTransform _rightcube))
  (bind _returnvalue_2 (Transformation|GetWorldTransform _leftcube))
  (Utilities|Array|AddUnique (Variables|Default|GetLeftActors) OtherActor)
  (bind _asbp_scale_item (Utilities|Casting|CastToBP_ScaleItem OtherActor)
    (:then
      (CallFunction|-Mass _asbp_scale_item))
    (:CastFailed
      (Math|Integer|DecrementInt (Variables|Default|GetTotalMass)
        (:%20%20
          _))))
  (CallFunction|AddMass)
  (bind _alpha (Timeline|Timeline PlayFromStart)
    (:Update
      (Transformation|SetWorldTransform _leftcube (Math|Transform|MakeTransform (Math|Vector|Lerp(Vector) (.location _returnvalue_2) (Spline|GetLocationatDistanceAlongSpline (Variables|Default|GetLeft%20Spline) (Variables|Default|GetCurrentLeftLength) "World") _alpha) (.rotation _returnvalue_2) (.scale _returnvalue_2)) false false)
      (Transformation|SetWorldTransform _rightcube (Math|Transform|MakeTransform (Math|Vector|Lerp(Vector) (.location _returnvalue) (Spline|GetLocationatDistanceAlongSpline (Variables|Default|GetRight%20Spline) (Variables|Default|GetCurrentRightLength) "World") _alpha) (.rotation _returnvalue) (.scale _returnvalue)) false false))))

(event OnComponentEndOverlap(leftbox)
  (params (OverlappedComponent :type Primitive%20Component%20Object%20Reference) (OtherActor :type Actor%20Object%20Reference) (OtherComp :type Primitive%20Component%20Object%20Reference) (OtherBodyIndex :type Integer))
  (bind _rightcube (Variables|Default|GetRightCube))
  (bind _leftcube (Variables|Default|GetLeftCube))
  (bind _returnvalue (Transformation|GetWorldTransform _rightcube))
  (bind _returnvalue_2 (Transformation|GetWorldTransform _leftcube))
  (Utilities|Array|RemoveItem (Variables|Default|GetLeftActors) OtherActor)
  (bind _asbp_scale_item (Utilities|Casting|CastToBP_ScaleItem OtherActor)
    (:then
      (CallFunction|+Mass _asbp_scale_item))
    (:CastFailed
      (Math|Integer|IncrementInt (Variables|Default|GetTotalMass)
        (:%20%20
          _))))
  (CallFunction|AddMass)
  (bind _alpha (Timeline|Timeline PlayFromStart)
    (:Update
      (Transformation|SetWorldTransform _leftcube (Math|Transform|MakeTransform (Math|Vector|Lerp(Vector) (.location _returnvalue_2) (Spline|GetLocationatDistanceAlongSpline (Variables|Default|GetLeft%20Spline) (Variables|Default|GetCurrentLeftLength) "World") _alpha) (.rotation _returnvalue_2) (.scale _returnvalue_2)) false false)
      (Transformation|SetWorldTransform _rightcube (Math|Transform|MakeTransform (Math|Vector|Lerp(Vector) (.location _returnvalue) (Spline|GetLocationatDistanceAlongSpline (Variables|Default|GetRight%20Spline) (Variables|Default|GetCurrentRightLength) "World") _alpha) (.rotation _returnvalue) (.scale _returnvalue)) false false))))

(event EventBeginPlay
  (bind _defaultsceneroot (Variables|Default|GetDefaultSceneRoot))
  (bind _leftcube (Variables|Default|GetLeftCube))
  (bind _left_spline (Variables|Default|GetLeft%20Spline))
  (bind _right_spline (Variables|Default|GetRight%20Spline))
  (bind _rightcube (Variables|Default|GetRightCube))
  (bind _returnvalue (Spline|GetSplineLength _left_spline))
  (bind _returnvalue_2 (Spline|GetSplineLength _right_spline))
  (bind _returnvalue_3 (Transformation|GetWorldLocation _defaultsceneroot))
  (Utilities|FlowControl|Sequence
    (:then_0
      ;[1 1 1] Sets to the middle
      (Variables|Default|SetLeft%20Length _returnvalue)
      (Transformation|SetWorldTransform _leftcube (Math|Transform|MakeTransform (Spline|GetLocationatDistanceAlongSpline _left_spline (/ _returnvalue 2.0) "World") (Transformation|GetWorldRotation _leftcube) (Transformation|GetWorldScale _leftcube)) false false)
      (Variables|Default|SetRight%20Length _returnvalue_2)
      (Transformation|SetWorldTransform _rightcube (Math|Transform|MakeTransform (Spline|GetLocationatDistanceAlongSpline _right_spline (/ _returnvalue_2 2.0) "World") (Transformation|GetWorldRotation _rightcube) (Transformation|GetWorldScale _rightcube)) false false))
    (:then_1
      (bind _newtrack_0 (Timeline|Lower Play)
        (:Update
          (Transformation|SetWorldLocation _defaultsceneroot (Math|Vector|MakeVector (.x _returnvalue_3) (.y _returnvalue_3) (Math|Float|Lerp (.z _returnvalue_3) (- (.z _returnvalue_3) (Variables|Default|GetLowerLength)) _newtrack_0)) false false))))))

(fn ConstructionScript)

(fn AddMass
  (bind _totalmass (Variables|Default|GetTotalMass))
  (if (< _totalmass -3)
    (Variables|Default|SetCurrentLeftLength (* (Variables|Default|GetLeft%20Length) 1.0))
    (Variables|Default|SetCurrentRightLength (* (Variables|Default|GetRight%20Length) 0.0))
    (elif (> _totalmass 3)
      (Variables|Default|SetCurrentLeftLength (* (Variables|Default|GetLeft%20Length) 0.0))
      (Variables|Default|SetCurrentRightLength (* (Variables|Default|GetRight%20Length) 1.0))
      (else
        (switch int (Variables|Default|GetTotalMass)
          (:-3
            (Variables|Default|SetCurrentLeftLength (* (Variables|Default|GetLeft%20Length) 1.0))
            (Variables|Default|SetCurrentRightLength (* (Variables|Default|GetRight%20Length) 0.0)))
          (:-2
            (Variables|Default|SetCurrentLeftLength (* (Variables|Default|GetLeft%20Length) 0.8))
            (Variables|Default|SetCurrentRightLength (* (Variables|Default|GetRight%20Length) 0.2)))
          (:-1
            (Variables|Default|SetCurrentLeftLength (* (Variables|Default|GetLeft%20Length) 0.65))
            (Variables|Default|SetCurrentRightLength (* (Variables|Default|GetRight%20Length) 0.35)))
          (:0
            (Variables|Default|SetCurrentLeftLength (* (Variables|Default|GetLeft%20Length) 0.5))
            (Variables|Default|SetCurrentRightLength (* (Variables|Default|GetRight%20Length) 0.5))
            (if (and (> (Utilities|Array|Length (Variables|Default|GetLeftActors)) 0) (> (Utilities|Array|Length (Variables|Default|GetRightActors)) 0))
              (Default|CallDispatch true)))
          (:1
            (Variables|Default|SetCurrentLeftLength (* (Variables|Default|GetLeft%20Length) 0.35))
            (Variables|Default|SetCurrentRightLength (* (Variables|Default|GetRight%20Length) 0.65)))
          (:2
            (Variables|Default|SetCurrentLeftLength (* (Variables|Default|GetLeft%20Length) 0.25))
            (Variables|Default|SetCurrentRightLength (* (Variables|Default|GetRight%20Length) 0.75)))
          (:3
            (Variables|Default|SetCurrentLeftLength (* (Variables|Default|GetLeft%20Length) 0.0))
            (Variables|Default|SetCurrentRightLength (* (Variables|Default|GetRight%20Length) 1.0))))
        (return))))
  (return))

(fn +Mass
  (params (Target :type BP%20Scale%20Item%20Object%20Reference))
  (Variables|Default|SetTotalMass (+ (Variables|Default|GetTotalMass) (Variables|/Game/Blueprints/Interactables/Level2/BP_ScaleItem.BP_ScaleItem_C|GetScale%20Mass Target))))

(fn -Mass
  (params (Target :type BP%20Scale%20Item%20Object%20Reference))
  (Variables|Default|SetTotalMass (- (Variables|Default|GetTotalMass) (Variables|/Game/Blueprints/Interactables/Level2/BP_ScaleItem.BP_ScaleItem_C|GetScale%20Mass Target))))