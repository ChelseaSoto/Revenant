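; BP_PickUp is a Level 2 interactable Blueprint that lets the player pick up and carry BP_ScaleItem objects while the interact input is held.
; On BeginPlay it adds a Physics Handle to the player character; pressing interact sphere-traces physics bodies around the player and grabs the scale item found.
; Tick moves the handle target ahead of AbilitySpawn along the follow camera's forward vector, and releasing interact drops the item.
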(event Input|EnhancedActionEvents|EnhancedInputActionIA_Interact
  (params (ActionValue :type Boolean) (ElapsedSeconds :type Float%20%28double-precision%29) (TriggeredSeconds :type Float%20%28double-precision%29) (InputAction :type Input%20Action%20Object%20Reference :default "/Game/ThirdPerson/Input/Actions/IA_Interact.IA_Interact"))
  (bind _returnvalue (Game|Player|GetPlayerPawn 0))
  (bind _returnvalue_2 (Transformation|GetActorLocation _returnvalue))
  (:Started
    ;[1 1 1] Grabbing System
    (bind (_outhit _returnvalue_3) (Collision|SphereTraceForObjects _returnvalue_2 _returnvalue_2 1.4e+02 (Utilities|Array|MakeArray "ObjectTypeQuery4") false 0 "None"))
    (bind _asbp_scale_item (Utilities|Casting|CastToBP_ScaleItem (.HitActor (Collision|BreakHitResult _outhit))))
    (Default|PickedUp _asbp_scale_item)
    (if (and _returnvalue_3 (Utilities|String|Contains (Utilities|GetDisplayName (.HitActor (Collision|BreakHitResult _outhit))) "ScaleItem"))
      (Physics|Components|PhysicsHandle|GrabComponentatLocationwithRotation (Variables|Default|GetPhysicsHandle) (.HitComponent (Collision|BreakHitResult _outhit)) "None" (.location (Transformation|GetWorldTransform (.HitComponent (Collision|BreakHitResult _outhit)))) (.rotation (Transformation|GetWorldTransform (.HitComponent (Collision|BreakHitResult _outhit)))))
      (Variables|Default|SetisGrabbingObject? true)
      (Variables|/Game/ThirdPerson/Blueprints/BP_ThirdPersonCharacter.BP_ThirdPersonCharacter_C|SetisPickingup (CallFunction|GetMyPlayerCharacter) true)))
  (:Completed
    (if (Variables|Default|GetisGrabbingObject?)
      (Physics|Components|PhysicsHandle|ReleaseComponent (stale EventBeginPlay _returnvalue))
      (Variables|Default|SetisGrabbingObject? false)
      (Variables|/Game/ThirdPerson/Blueprints/BP_ThirdPersonCharacter.BP_ThirdPersonCharacter_C|SetisPickingup (CallFunction|GetMyPlayerCharacter) false))))

(event EventTick
  (params (DeltaSeconds :type Float%20%28single-precision%29))
  (bind _my_player_character (CallFunction|GetMyPlayerCharacter))
  ;[1 1 1] Object Picked Up Loop
  (if (Variables|Default|GetisGrabbingObject?)
    (Physics|Components|PhysicsHandle|SetTargetLocation (Variables|Default|GetPhysicsHandle) (+ (* (Math|Vector|GetForwardVector (Transformation|GetWorldRotation (Variables|/Game/ThirdPerson/Blueprints/BP_ThirdPersonCharacter.BP_ThirdPersonCharacter_C|GetFollowCamera _my_player_character))) 5e+01) (Transformation|GetWorldLocation (Variables|/Game/ThirdPerson/Blueprints/BP_ThirdPersonCharacter.BP_ThirdPersonCharacter_C|GetAbilitySpawn _my_player_character))))))

(event EventBeginPlay
  (bind _returnvalue (Game|AddComponentbyClass (CallFunction|GetMyPlayerCharacter) "/Script/Engine.PhysicsHandleComponent"))
  (Variables|Default|SetPhysicsHandle _returnvalue))