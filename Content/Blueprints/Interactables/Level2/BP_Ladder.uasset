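; BP_Ladder is a Level 2 interactable ladder that moves the player by teleport instead of climbing.
; Entering its Box trigger creates and shows a P_Interact prompt, passing whether the player uses a gamepad, and leaving removes it.
; Its Interact function teleports the player character to the Arrow component's world location and rotation, so the Arrow marks the destination, and returns an empty string.
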(event OnComponentBeginOverlap(Box)
  (params (OverlappedComponent :type Primitive%20Component%20Object%20Reference) (OtherActor :type Actor%20Object%20Reference) (OtherComp :type Primitive%20Component%20Object%20Reference) (OtherBodyIndex :type Integer) (bFromSweep :type Boolean) (SweepResult :type Hit%20Result%20Structure%20%28by%20ref%29))
  (bind _my_player_character (CallFunction|GetMyPlayerCharacter))
  (if (== OtherActor _my_player_character)
    (bind _returnvalue (UserInterface|CreateWidget "/Game/UI/P_Interact.P_Interact_C" 0 (Variables|/Game/ThirdPerson/Blueprints/BP_ThirdPersonCharacter.BP_ThirdPersonCharacter_C|GetUsingGamepad _my_player_character)))
    (bind _output_get (Variables|Default|SetInteractPrompt _returnvalue))
    (UserInterface|Viewport|AddtoViewport _output_get 0)))

(event OnComponentEndOverlap(Box)
  (params (OverlappedComponent :type Primitive%20Component%20Object%20Reference) (OtherActor :type Actor%20Object%20Reference) (OtherComp :type Primitive%20Component%20Object%20Reference) (OtherBodyIndex :type Integer))
  (if (== OtherActor (CallFunction|GetMyPlayerCharacter))
    (Widget|RemovefromParent (Variables|Default|GetInteractPrompt))))

(fn ConstructionScript)

(fn Interact
  (bind _arrow (Variables|Default|GetArrow))
  (bind _returnvalue (Transformation|GetWorldTransform _arrow))
  (Transformation|Teleport (CallFunction|GetMyPlayerCharacter) (.location _returnvalue) (.rotation _returnvalue))
  (return ""))