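; Interactable apothecary balance scale for Level 2 that tips its left and right cubes according to mass totals tracked per side.
; Trigger overlap events update each total from the OverlappedComponent's mass; end overlap sets it to that mass minus the total.
; CheckMass then picks sides, and a timeline lerps the cubes to bottom and top markers, or to their starting heights when equal.
; Optionally, the whole scale lowers to LowerTo's height on BeginPlay.
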(event OnComponentBeginOverlap(RightTrigger)
  (params (OverlappedComponent :type Primitive%20Component%20Object%20Reference) (OtherActor :type Actor%20Object%20Reference) (OtherComp :type Primitive%20Component%20Object%20Reference) (OtherBodyIndex :type Integer) (bFromSweep :type Boolean) (SweepResult :type Hit%20Result%20Structure%20%28by%20ref%29))
  (Variables|Default|SetRightMass (+ (Physics|GetMass OverlappedComponent) (Variables|Default|GetRightMass)))
  (bind (_to_lower _to_raise _is_equal_) (CallFunction|CheckMass))
  (Variables|Default|SetTo%20Lower _to_lower)
  (Variables|Default|SetTo%20Raise _to_raise)
  (bind _alpha (Timeline|Timeline PlayFromStart)
    (:Update
      (if (not _is_equal_)
        (CallFunction|Lower+Raise (Variables|Default|GetTo%20Lower) (Variables|Default|GetTo%20Raise) _alpha)
        (else
          (CallFunction|EvenOut (Variables|Default|GetLeftCube) (Variables|Default|GetRightCube) _alpha))))))

(event OnComponentEndOverlap(RightTrigger)
  (params (OverlappedComponent :type Primitive%20Component%20Object%20Reference) (OtherActor :type Actor%20Object%20Reference) (OtherComp :type Primitive%20Component%20Object%20Reference) (OtherBodyIndex :type Integer))
  (Variables|Default|SetRightMass (- (Physics|GetMass OverlappedComponent) (Variables|Default|GetRightMass)))
  (bind (_to_lower _to_raise _is_equal_) (CallFunction|CheckMass))
  (Variables|Default|SetTo%20Lower _to_lower)
  (Variables|Default|SetTo%20Raise _to_raise)
  (bind _alpha (Timeline|Timeline PlayFromStart)
    (:Update
      (if (not _is_equal_)
        (CallFunction|Lower+Raise (Variables|Default|GetTo%20Lower) (Variables|Default|GetTo%20Raise) _alpha)
        (else
          (CallFunction|EvenOut (Variables|Default|GetLeftCube) (Variables|Default|GetRightCube) _alpha))))))

(event OnComponentBeginOverlap(LeftTrigger)
  (params (OverlappedComponent :type Primitive%20Component%20Object%20Reference) (OtherActor :type Actor%20Object%20Reference) (OtherComp :type Primitive%20Component%20Object%20Reference) (OtherBodyIndex :type Integer) (bFromSweep :type Boolean) (SweepResult :type Hit%20Result%20Structure%20%28by%20ref%29))
  (Variables|Default|SetLeftmass (+ (Physics|GetMass OverlappedComponent) (Variables|Default|GetLeftmass)))
  (bind (_to_lower _to_raise _is_equal_) (CallFunction|CheckMass))
  (Variables|Default|SetTo%20Lower _to_lower)
  (Variables|Default|SetTo%20Raise _to_raise)
  (bind _alpha (Timeline|Timeline PlayFromStart)
    (:Update
      (if (not _is_equal_)
        (CallFunction|Lower+Raise (Variables|Default|GetTo%20Lower) (Variables|Default|GetTo%20Raise) _alpha)
        (else
          (CallFunction|EvenOut (Variables|Default|GetLeftCube) (Variables|Default|GetRightCube) _alpha))))))

(event OnComponentEndOverlap(LeftTrigger)
  (params (OverlappedComponent :type Primitive%20Component%20Object%20Reference) (OtherActor :type Actor%20Object%20Reference) (OtherComp :type Primitive%20Component%20Object%20Reference) (OtherBodyIndex :type Integer))
  (Variables|Default|SetLeftmass (- (Physics|GetMass OverlappedComponent) (Variables|Default|GetLeftmass)))
  (bind (_to_lower _to_raise _is_equal_) (CallFunction|CheckMass))
  (Variables|Default|SetTo%20Lower _to_lower)
  (Variables|Default|SetTo%20Raise _to_raise)
  (bind _alpha (Timeline|Timeline PlayFromStart)
    (:Update
      (if (not _is_equal_)
        (CallFunction|Lower+Raise (Variables|Default|GetTo%20Lower) (Variables|Default|GetTo%20Raise) _alpha)
        (else
          (CallFunction|EvenOut (Variables|Default|GetLeftCube) (Variables|Default|GetRightCube) _alpha))))))

(event EventBeginPlay
  (bind _defaultsceneroot (Variables|Default|GetDefaultSceneRoot))
  (bind _returnvalue (Transformation|GetWorldLocation _defaultsceneroot))
  (Utilities|FlowControl|Sequence
    (:then_0
      (Variables|Default|SetTop%20Of%20Scale (.z (Variables|/Script/Engine.SceneComponent|GetRelativeLocation (Variables|Default|GetTop))))
      (Variables|Default|SetBottom%20Of%20Scale (.z (Variables|/Script/Engine.SceneComponent|GetRelativeLocation (Variables|Default|GetBottom))))
      (Variables|Default|SetLeft%20Middle (.z (Variables|/Script/Engine.SceneComponent|GetRelativeLocation (Variables|Default|GetLeftCube))))
      (Variables|Default|SetRight%20Middle (.z (Variables|/Script/Engine.SceneComponent|GetRelativeLocation (Variables|Default|GetRightCube)))))
    (:then_1
      (if (Variables|Default|GetLower%20After%20Spawn?)
        (Variables|Default|SetHeightAdjustment (.z (Transformation|GetWorldLocation (Variables|Default|GetLowerTo))))
        (bind _alpha (Timeline|Timeline_0 Play)
          (:Update
            (Transformation|SetWorldLocation _defaultsceneroot (Math|Vector|MakeVector (.x _returnvalue) (.y _returnvalue) (Math|Float|Lerp (.z _returnvalue) (Variables|Default|GetHeightAdjustment) _alpha)) false false)))))))

(fn ConstructionScript)

(fn CheckMass
  (if (> (Variables|Default|GetLeftmass) (Variables|Default|GetRightMass))
    (return (Variables|Default|GetLeftCube) (Variables|Default|GetRightCube) false)
    (elif (< (Variables|Default|GetLeftmass) (Variables|Default|GetRightMass))
      (return (Variables|Default|GetRightCube) (Variables|Default|GetLeftCube) false)
      (elif (== (Variables|Default|GetLeftmass) (Variables|Default|GetRightMass))
        (return (Variables|Default|GetRightCube) (Variables|Default|GetLeftCube) true)))))

(fn Lower+Raise
  (params (To%20Lower :type Scene%20Component%20Object%20Reference) (To%20Raise :type Scene%20Component%20Object%20Reference) (Alpha :type Float%20%28double-precision%29))
  (bind _relativelocation (Variables|/Script/Engine.SceneComponent|GetRelativeLocation To%20Lower))
  (bind _relativelocation_2 (Variables|/Script/Engine.SceneComponent|GetRelativeLocation To%20Raise))
  (Utilities|FlowControl|Sequence
    (:then_0
      (Transformation|SetRelativeLocation To%20Lower (Math|Vector|MakeVector (.x _relativelocation) (.y _relativelocation) (Math|Float|Lerp (.z _relativelocation) (Variables|Default|GetBottom%20Of%20Scale) Alpha)) false false))
    (:then_1
      (Transformation|SetRelativeLocation To%20Raise (Math|Vector|MakeVector (.x _relativelocation_2) (.y _relativelocation_2) (Math|Float|Lerp (.z _relativelocation_2) (Variables|Default|GetTop%20Of%20Scale) Alpha)) false false))))

(fn EvenOut
  (params (Left :type Scene%20Component%20Object%20Reference) (Right :type Scene%20Component%20Object%20Reference) (Alpha :type Float%20%28double-precision%29))
  (bind _relativelocation (Variables|/Script/Engine.SceneComponent|GetRelativeLocation Left))
  (bind _relativelocation_2 (Variables|/Script/Engine.SceneComponent|GetRelativeLocation Right))
  (Utilities|FlowControl|Sequence
    (:then_0
      (Transformation|SetRelativeLocation Left (Math|Vector|MakeVector (.x _relativelocation) (.y _relativelocation) (Math|Float|Lerp (.z _relativelocation) (Variables|Default|GetLeft%20Middle) Alpha)) false false))
    (:then_1
      (Transformation|SetRelativeLocation Right (Math|Vector|MakeVector (.x _relativelocation_2) (.y _relativelocation_2) (Math|Float|Lerp (.z _relativelocation_2) (Variables|Default|GetRight%20Middle) Alpha)) false false))))