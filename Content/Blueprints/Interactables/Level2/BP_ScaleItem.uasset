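; BP_ScaleItem is a Level 2 interactable physics item with a widget that shows while the player is inside its overlap sphere.
; Tick keeps the widget floating above the mesh in world space, and the PickedUp event hides it.
; A looping timer checks the mesh's distance from its start location and, if it strays too far, teleports it back, briefly disabling physics during the reset.
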(event OnComponentBeginOverlap(Sphere)
  (params (OverlappedComponent :type Primitive%20Component%20Object%20Reference) (OtherActor :type Actor%20Object%20Reference) (OtherComp :type Primitive%20Component%20Object%20Reference) (OtherBodyIndex :type Integer) (bFromSweep :type Boolean) (SweepResult :type Hit%20Result%20Structure%20%28by%20ref%29))
  (if (== OtherActor (Game|Player|GetPlayerPawn 0))
    (Rendering|SetVisibility (Variables|Default|GetWidget) true false)))

(event OnComponentEndOverlap(Sphere)
  (params (OverlappedComponent :type Primitive%20Component%20Object%20Reference) (OtherActor :type Actor%20Object%20Reference) (OtherComp :type Primitive%20Component%20Object%20Reference) (OtherBodyIndex :type Integer))
  (if (== OtherActor (Game|Player|GetPlayerPawn 0))
    (Rendering|SetVisibility (Variables|Default|GetWidget) false false)))

(event Custom|Check%20Distance
  (bind _staticmesh (Variables|Default|GetStaticMesh))
  (if (> (Math|Vector|Distance(Vector) (Transformation|GetWorldLocation (Variables|Default|GetStaticMesh)) (Variables|Default|GetStart%20Location)) 2.5e+03)
    (Physics|SetSimulatePhysics _staticmesh false)
    (Transformation|SetWorldLocation _staticmesh (Variables|Default|GetStart%20Location) false false)
    (Utilities|FlowControl|Delay 0.2)
    (Physics|SetSimulatePhysics _staticmesh true)))

(event Custom|Picked%20Up
  (Rendering|SetVisibility (Variables|Default|GetWidget) false false))

(event EventBeginPlay
  (Variables|Default|SetStart%20Location (Transformation|GetWorldLocation (Variables|Default|GetDefaultSceneRoot)))
  (Utilities|Time|SetTimerbyEvent (delegate Custom|Check%20Distance) 5.0 true))

(event EventTick
  (params (DeltaSeconds :type Float%20%28single-precision%29))
  (bind _staticmesh (Variables|Default|GetStaticMesh))
  (bind _returnvalue (Transformation|GetWorldLocation _staticmesh))
  (Transformation|SetWorldLocation (Variables|Default|GetWidget) (Math|Vector|MakeVector (.x _returnvalue) (.y _returnvalue) (+ (.z _returnvalue) 1e+02)) false false))

(fn ConstructionScript)