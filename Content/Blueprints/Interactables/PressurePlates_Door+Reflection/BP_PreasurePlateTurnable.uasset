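; Puzzle-driven turnable object that rotates its visual mesh in yaw once enough linked puzzles are active.
; Activate and Deactivate adjust a running count that is compared against the required number.
; Reaching the threshold plays a Timeline that sets the mesh's relative yaw, noted as a 90-degree turn.
; Deactivating below the threshold reverses the Timeline to turn it back.
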(event Custom|Activate
  (bind _puzzlesactive (Variables|Default|GetPuzzlesActive))
  ;[1 1 1] Turns 90 degrees then saves rotation
  (Math|Integer|IncrementInt _puzzlesactive
    (:%20%20
      (if (>= _puzzlesactive (Variables|Default|GetPuzzlesNeededToActivate))
        (bind _newtrack_0 (Timeline|Timeline Play)
          (:Update
            (Transformation|SetRelativeRotation (Variables|Default|GetSM_Visual) (Math|Rotator|MakeRotator 0.0 0.0 _newtrack_0) false false)))))))

(event Custom|Deactivate
  (bind _puzzlesactive (Variables|Default|GetPuzzlesActive))
  ;[1 1 1] Turns 90 degrees then saves rotation
  (Math|Integer|DecrementInt _puzzlesactive
    (:%20%20
      (if (not (>= _puzzlesactive (Variables|Default|GetPuzzlesNeededToActivate)))
        (bind _newtrack_0 (Timeline|Timeline Reverse)
          (:Update
            (Transformation|SetRelativeRotation (Variables|Default|GetSM_Visual) (Math|Rotator|MakeRotator 0.0 0.0 _newtrack_0) false false)))))))

(fn ConstructionScript
  (|CallParentFunction))