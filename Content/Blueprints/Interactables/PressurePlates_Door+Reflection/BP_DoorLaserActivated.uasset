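; A puzzle door that slides vertically when enough activations are registered, named for laser activation.
; On BeginPlay it binds to its target's puzzle-finished event, which increments an active count compared against a required threshold.
; A timeline drives the door's height forward or in reverse, with an attached sound during movement.
; A separate deactivation event, not bound here, decrements the count when allowed and re-evaluates the door.
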(event Custom|Switch%20Activated
  (bind _puzzles_active (Variables|Default|GetPuzzles%20Active))
  ;[1 1 1] Move door up and down on activate //Omar
  (Math|Integer|IncrementInt _puzzles_active
    (:%20%20
      (if (>= _puzzles_active (Variables|Default|GetPuzzles%20Completed%20to%20Open))
        (bind _returnvalue (Audio|SpawnSoundAttached (Variables|Default|GetSound) (Variables|Default|GetDoor) "None" "0, 0, 0" "0, 0, 0" "KeepRelativeOffset" false 0.5 1.0 0.0 0 0))
        (Variables|Default|SetAudioIsPlaying _returnvalue)
        (bind _doorpos (Timeline|Door%20Open Play)
          (:Update
            (Transformation|SetRelativeLocation (Variables|Default|GetDoor) (Math|Vector|MakeVector 0.0 0.0 _doorpos) false false))
          (:Finished
            (Audio|Components|Audio|Stop (Variables|Default|GetAudioIsPlaying))))
        (else
          (bind _returnvalue_2 (Audio|SpawnSoundAttached (Variables|Default|GetSound) (Variables|Default|GetDoor) "None" "0, 0, 0" "0, 0, 0" "KeepRelativeOffset" false 0.5 1.0 0.0 0 0))
          (Variables|Default|SetAudioIsPlaying _returnvalue_2)
          (Timeline|Door%20Open Reverse))))))

(event Custom|Switch%20Deativated
  (bind _puzzles_active (Variables|Default|GetPuzzles%20Active))
  ;[1 1 1] Move door up and down on activate //Omar
  (if (Variables|Default|GetCanDeactivate)
    (Math|Integer|DecrementInt _puzzles_active
      (:%20%20
        (if (>= _puzzles_active (Variables|Default|GetPuzzles%20Completed%20to%20Open))
          (bind _returnvalue (Audio|SpawnSoundAttached (Variables|Default|GetSound) (Variables|Default|GetDoor) "None" "0, 0, 0" "0, 0, 0" "KeepRelativeOffset" false 0.5 1.0 0.0 0 0))
          (Variables|Default|SetAudioIsPlaying _returnvalue)
          (bind _doorpos (Timeline|Door%20Open Play)
            (:Update
              (Transformation|SetRelativeLocation (Variables|Default|GetDoor) (Math|Vector|MakeVector 0.0 0.0 _doorpos) false false))
            (:Finished
              (Audio|Components|Audio|Stop (Variables|Default|GetAudioIsPlaying))))
          (else
            (bind _returnvalue_2 (Audio|SpawnSoundAttached (Variables|Default|GetSound) (Variables|Default|GetDoor) "None" "0, 0, 0" "0, 0, 0" "KeepRelativeOffset" false 0.5 1.0 0.0 0 0))
            (Variables|Default|SetAudioIsPlaying _returnvalue_2)
            (Timeline|Door%20Open Reverse)))))))

(event EventBeginPlay
  (EventDispatchers|BindEventtoPuzzleFinished (Variables|Default|GetTarget%20I%20need%20activated) (delegate Custom|Switch%20Activated)))

(fn ConstructionScript)