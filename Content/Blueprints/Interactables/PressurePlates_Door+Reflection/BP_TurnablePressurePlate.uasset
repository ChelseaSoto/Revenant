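; Turnable pressure plate actor that yaws its visual mesh in response to puzzle completion events, noted as 90-degree turns.
; OnPuzzleComplete and OnPuzzleIncomplete adjust an active-puzzle count and compare it to the required threshold.
; Each event plays or reverses its own timeline, one for each turn direction.
; Timeline updates add local yaw incrementally, negated for the incomplete event, rather than setting an absolute rotation.
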(event Custom|OnPuzzleComplete
  (bind _puzzles_active (Variables|Default|GetPuzzles%20Active))
  ;[1 1 1] Rotate 90 Degrees //Omar
  (Math|Integer|IncrementInt _puzzles_active
    (:%20%20
      (if (>= _puzzles_active (Variables|Default|GetPuzzles%20needed%20to%20activate))
        (bind _newtrack_0 (Timeline|Timeline Play)
          (:Update
            (Transformation|AddLocalRotation (Variables|Default|GetSM_Visual) (Math|Rotator|MakeRotator 0.0 0.0 _newtrack_0) false false)))
        (else
          (Timeline|Timeline Reverse))))))

(event Custom|OnPuzzleIncomplete
  (bind _puzzles_active (Variables|Default|GetPuzzles%20Active))
  ;[1 1 1] Rotate -90 Degrees //Omar
  (Math|Integer|DecrementInt _puzzles_active
    (:%20%20
      (if (>= _puzzles_active (Variables|Default|GetPuzzles%20needed%20to%20activate))
        (bind _newtrack_0 (Timeline|Timeline_0 Reverse)
          (:Update
            (Transformation|AddLocalRotation (Variables|Default|GetSM_Visual) (Math|Rotator|MakeRotator 0.0 0.0 (* _newtrack_0 -1.0)) false false)))
        (else
          (Timeline|Timeline_0 Play))))))

(event EventBeginPlay
  (|CallParentFunction) ; This node is disabled and will not be called.\nDrag off pins to build functionality.
)

(event Collision|EventActorBeginOverlap
  (params (OtherActor :type Actor%20Object%20Reference))
  (|CallParentFunction OtherActor) ; This node is disabled and will not be called.\nDrag off pins to build functionality.
)

(event EventTick
  (params (DeltaSeconds :type Float%20%28single-precision%29))
  (|CallParentFunction DeltaSeconds) ; This node is disabled and will not be called.\nDrag off pins to build functionality.
)

(fn ConstructionScript
  (|CallParentFunction))