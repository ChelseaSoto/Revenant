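; BP_DoorScale is a puzzle door that moves vertically according to whether a linked Scale reports equal.
; It binds to the Scale's dispatcher on BeginPlay, playing the DoorOpen timeline when equal and reversing it otherwise.
; The timeline drives the door's relative Z, while an attached sound and two sand-trickle effects start with the movement and stop when it finishes.
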(event Custom|Check%20if%20Equal
  (params (Is%20Equal? :type Boolean))
  ;[1 1 1] Move door up and down on activate //Omar
  (if Is%20Equal?
    (bind _returnvalue (Audio|SpawnSoundAttached 0 0 "None" "0, 0, 0" "0, 0, 0" "KeepRelativeOffset" false 0.5 1.0 0.0 "/Game/Audio/NewSoundAttenuation.NewSoundAttenuation" 0))
    (Variables|Default|SetAudioIsPlaying _returnvalue)
    (bind _doorpos (Timeline|Door%20Open Play)
      (:Update
        (Transformation|SetRelativeLocation (Variables|Default|GetDoor) (Math|Vector|MakeVector 0.0 0.0 _doorpos) false false)
        (Utilities|FlowControl|DoOnce false :!label _label
          (:Completed
            (Components|Activation|Activate (Variables|Default|GetNS_SandTrickle) false)
            (Components|Activation|Activate (Variables|Default|GetNS_SandTrickle1) false))))
      (:Finished
        (Components|DestroyComponent (Variables|Default|GetAudioIsPlaying))
        (Components|Activation|Deactivate (Variables|Default|GetNS_SandTrickle1))
        (Components|Activation|Deactivate (Variables|Default|GetNS_SandTrickle))
        (goto _label Reset)))
    (else
      (bind _returnvalue_2 (Audio|SpawnSoundAttached 0 0 "None" "0, 0, 0" "0, 0, 0" "SnapToTargetIncludingScale" false 0.5 1.0 0.0 "/Game/Audio/NewSoundAttenuation.NewSoundAttenuation" 0))
      (Variables|Default|SetAudioIsPlaying _returnvalue_2)
      (Timeline|Door%20Open Reverse))))

(event EventBeginPlay
  (EventDispatchers|BindEventtoDispatch (Variables|Default|GetScale) (delegate Custom|Check%20if%20Equal)))

(fn ConstructionScript)