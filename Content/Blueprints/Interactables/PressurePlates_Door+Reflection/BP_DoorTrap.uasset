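; Trap door that drops on the player's first overlap, enabling a collision box, with a sound and sand-trickle effects.
; One timeline lerps the door's height and plays in reverse to raise it, disabling the box.
; It raises when all listed enemies die or, in light-activation mode, when a linked puzzle finishes; that mode also resets it on player death.
; CanOpen raises it at BeginPlay and on later overlaps.
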(event Custom|Reset
  (bind _audioisplaying (Variables|Default|GetAudioIsPlaying))
  (bind _door (Variables|Default|GetDoor))
  (bind _relativelocation (Variables|/Script/Engine.SceneComponent|GetRelativeLocation _door))
  ;[1 1 1] Move door up and down on activate //Omar
  (Variables|Default|SethasActivated? false)
  (Collision|SetCollisionEnabled (Variables|Default|GetBox) "NoCollision")
  (bind _doorpos (Timeline|Door%20Open Reverse)
    (:Update
      (Transformation|SetRelativeLocation (Variables|Default|GetDoor) (Math|Vector|MakeVector (.x _relativelocation) (.y _relativelocation) (Math|Float|Lerp (Variables|Default|GetStart%20Position) (Variables|Default|GetLower%20Position) _doorpos)) false false))
    (:Finished
      (Utilities|IsValid _audioisplaying
        (:Is%20Valid
          (Audio|Components|Audio|Stop _audioisplaying))
        (:Is%20Not%20Valid
          _))
      (Components|Activation|Deactivate (Variables|Default|GetNS_SandTrickle))
      (Components|Activation|Deactivate (Variables|Default|GetNS_SandTrickle1))))
  (Utilities|FlowControl|DoOnce false
    (:Completed
      (Components|Activation|Activate (Variables|Default|GetNS_SandTrickle) false)
      (Components|Activation|Activate (Variables|Default|GetNS_SandTrickle1) false))))

(event Custom|DoorLower
  (bind _door (Variables|Default|GetDoor))
  (bind _relativelocation (Variables|/Script/Engine.SceneComponent|GetRelativeLocation _door))
  ;[1 1 1] Move door up and down on activate //Omar
  (Collision|SetCollisionEnabled (Variables|Default|GetBox) "QueryAndPhysics")
  (bind _returnvalue (Audio|SpawnSoundAttached (Variables|Default|GetSound) (Variables|Default|GetDoor) "None" "0, 0, 0" "0, 0, 0" "KeepRelativeOffset" false 0.5 1.0 0.0 0 0))
  (Variables|Default|SetAudioIsPlaying _returnvalue)
  (bind _doorpos (Timeline|Door%20Open Play)
    (:Update
      (Transformation|SetRelativeLocation (Variables|Default|GetDoor) (Math|Vector|MakeVector (.x _relativelocation) (.y _relativelocation) (Math|Float|Lerp (Variables|Default|GetStart%20Position) (Variables|Default|GetLower%20Position) _doorpos)) false false))
    (:Finished
      (Utilities|IsValid (Variables|Default|GetAudioIsPlaying)
        (:Is%20Valid
          (Audio|Components|Audio|Stop (Variables|Default|GetAudioIsPlaying)))
        (:Is%20Not%20Valid
          _))
      (Components|Activation|Deactivate (Variables|Default|GetNS_SandTrickle))
      (Components|Activation|Deactivate (Variables|Default|GetNS_SandTrickle1))))
  (Utilities|FlowControl|DoOnce false
    (:Completed
      (Components|Activation|Activate (Variables|Default|GetNS_SandTrickle) false)
      (Components|Activation|Activate (Variables|Default|GetNS_SandTrickle1) false))))

(event Custom|DoorRaise
  (bind _door (Variables|Default|GetDoor))
  (bind _relativelocation (Variables|/Script/Engine.SceneComponent|GetRelativeLocation _door))
  ;[1 1 1] Move door up and down on activate //Omar
  (bind _returnvalue (Audio|SpawnSoundAttached (Variables|Default|GetSound) (Variables|Default|GetDoor) "None" "0, 0, 0" "0, 0, 0" "KeepRelativeOffset" false 1.0 1.0 0.0 0 0))
  (Variables|Default|SetAudioIsPlaying _returnvalue)
  (Variables|Default|SethasActivated? true)
  (Collision|SetCollisionEnabled (Variables|Default|GetBox) "NoCollision")
  (bind _doorpos (Timeline|Door%20Open Reverse)
    (:Update
      (Transformation|SetRelativeLocation (Variables|Default|GetDoor) (Math|Vector|MakeVector (.x _relativelocation) (.y _relativelocation) (Math|Float|Lerp (Variables|Default|GetStart%20Position) (Variables|Default|GetLower%20Position) _doorpos)) false false))
    (:Finished
      (Utilities|IsValid (Variables|Default|GetAudioIsPlaying)
        (:Is%20Valid
          (Audio|Components|Audio|Stop (Variables|Default|GetAudioIsPlaying)))
        (:Is%20Not%20Valid
          _))
      (Components|Activation|Deactivate (Variables|Default|GetNS_SandTrickle))
      (Components|Activation|Deactivate (Variables|Default|GetNS_SandTrickle1))))
  (Utilities|FlowControl|DoOnce false
    (:Completed
      (Components|Activation|Activate (Variables|Default|GetNS_SandTrickle) false)
      (Components|Activation|Activate (Variables|Default|GetNS_SandTrickle1) false))))

(event Custom|EnemyDeath
  ;[1 1 1] Check If I got the amount of enemies I needed to kill to open //Omar
  (bind _result (Math|Integer|IncrementInt (Variables|Conditions|GetEnemiesKilled))
    (:%20%20
      (if (>= _result (Utilities|Array|Length (Variables|Conditions|GetEnemiesNeeded)))
        (CallFunction|DoorRaise)))))

(event EventBeginPlay
  (bind _start_location (Variables|Default|GetStart%20Location))
  (bind _door (Variables|Default|GetDoor))
  (bind _door_2 (Variables|Default|GetDoor))
  (bind _relativelocation (Variables|/Script/Engine.SceneComponent|GetRelativeLocation _door))
  (bind _relativelocation_2 (Variables|/Script/Engine.SceneComponent|GetRelativeLocation _start_location))
  (bind _relativelocation_3 (Variables|/Script/Engine.SceneComponent|GetRelativeLocation _door_2))
  (Collision|SetCollisionEnabled (Variables|Default|GetBox) "NoCollision")
  (Utilities|FlowControl|Sequence
    (:then_0
      ;[1 1 1] Check If I got the amount of enemies I needed to kill to open //Omar
      (if (Variables|Conditions|GetuseEnemies?)
        (for _array_element (Variables|Conditions|GetEnemiesNeeded)
          (EventDispatchers|BindEventtoDeathDispatch _array_element (delegate Custom|EnemyDeath)))
        (elif (Variables|Conditions|GetuseLightActivation?)
          (EventDispatchers|BindEventtoPuzzleFinished (Variables|Conditions|GetLasterNeeded) (delegate Custom|DoorRaise))
          (bind _asbp_third_person_character (Utilities|Casting|CastToBP_ThirdPersonCharacter (Game|Player|GetPlayerPawn 0)))
          (EventDispatchers|BindEventtoPlayerDied! _asbp_third_person_character (delegate Custom|Reset)))))
    (:then_1
      (Variables|Default|SetLower%20Position (.z _relativelocation_3))
      (bind _output_get (Variables|Default|SetStart%20Position (.z _relativelocation_2)))
      (if (Variables|Default|GetcanOpen?)
        (CallFunction|DoorRaise)
        (Components|MoveComponentTo (Variables|Default|GetDoor) (Math|Vector|MakeVector (.x _relativelocation) (.y _relativelocation) _output_get) (Variables|/Script/Engine.SceneComponent|GetRelativeRotation _door) false false 5.0 false)
        (else
          (Transformation|SetRelativeLocation (Variables|Default|GetDoor) (Math|Vector|MakeVector (.x _relativelocation_3) (.y _relativelocation_3) (.z _relativelocation_2)) false true))))))

(event Collision|EventActorBeginOverlap
  (params (OtherActor :type Actor%20Object%20Reference))
  ;[1 1 1] Lower Door for Collision
  (if (== OtherActor (Game|Player|GetPlayerPawn 0))
    (if (Variables|Default|GethasActivated?)
      (if (Variables|Default|GetcanOpen?)
        (CallFunction|DoorRaise))
      (else
        (CallFunction|DoorLower)
        (Variables|Default|SethasActivated? true)))))

(fn ConstructionScript)