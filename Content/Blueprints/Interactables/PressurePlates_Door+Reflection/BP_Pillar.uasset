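; BP_Pillar is a door-like interactable that slides vertically once enough puzzle switches are active.
; Switch activate and deactivate events adjust a counter, with decrements gated by CanDeactivate, then compare it to a threshold.
; The DoorOpen timeline plays or reverses accordingly, driving the Door's relative Z, with IsReverse choosing direction.
; An attached sound accompanies movement, and two Niagara sand trickles start once per run through a DoOnce, stopping on finish.
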(event Custom|Switch%20Activated
  (bind _puzzles_active (Variables|Default|GetPuzzles%20Active))
  ;[1 1 1] Move door up and down on activate //Omar
  (Math|Integer|IncrementInt _puzzles_active
    (:%20%20
      (if (>= _puzzles_active (Variables|Default|GetPuzzles%20Completed%20to%20Open))
        (bind _returnvalue (Audio|SpawnSoundAttached (Variables|Default|GetSound) (Variables|Default|GetDoor) "None" "0, 0, 0" "0, 0, 0" "KeepRelativeOffset" false 0.5 1.0 0.0 0 0))
        (Variables|Default|SetAudioIsPlaying _returnvalue)
        (bind _doorpos (Timeline|Door%20Open Play)
          (:Update
            (if (Variables|Default|GetisReverse)
              (Transformation|SetRelativeLocation (Variables|Default|GetDoor) (Math|Vector|MakeVector 0.0 0.0 _doorpos) false false)
              (else
                (Transformation|SetRelativeLocation (Variables|Default|GetDoor) (Math|Vector|MakeVector 0.0 0.0 (* _doorpos -1.0)) false false)))
            (Utilities|FlowControl|DoOnce false :!label _label
              (:Completed
                (Components|Activation|Activate (Variables|Default|GetNS_SandTrickle) false)
                (Components|Activation|Activate (Variables|Default|GetNS_SandTrickle1) false))))
          (:Finished
            (Audio|Components|Audio|Stop (Variables|Default|GetAudioIsPlaying))
            (Components|Activation|Deactivate (Variables|Default|GetNS_SandTrickle))
            (Components|Activation|Deactivate (Variables|Default|GetNS_SandTrickle1))
            (goto _label Reset)))
        (else
          (bind _returnvalue_2 (Audio|SpawnSoundAttached (Variables|Default|GetSound) (Variables|Default|GetDoor) "None" "0, 0, 0" "0, 0, 0" "KeepRelativeOffset" false 0.5 1.0 0.0 0 0))
          (Variables|Default|SetAudioIsPlaying _returnvalue_2)
          (Timeline|Door%20Open Reverse))))))

(event Custom|Switch%20Deativated
  (bind _puzzles_active (Variables|Default|GetPuzzles%20Active))
  ;[1 1 1] Move door up and down on activate //Omar
  (if (Variables|Default|GetCanDeactivate)
    (Math|Integer|DecrementInt _puzzles_active
      (:%20%20
        (if (>= _puzzles_active (Variables|Default|GetPuzzles%20Completed%20to%20Open))
          (bind _returnvalue (Audio|SpawnSoundAttached (Variables|Default|GetSound) (Variables|Default|GetDoor) "None" "0, 0, 0" "0, 0, 0" "KeepRelativeOffset" false 0.5 1.0 0.0 0 0))
          (Variables|Default|SetAudioIsPlaying _returnvalue)
          (bind _doorpos (Timeline|Door%20Open Play)
            (:Update
              (if (Variables|Default|GetisReverse)
                (Transformation|SetRelativeLocation (Variables|Default|GetDoor) (Math|Vector|MakeVector 0.0 0.0 _doorpos) false false)
                (else
                  (Transformation|SetRelativeLocation (Variables|Default|GetDoor) (Math|Vector|MakeVector 0.0 0.0 (* _doorpos -1.0)) false false)))
              (Utilities|FlowControl|DoOnce false :!label _label
                (:Completed
                  (Components|Activation|Activate (Variables|Default|GetNS_SandTrickle) false)
                  (Components|Activation|Activate (Variables|Default|GetNS_SandTrickle1) false))))
            (:Finished
              (Audio|Components|Audio|Stop (Variables|Default|GetAudioIsPlaying))
              (Components|Activation|Deactivate (Variables|Default|GetNS_SandTrickle))
              (Components|Activation|Deactivate (Variables|Default|GetNS_SandTrickle1))
              (goto _label Reset)))
          (else
            (bind _returnvalue_2 (Audio|SpawnSoundAttached (Variables|Default|GetSound) (Variables|Default|GetDoor) "None" "0, 0, 0" "0, 0, 0" "KeepRelativeOffset" false 0.5 1.0 0.0 0 0))
            (Variables|Default|SetAudioIsPlaying _returnvalue_2)
            (Timeline|Door%20Open Reverse)))))))

(event EventBeginPlay)

(event Collision|EventActorBeginOverlap
  (params (OtherActor :type Actor%20Object%20Reference)))

(event EventTick
  (params (DeltaSeconds :type Float%20%28single-precision%29)))

(fn ConstructionScript)