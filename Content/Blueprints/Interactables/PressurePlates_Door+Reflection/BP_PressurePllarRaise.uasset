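; Pressure plate actor that raises or otherwise switches its linked pillars when an actor steps on or off it.
; Overlap begin calls SwitchActivated on each actor in PillarToMove, and overlap end calls SwitchDeativated, with no count of overlapping actors.
; The SwitchActivate timeline, triggered inside each loop, moves the Switch component along local Z and reverses on exit.
; Actors whose display name contains "TestEnemy" are ignored.
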(event Collision|EventActorBeginOverlap
  (params (OtherActor :type Actor%20Object%20Reference))
  (if (not (Utilities|String|Contains (Utilities|GetDisplayName OtherActor) "TestEnemy"))
    (for _array_element (Variables|Default|GetPillar%20To%20move)
      (Default|SwitchActivated _array_element)
      (bind _switch_pos (Timeline|SwitchActivate Play)
        (:Update
          (Transformation|SetRelativeLocation (Variables|Default|GetSwitch) (Math|Vector|MakeVector 0.0 0.0 _switch_pos) false false))))))

(event Collision|EventActorEndOverlap
  (params (OtherActor :type Actor%20Object%20Reference))
  (if (not (Utilities|String|Contains (Utilities|GetDisplayName OtherActor) "TestEnemy"))
    (for _array_element (Variables|Default|GetPillar%20To%20move)
      (Default|SwitchDeativated _array_element)
      (bind _switch_pos (Timeline|SwitchActivate Reverse)
        (:Update
          (Transformation|SetRelativeLocation (Variables|Default|GetSwitch) (Math|Vector|MakeVector 0.0 0.0 _switch_pos) false false))))))

(fn ConstructionScript)