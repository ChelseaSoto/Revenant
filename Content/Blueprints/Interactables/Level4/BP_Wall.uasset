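; BP_Wall is a Level 4 interactable that hides itself in game on BeginPlay and serves as an overlap zone for the interact prompt.
; When the player character begins overlapping, it creates a P_Interact widget, passing the player's UsingGamepad state, and adds it to the viewport.
; Ending the overlap removes that widget; the graph contains no interaction logic beyond the prompt.
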(event EventBeginPlay
  (Rendering|SetActorHiddenInGame true))

(event Collision|EventActorBeginOverlap
  (params (OtherActor :type Actor%20Object%20Reference))
  (bind _my_player_character (CallFunction|GetMyPlayerCharacter))
  (if (== OtherActor _my_player_character)
    (bind _returnvalue (UserInterface|CreateWidget "/Game/UI/P_Interact.P_Interact_C" 0 (Variables|/Game/ThirdPerson/Blueprints/BP_ThirdPersonCharacter.BP_ThirdPersonCharacter_C|GetUsingGamepad _my_player_character)))
    (UserInterface|Viewport|AddtoViewport _returnvalue 0)))

(event Collision|EventActorEndOverlap
  (params (OtherActor :type Actor%20Object%20Reference))
  (if (== OtherActor (Game|GetPlayerCharacter 0))
    (Widget|RemovefromParent (stale Collision|EventActorBeginOverlap _returnvalue))))

(fn ConstructionScript)