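; BP_Switch_Book is a book-themed switch interactable that highlights its mesh while an actor overlaps it.
; Begin overlap runs the parent handler, then applies M_OverlayMat as an overlay material on the static mesh.
; End overlap clears the overlay without calling the parent handler.
; The Blueprint adds no switch logic of its own, and its construction script only calls the parent.
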(event EventBeginPlay
  (|CallParentFunction) ; This node is disabled and will not be called.\nDrag off pins to build functionality.
)

(event Collision|EventActorBeginOverlap
  (params (OtherActor :type Actor%20Object%20Reference))
  (|CallParentFunction OtherActor)
  (Rendering|Material|SetOverlayMaterial (Variables|Default|GetStaticMesh) "/Game/Materials/M_OverlayMat.M_OverlayMat" :!class /Script/Engine.MeshComponent))

(event EventTick
  (params (DeltaSeconds :type Float%20%28single-precision%29))
  (|CallParentFunction DeltaSeconds) ; This node is disabled and will not be called.\nDrag off pins to build functionality.
)

(event Collision|EventActorEndOverlap
  (params (OtherActor :type Actor%20Object%20Reference))
  (Rendering|Material|SetOverlayMaterial (Variables|Default|GetStaticMesh) 0 :!class /Script/Engine.MeshComponent))

(fn ConstructionScript
  (|CallParentFunction))