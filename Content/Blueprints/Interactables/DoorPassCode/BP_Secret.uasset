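; BP_Secret is a passcode-locked obstacle, likely a secret door, that disappears when the correct code is entered.
; On BeginPlay it binds to the activate event of a referenced button puzzle, which passes in a value per press.
; Each value is appended to an input string and compared to the correct password; a match destroys the actor, while a full-length mismatch clears the input.
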(event Custom|CustomEvent
  (params (button%20puzzle%20Value%20ABC :type String))
  (bind _output_get (Variables|Default|SetInput (Utilities|String|Append (Variables|Default|GetInput) button%20puzzle%20Value%20ABC)))
  (if (Utilities|Enum|Equal(Enum) _output_get (Variables|Default|GetCorrectPassWord))
    (Actor|DestroyActor)
    (elif (>= (Utilities|String|Len (Variables|Default|GetInput)) (Utilities|String|Len (Variables|Default|GetCorrectPassWord)))
      (Variables|Default|SetInput ""))))

(event EventBeginPlay
  (EventDispatchers|BindEventtoActivate (Variables|Default|GetPuzzle%20Ref) (delegate Custom|CustomEvent)))

(fn ConstructionScript)