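; Level 1 passcode door that opens the way to the Level 2 unlock.
; It binds to every puzzle switch's activate event, appends their values to an input string, and resets a full-length wrong entry.
; A correct code enables the trigger box's overlap events and shows a point light.
; The player character overlapping it then writes a newly created save object to slot1 with Level 2 unlocked.
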(event Custom|Add%20to%20puzzle
  (params (button%20puzzle%20Value%20ABC :type String))
  ;[1 1 1] Level 1 puzzle //Omar
  (bind _output_get (Variables|Default|SetInput (Utilities|AddtoPassword button%20puzzle%20Value%20ABC)))
  (if (Utilities|DoesInputMatchPassword? _output_get)
    (CallFunction|EnableTrigger)
    (else
      (Development|PrintString (Variables|Default|GetInput))
      (Development|PrintString (Variables|Default|GetCorrectPassWord))
      (CallFunction|ResetInputifLongerThan3))))

(event EventBeginPlay
  (|CallParentFunction)
  ;[1 1 1] Gets Input From puzzle buttons //Omar
  (bind _outactors (Actor|GetAllActorsOfClass "/Game/Blueprints/Interactables/DoorPassCode/BP_Level1PuzzleSwitch.BP_Level1PuzzleSwitch_C"))
  (bind _output_get (Variables|Default|SetPuzzle%20Ref _outactors))
  (EventDispatchers|BindEventtoActivate _output_get (delegate Custom|Add%20to%20puzzle)))

(event Collision|EventActorBeginOverlap
  (params (OtherActor :type Actor%20Object%20Reference))
  ;[1 1 1] unlocks level 2 save stats //Omar
  (Utilities|Casting|CastToBP_ThirdPersonCharacter OtherActor)
  (bind _returnvalue (SaveGame|CreateSaveGameObject "/Game/Savegame/BPC_levellock.BPC_levellock_C"))
  (Variables|/Game/Savegame/BPC_levellock.BPC_levellock_C|SetLevel2%20Unlock _returnvalue true)
  (SaveGame|SaveGametoSlot _returnvalue "slot1"))

(event EventTick
  (params (DeltaSeconds :type Float%20%28single-precision%29))
  (|CallParentFunction DeltaSeconds))

(fn ConstructionScript
  (|CallParentFunction))

(fn ResetInputifLongerThan3
  (if (>= (Utilities|String|Len (Variables|Default|GetInput)) (Utilities|String|Len (Variables|Default|GetCorrectPassWord)))
    (Variables|Default|SetInput "")
    (Development|PrintString "Wrong try again!")))

(fn NewFunction
  (params (B :type String))
  (Variables|Default|SetInput (Utilities|String|Append (Variables|Default|GetInput) B)))

(fn EnableTrigger
  (Variables|/Script/Engine.PrimitiveComponent|SetbGenerateOverlapEvents (Variables|Default|GetBox) true)
  (Rendering|SetVisibility (Variables|Default|GetPointLight) true false))