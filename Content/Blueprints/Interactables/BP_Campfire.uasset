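; BP_Campfire is an interactable checkpoint that sets the player's respawn position, refills potions and restores health.
; Interact fires PlayerInteract and reports progress to the quest objective matching its QuestID.
; A DoOnce with a five-second delay throttles the rest effect while toggling the Hieroglyphics visibility as feedback.
; A sphere overlap shows and removes a gamepad-aware interact prompt for the player.
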(event OnComponentBeginOverlap(Sphere)
  (params (OverlappedComponent :type Primitive%20Component%20Object%20Reference) (OtherActor :type Actor%20Object%20Reference) (OtherComp :type Primitive%20Component%20Object%20Reference) (OtherBodyIndex :type Integer) (bFromSweep :type Boolean) (SweepResult :type Hit%20Result%20Structure%20%28by%20ref%29))
  (bind _returnvalue (Game|GetPlayerCharacter 0))
  (bind _returnvalue_2 (== OtherActor _returnvalue))
  (if _returnvalue_2
    (bind _returnvalue_3 (UserInterface|CreateWidget "/Game/UI/P_Interact.P_Interact_C" 0 (Variables|/Game/ThirdPerson/Blueprints/BP_ThirdPersonCharacter.BP_ThirdPersonCharacter_C|GetUsingGamepad (CallFunction|GetMyPlayerCharacter))))
    (Variables|Default|SetInteractPrompt _returnvalue_3)
    (if _returnvalue_2
      (UserInterface|Viewport|AddtoViewport (Variables|Default|GetInteractPrompt) 0))))

(event OnComponentEndOverlap(Sphere)
  (params (OverlappedComponent :type Primitive%20Component%20Object%20Reference) (OtherActor :type Actor%20Object%20Reference) (OtherComp :type Primitive%20Component%20Object%20Reference) (OtherBodyIndex :type Integer))
  (if (== (Game|GetPlayerCharacter 0) OtherActor)
    (Widget|RemovefromParent (Variables|Default|GetInteractPrompt))))

(event Custom|Player%20Interact
  (bind _hieroglyphics (Variables|Default|GetHieroglyphics))
  ;[1 1 1] Sets this campfire to the player's respawn point, fills their potions to the max amount, and resets health to full //Julian
  (Utilities|FlowControl|DoOnce false :!label _label
    (:Completed
      (bind _asbp_third_person_character (Utilities|Casting|CastToBP_ThirdPersonCharacter (Game|GetPlayerCharacter 0)))
      (Variables|/Game/ThirdPerson/Blueprints/BP_ThirdPersonCharacter.BP_ThirdPersonCharacter_C|SetCampfirePosition _asbp_third_person_character (Transformation|GetWorldLocation (Variables|Default|GetRespawnPoint)))
      (Variables|/Game/ThirdPerson/Blueprints/BP_ThirdPersonCharacter.BP_ThirdPersonCharacter_C|SetPotionAmount _asbp_third_person_character (Variables|Default|GetMaxPotions))
      (Variables|/Game/ThirdPerson/Blueprints/BP_ThirdPersonCharacter.BP_ThirdPersonCharacter_C|SetHealth _asbp_third_person_character 1e+02)
      (Variables|/Game/ThirdPerson/Blueprints/BP_ThirdPersonCharacter.BP_ThirdPersonCharacter_C|SetHasUsedCampfire _asbp_third_person_character true)
      (Variables|/Game/ThirdPerson/Blueprints/BP_ThirdPersonCharacter.BP_ThirdPersonCharacter_C|SetLastUsedCampfire _asbp_third_person_character self)
      (Rendering|ToggleVisibility _hieroglyphics false)
      (Utilities|FlowControl|Delay 5.0)
      (Rendering|ToggleVisibility _hieroglyphics false)
      (goto _label Reset))))

(fn ConstructionScript)

(fn Interact
  (CallFunction|PlayerInteract)
  (Default|CallOnObjectIDCalled (CallFunction|GetMyPlayerCharacter) (Variables|Default|GetQuestID) 1)
  (return ""))