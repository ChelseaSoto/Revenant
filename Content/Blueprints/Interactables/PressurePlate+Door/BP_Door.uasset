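; BP_Door is a puzzle door that opens once enough switches, such as its companion pressure plates, are active.
; SwitchActivated and SwitchDeativated events raise and lower an active count, then compare it to PuzzlesCompletedToOpen.
; Meeting the threshold plays the DoorOpen timeline, which drives the door's relative Z location; falling short reverses it to close the door.
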(event Custom|Switch%20Activated
  (bind _puzzles_active (Variables|Default|GetPuzzles%20Active))
  (Math|Integer|IncrementInt _puzzles_active
    (:%20%20
      (if (>= _puzzles_active (Variables|Default|GetPuzzles%20Completed%20to%20Open))
        (bind _doorpos (Timeline|Door%20Open Play)
          (:Update
            (Transformation|SetRelativeLocation (Variables|Default|GetDoor) (Math|Vector|MakeVector 0.0 0.0 _doorpos) false false)))
        (else
          (Timeline|Door%20Open Reverse))))))

(event Custom|Switch%20Deativated
  (bind _puzzles_active (Variables|Default|GetPuzzles%20Active))
  (Math|Integer|DecrementInt _puzzles_active
    (:%20%20
      (if (>= _puzzles_active (Variables|Default|GetPuzzles%20Completed%20to%20Open))
        (bind _doorpos (Timeline|Door%20Open Play)
          (:Update
            (Transformation|SetRelativeLocation (Variables|Default|GetDoor) (Math|Vector|MakeVector 0.0 0.0 _doorpos) false false)))
        (else
          (Timeline|Door%20Open Reverse))))))

(event EventBeginPlay)

(event Collision|EventActorBeginOverlap
  (params (OtherActor :type Actor%20Object%20Reference)))

(event EventTick
  (params (DeltaSeconds :type Float%20%28single-precision%29)))

(fn ConstructionScript)