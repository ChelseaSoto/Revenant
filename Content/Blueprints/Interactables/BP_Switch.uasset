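; BP_Switch is an interactable switch actor that can enable or disable another actor passed to it.
; Any actor overlap applies an overlay material to its mesh as a highlight, cleared when an overlap ends.
; DisableActor and EnableActor toggle the target's collision, hidden-in-game state and root visibility, setting IsActive true on disable and false on enable.
; Neither function is called within this Blueprint.
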(event Collision|EventActorBeginOverlap
  (params (OtherActor :type Actor%20Object%20Reference))
  ;[1 1 1] Object outline//Omar
  (Rendering|Material|SetOverlayMaterial (Variables|Default|GetStaticMesh) "/Game/Materials/M_OverlayMat.M_OverlayMat" :!class /Script/Engine.MeshComponent))

(event EventTick
  (params (DeltaSeconds :type Float%20%28single-precision%29)))

(event Collision|EventActorEndOverlap
  (params (OtherActor :type Actor%20Object%20Reference))
  ;[1 1 1] Object outline//Omar
  (Rendering|Material|SetOverlayMaterial (Variables|Default|GetStaticMesh) 0 :!class /Script/Engine.MeshComponent))

(fn ConstructionScript)

(fn DisableActor
  (params (InputPin :type Actor%20Object%20Reference))
  (bind _output_get (Variables|Default|SetisActive true))
  (Rendering|SetVisibility (Variables|/Script/Engine.Actor|GetRootComponent InputPin) _output_get true)
  (Collision|SetActorEnableCollision InputPin false)
  (Rendering|SetActorHiddenInGame InputPin true))

(fn EnableActor
  (params (Target :type Actor%20Object%20Reference))
  (Variables|Default|SetisActive false)
  (Rendering|SetVisibility (Variables|/Script/Engine.Actor|GetRootComponent Target) false false)
  (Collision|SetActorEnableCollision Target true)
  (Rendering|SetActorHiddenInGame Target false))