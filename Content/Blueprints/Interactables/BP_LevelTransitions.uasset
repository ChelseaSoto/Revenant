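; Level transition trigger that moves the player to the level named in LevelToTransitionTo when their pawn overlaps its box.
; On overlap it reports hubPortal objective progress, fades the camera to full, ignores move input and waits out the fade.
; It then sets a display movie index based on the destination name and opens that level.
; A separate Givemission event calls Interact on the quest giver component and prints a debug greeting.
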(event OnComponentBeginOverlap(Box)
  (params (OverlappedComponent :type Primitive%20Component%20Object%20Reference) (OtherActor :type Actor%20Object%20Reference) (OtherComp :type Primitive%20Component%20Object%20Reference) (OtherBodyIndex :type Integer) (bFromSweep :type Boolean) (SweepResult :type Hit%20Result%20Structure%20%28by%20ref%29))
  (bind _duration (Variables|Default|GetDuration))
  (if (== OtherActor (Game|Player|GetPlayerPawn 0))
    ;[1 1 1] Simple Level Transition //Omar (Will Update)
    (Default|CallOnObjectIDCalled (CallFunction|GetMyPlayerCharacter) "hubPortal" 1)
    (CameraFades|StartCameraFade :self (Game|GetPlayerCameraManager 0) :ToAlpha 1.0 :Duration _duration :bHoldWhenFinished true)
    (Input|SetIgnoreMoveInput (Game|GetPlayerController 0) true)
    (Utilities|FlowControl|Delay _duration)
    (switch name (Variables|Default|GetLevel%20To%20Transition%20To)
      (:Default
        (Class|AsyncLoadingScreenLibrary|SetDisplayMovieIndex :!label _label))
      (:TutorialWorld
        (goto _label))
      (:Hub
        (Class|AsyncLoadingScreenLibrary|SetDisplayMovieIndex 1 :!label _label_2))
      (:Maze
        (goto _label_2))
      (:CourthouseNew
        (Class|AsyncLoadingScreenLibrary|SetDisplayMovieIndex 2))
      (:FieldOfReeds
        (Class|AsyncLoadingScreenLibrary|SetDisplayMovieIndex 3 :!label _label_3))
      (:LVL4
        (goto _label_3)))
    (Game|OpenLevel(byName) (Variables|Default|GetLevel%20To%20Transition%20To))))

(event Custom|Give%20mission
  (Default|Interact (Variables|Default|GetBPC_QuestGiver))
  (Development|PrintString "Hello"))

(fn ConstructionScript)