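; Spinning statue puzzle piece that counts toward opening a connected door when stopped facing the correct direction.
; A rotating movement component spins the statue, and Tick shows a Niagara effect while the current aim is within tolerance of the target rotation.
; TimeStop halts movement: an aligned statue completes once, increments the door's count and destroys its movement component, while a misaligned one re-assigns it after a delay.
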(event EventBeginPlay
  (Components|Movement|SetUpdatedComponent (Variables|Default|GetRotatingMovement) (Variables|Default|GetStatue)))

(event EventTick
  (params (DeltaSeconds :type Float%20%28single-precision%29))
  (if (Utilities|Operators|EqualEqual (Transformation|GetWorldRotation (Variables|Default|GetCurrentAim)) (Transformation|GetWorldRotation (Variables|Default|GetCorrect%20Aim)) 3e+01)
    (Rendering|SetVisibility (Variables|Default|GetNiagara) true false)
    (else
      (Rendering|SetVisibility (Variables|Default|GetNiagara) false false))))

(event EventTimeStop
  (bind _rotatingmovement (Variables|Default|GetRotatingMovement))
  (bind _doorconnected (Variables|Default|GetDoorConnected))
  (if (or (Utilities|Operators|EqualEqual (Transformation|GetWorldRotation (Variables|Default|GetCurrentAim)) (Transformation|GetWorldRotation (Variables|Default|GetCorrect%20Aim)) 3e+01) (Variables|Default|GetisComplete))
    (Components|Movement|StopMovementImmediately (Variables|Default|GetRotatingMovement))
    (Variables|Default|SetisComplete true)
    (Utilities|FlowControl|DoOnce false
      (:Completed
        (bind _result (Math|Integer|IncrementInt (Variables|/Game/Blueprints/Interactables/Statues/BP_StatueDoor.BP_StatueDoor_C|GetStatuesCurrent _doorconnected))
          (:%20%20
            (Variables|/Game/Blueprints/Interactables/Statues/BP_StatueDoor.BP_StatueDoor_C|SetStatuesCurrent _doorconnected _result)
            (Default|CheckStatues _doorconnected)
            (Components|DestroyComponent (Variables|Default|GetRotatingMovement))))))
    (else
      (Variables|Default|SetisComplete false)
      (Components|Movement|StopMovementImmediately _rotatingmovement)
      (Utilities|FlowControl|Delay 3.0)
      (if (not (Variables|Default|GetisComplete))
        (Components|Movement|SetUpdatedComponent _rotatingmovement (Variables|Default|GetStatue))))))

(fn ConstructionScript)