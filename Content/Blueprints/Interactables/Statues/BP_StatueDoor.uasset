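; BP_StatueDoor is a puzzle door that opens once enough statues are counted.
; CheckStatues compares the current count to the required one; on success it runs once, moving water and door to marker positions, spawning from linked enemy spawners and calling Completed.
; Below the threshold, it moves the door back to the start transform cached on BeginPlay.
; The statue count is not changed within this Blueprint.
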(event Custom|CheckStatues
  (bind _door (Variables|Default|GetDoor))
  (bind _water (Variables|Default|GetWater))
  (bind _door_2 (Variables|Default|GetDoor))
  (if (>= (Variables|Default|GetStatuesCurrent) (Variables|Default|GetStatuesNeeded))
    (Utilities|FlowControl|DoOnce false
      (:Completed
        (Components|MoveComponentTo _water (Variables|/Script/Engine.SceneComponent|GetRelativeLocation (Variables|Default|GetWater%20Arrow)) (Variables|/Script/Engine.SceneComponent|GetRelativeRotation _water) false false 4.0 false)
        (Components|MoveComponentTo _door_2 (Variables|/Script/Engine.SceneComponent|GetRelativeLocation (Variables|Default|GetMoveToLocation)) (Variables|/Script/Engine.SceneComponent|GetRelativeRotation _door_2) false false 2.0 false)
        (for _array_element (Variables|Default|GetEnemySpawn)
          (Default|Spawn _array_element))
        (Default|CallCompleted!)))
    (else
      (Components|MoveComponentTo _door (.location (Variables|Default|GetStart%20Location)) (Variables|/Script/Engine.SceneComponent|GetRelativeRotation _door) false false 2.0 false))))

(event EventBeginPlay
  (Variables|Default|SetStart%20Location (Transformation|GetRelativeTransform (Variables|Default|GetDoor))))

(fn ConstructionScript)