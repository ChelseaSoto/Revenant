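; Puzzle statue that the player turns in eased 90-degree steps through Interact, linked to a connected door.
; After each turn, two arrows' world rotations are compared within a tolerance.
; A match shows water, marks completion, increments the door's statue count and rechecks it; a mismatch hides water, touching the count only when already zero.
; A sphere overlap shows and removes the interact prompt widget.
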(event OnComponentBeginOverlap(Sphere)
  (params (OverlappedComponent :type Primitive%20Component%20Object%20Reference) (OtherActor :type Actor%20Object%20Reference) (OtherComp :type Primitive%20Component%20Object%20Reference) (OtherBodyIndex :type Integer) (bFromSweep :type Boolean) (SweepResult :type Hit%20Result%20Structure%20%28by%20ref%29))
  (bind _my_player_character (CallFunction|GetMyPlayerCharacter))
  (if (== OtherActor _my_player_character)
    (bind _returnvalue (UserInterface|CreateWidget "/Game/UI/P_Interact.P_Interact_C" 0 (Variables|/Game/ThirdPerson/Blueprints/BP_ThirdPersonCharacter.BP_ThirdPersonCharacter_C|GetUsingGamepad _my_player_character)))
    (bind _output_get (Variables|Default|SetNewVar _returnvalue))
    (UserInterface|Viewport|AddtoViewport _returnvalue 0)))

(event OnComponentEndOverlap(Sphere)
  (params (OverlappedComponent :type Primitive%20Component%20Object%20Reference) (OtherActor :type Actor%20Object%20Reference) (OtherComp :type Primitive%20Component%20Object%20Reference) (OtherBodyIndex :type Integer))
  (if (== OtherActor (Game|GetPlayerCharacter 0))
    (Widget|RemovefromParent (Variables|Default|GetNewVar))))

(event Custom|Rotate
  (bind _staticmesh (Variables|Default|GetStaticMesh))
  (bind _doorconnected (Variables|Default|GetDoorConnected))
  (bind _doorconnected_2 (Variables|Default|GetDoorConnected))
  (bind _relativerotation (Variables|/Script/Engine.SceneComponent|GetRelativeRotation _staticmesh))
  (if (not (Variables|Default|GetisMoving))
    (Variables|Default|SetisMoving true)
    (Components|MoveComponentTo (Variables|Default|GetStaticMesh) (Variables|/Script/Engine.SceneComponent|GetRelativeLocation _staticmesh) (Math|Rotator|MakeRotator (.roll _relativerotation) (.pitch _relativerotation) (+ (.yaw _relativerotation) 9e+01)) true true 0.7 false)
    (Variables|Default|SetisMoving false)
    (if (Utilities|Operators|EqualEqual (Transformation|GetWorldRotation (Variables|Default|GetArrow)) (Transformation|GetWorldRotation (Variables|Default|GetArrow1)) 3e+01)
      (Rendering|SetVisibility (Variables|Default|GetWater) true false)
      (Variables|Default|SetisComplete? true)
      (bind _result (Math|Integer|IncrementInt (Variables|/Game/Blueprints/Interactables/Statues/BP_StatueDoor.BP_StatueDoor_C|GetStatuesCurrent _doorconnected))
        (:%20%20
          (Variables|/Game/Blueprints/Interactables/Statues/BP_StatueDoor.BP_StatueDoor_C|SetStatuesCurrent _doorconnected _result)
          (Default|CheckStatues _doorconnected)))
      (else
        (Rendering|SetVisibility (Variables|Default|GetWater) false false)
        (if (== (Variables|/Game/Blueprints/Interactables/Statues/BP_StatueDoor.BP_StatueDoor_C|GetStatuesCurrent (Variables|Default|GetDoorConnected)) 0)
          (Math|Integer|DecrementInt (Variables|/Game/Blueprints/Interactables/Statues/BP_StatueDoor.BP_StatueDoor_C|GetStatuesCurrent _doorconnected_2)
            (:%20%20
              (Variables|/Game/Blueprints/Interactables/Statues/BP_StatueDoor.BP_StatueDoor_C|SetStatuesCurrent _doorconnected_2 0)
              (Default|CheckStatues _doorconnected_2))))))))

(event EventBeginPlay
  (Rendering|SetVisibility (Variables|Default|GetWater) false false))

(fn ConstructionScript)

(fn Interact
  (CallFunction|Rotate)
  (return ""))