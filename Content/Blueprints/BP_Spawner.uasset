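; BP_Spawner is a trigger-volume enemy spawner that ambushes the player with a group of Jackal enemies.
; When player pawn 0 first overlaps the Box, a DoOnce gate calls SpawnAI so the group spawns only once.
; SpawnAI spawns four BP_JackalEnemy pawns running BT_Enemy_Jackal, each at the location and rotation of its own Billboard component, which serves as a spawn marker.
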(event OnComponentBeginOverlap(Box)
  (params (OverlappedComponent :type Primitive%20Component%20Object%20Reference) (OtherActor :type Actor%20Object%20Reference) (OtherComp :type Primitive%20Component%20Object%20Reference) (OtherBodyIndex :type Integer) (bFromSweep :type Boolean) (SweepResult :type Hit%20Result%20Structure%20%28by%20ref%29))
  (if (== OtherActor (Game|Player|GetPlayerPawn 0))
    (Utilities|FlowControl|DoOnce false
      (:Completed
        (CallFunction|SpawnAI)))))

(event Custom|SpawnAI
  (bind _billboard3 (Variables|Default|GetBillboard3))
  (bind _billboard (Variables|Default|GetBillboard))
  (bind _billboard1 (Variables|Default|GetBillboard1))
  (bind _billboard2 (Variables|Default|GetBillboard2))
  (Utilities|FlowControl|Sequence
    (:then_0
      (AI|SpawnAIFromClass "/Game/Blueprints/Enemies/Blueprints/BP_JackalEnemy.BP_JackalEnemy_C" "/Game/Blueprints/Enemies/JackalEnemyAI/BT_Enemy_Jackal.BT_Enemy_Jackal" (Transformation|GetWorldLocation _billboard) (Transformation|GetWorldRotation _billboard) false 0))
    (:then_1
      (AI|SpawnAIFromClass "/Game/Blueprints/Enemies/Blueprints/BP_JackalEnemy.BP_JackalEnemy_C" "/Game/Blueprints/Enemies/JackalEnemyAI/BT_Enemy_Jackal.BT_Enemy_Jackal" (Transformation|GetWorldLocation _billboard1) (Transformation|GetWorldRotation _billboard1) false 0))
    (:then_2
      (AI|SpawnAIFromClass "/Game/Blueprints/Enemies/Blueprints/BP_JackalEnemy.BP_JackalEnemy_C" "/Game/Blueprints/Enemies/JackalEnemyAI/BT_Enemy_Jackal.BT_Enemy_Jackal" (Transformation|GetWorldLocation _billboard2) (Transformation|GetWorldRotation _billboard2) false 0))
    (:then_3
      (AI|SpawnAIFromClass "/Game/Blueprints/Enemies/Blueprints/BP_JackalEnemy.BP_JackalEnemy_C" "/Game/Blueprints/Enemies/JackalEnemyAI/BT_Enemy_Jackal.BT_Enemy_Jackal" (Transformation|GetWorldLocation _billboard3) (Transformation|GetWorldRotation _billboard3) false 0))))

(event EventBeginPlay)

(fn ConstructionScript)