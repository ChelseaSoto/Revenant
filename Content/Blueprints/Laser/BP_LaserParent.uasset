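; BP_LaserParent is a base Blueprint for laser-related actors, with a time-stop response and cleanup of attached lasers.
; TimeStop toggles physics on SMVisual through a FlipFlop, freezing it and then resuming simulation.
; Linear velocity is read before freezing for reapplication, while angular velocity is only read on unfreeze.
; ClearAllLasersAttached destroys every valid actor in LasersAttached and empties the array.
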(event EventBeginPlay)

(event EventTick
  (params (DeltaSeconds :type Float%20%28single-precision%29)))

(event EventTimeStop
  (Utilities|Stop/StartPhysics (Variables|Default|GetSM_Visual)))

(event Collision|EventActorBeginOverlap
  (params (OtherActor :type Actor%20Object%20Reference)))

(fn ConstructionScript)

(fn ClearAllLasersAttached
  ;[1 1 1] Deletes all lasers within the Attached array //Omar
  (for _array_element (Variables|Default|GetLasersAttached)
    (Utilities|IsValid _array_element
      (:Is%20Valid
        (Actor|DestroyActor _array_element))))
  (Utilities|Array|Clear (Variables|Default|GetLasersAttached)))