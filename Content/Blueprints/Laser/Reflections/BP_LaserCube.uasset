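; BP_LaserCube is a laser reflection cube that emits a new child laser from its arrow while a laser hits it.
; LaserBounce takes the spawn reference from the incoming laser, then spawns a BP_LaserChild with the same color and an updated ID.
; The child attaches to the cube's visual mesh and registers in both the cube's and the spawn reference's laser arrays.
; When the hit ends, the cube clears its attached lasers.
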(fn ConstructionScript
  (|CallParentFunction))

(fn LaserBounce
  (params (LaserThatHit :type BP%20Laser%20Child%20Object%20Reference) (HitResponse :type Boolean) (HitResult :type Hit%20Result%20Structure))
  ;[1 1 1] If the laser that hit this is valid make it the spawn Ref //Omar
  (Utilities|IsValid LaserThatHit
    (:Is%20Valid
      (Variables|Default|SetSpawnRef (Variables|/Game/Blueprints/Laser/BP_LaserParent.BP_LaserParent_C|GetSpawnRef LaserThatHit))
      (bind _output_get (Variables|Default|SetActive HitResponse))
      ;[1 1 1] If I am getting hit spawn a new laser from my arrow! //Omar
      (if _output_get
        (bind _returnvalue (Game|SpawnActorfromClass "/Game/Blueprints/Laser/BP_LaserChild.BP_LaserChild_C" (Math|Transform|MakeTransform (Transformation|GetWorldLocation (Variables|Default|GetArrow)) (Math|Rotator|MakeRotfromX (Math|Vector|GetForwardVector (Variables|Default|GetArrow))) "1.000000,1.000000,1.000000") "Undefined" "MultiplyWithRoot" 0 (Default|UpdateID LaserThatHit "C") LaserThatHit (Variables|/Game/Blueprints/Laser/BP_LaserParent.BP_LaserParent_C|GetLinearColor LaserThatHit) (Variables|Default|GetSpawnRef) 0))
        ;[1 1 1] Attach laser to this box! //Omar
        (Transformation|AttachComponentToComponent _returnvalue (Variables|Default|GetSM_Visual) "None" "KeepWorld" "KeepWorld" "KeepRelative" false)
        ;[1 1 1] Add to this array and parents array //Omar
        (Utilities|Array|Add (Variables|Default|GetLasersAttached) _returnvalue)
        (Utilities|Array|Add (Variables|/Game/Blueprints/Laser/BP_LaserSpawn.BP_LaserSpawn_C|GetChild%20Lasers (Variables|Default|GetSpawnRef)) _returnvalue)
        (return _returnvalue)
        (else
          ;[1 1 1] If I am not getting hit anymore destroy any lasers I made //Omar
          (CallFunction|ClearAllLasersAttached))))))