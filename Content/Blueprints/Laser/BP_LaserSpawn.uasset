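; Laser emitter actor that spawns the first beam of a laser chain and tracks the child lasers in it.
; On BeginPlay it spawns a BP_LaserChild at its arrow, tagged with its display name as ID, attaches it to the visual mesh, then plays beam audio and camera shake.
; RemoveFollowingLasers walks the child array backwards, cancelling lasers whose ID contains the removed ID and dropping those that confirm.
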(event EventBeginPlay
  (bind _self self)
  (bind _arrow (Variables|Default|GetArrow))
  ;[1 1 1] Set ID and Spawn Ref //Omar
  (Variables|Default|SetSpawnRef _self)
  (Variables|Default|SetID (Utilities|GetDisplayName _self))
  ;[1 1 1] Spawn Laser From Arrow
  (bind _returnvalue (Game|SpawnActorfromClass "/Game/Blueprints/Laser/BP_LaserChild.BP_LaserChild_C" (Math|Transform|MakeTransform (Transformation|GetWorldLocation (Variables|Default|GetArrow)) (Transformation|GetActorRotation) "1.000000,1.000000,1.000000") "Undefined" "MultiplyWithRoot" 0 (Variables|Default|GetID) 0 (Variables|Default|GetLinearColor) (Variables|Default|GetSpawnRef) 0))
  ;[1 1 1] Makes Laser move with parent //Omar
  (Transformation|AttachComponentToComponent _returnvalue (Variables|Default|GetSM_Visual) "None" "KeepWorld" "KeepWorld" "KeepWorld" true)
  ;[1 1 1] Sets new lasers Refrences and adds to Array //Omar
  (Variables|/Game/Blueprints/Laser/BP_LaserChild.BP_LaserChild_C|SetParentActor _returnvalue self)
  (Utilities|Array|Add (Variables|Default|GetChild%20Lasers) _returnvalue)
  ;[1 1 1] Laser Audio play //Omar
  (Audio|SpawnSoundAttached "/Game/StarterContent/Audio/LightBeam_Cue.LightBeam_Cue" _arrow "None" (Transformation|GetWorldLocation _arrow) "0, 0, 0" "KeepRelativeOffset" true 1.0 1.0 0.0 0 0)
  (Camera|PlayWorldCameraShake "/Game/Blueprints/BP_CamShake.BP_CamShake_C" (Transformation|GetActorLocation (Game|Player|GetPlayerPawn 0)) 0.0 5e+03))

(event EventTick
  (params (DeltaSeconds :type Float%20%28single-precision%29)))

(fn ConstructionScript
  (|CallParentFunction))

(fn RemoveFollowingLasers
  (params (Laser%20Ref :type BP%20Laser%20Child%20Object%20Reference))
  (LocalVariables|SetL-ID_Removed (Variables|/Game/Blueprints/Laser/BP_LaserChild.BP_LaserChild_C|GetLaser_ID Laser%20Ref))
  ;[1 1 1] Removes this laser ID and ones made from it //Omar
  (bind _arrayelement (Utilities|Array|ReverseforEachLoop (Variables|Default|GetChild%20Lasers))
    (:LoopBody
      (Utilities|IsValid _arrayelement
        (:Is%20Valid
          (if (Utilities|String|Contains (Variables|/Game/Blueprints/Laser/BP_LaserChild.BP_LaserChild_C|GetLaser_ID _arrayelement) (LocalVariables|GetL-ID_Removed))
            (bind _remove_from_array (Default|CancleTargetHit _arrayelement (Utilities|Enum|Equal(Enum) (Variables|/Game/Blueprints/Laser/BP_LaserChild.BP_LaserChild_C|GetLaser_ID _arrayelement) (LocalVariables|GetL-ID_Removed))))
            (if _remove_from_array
              (Utilities|Array|RemoveItem (Variables|Default|GetChild%20Lasers) _arrayelement))))))))