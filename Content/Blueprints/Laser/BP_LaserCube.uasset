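; BP_LaserCube is a laser redirector that re-emits an incoming beam along the forward direction of its arrow component.
; On an active hit, LaserBounce spawns a child laser with an updated ID and the incoming color, attached to the cube's visual mesh.
; It registers each child with both the cube and the originating spawner reference.
; An inactive response clears all attached lasers.
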(fn ConstructionScript
  (|CallParentFunction))

(fn LaserBounce
  (params (LaserThatHit :type BP%20Laser%20Child%20Object%20Reference) (HitResponse :type Boolean) (HitResult :type Hit%20Result%20Structure))
  (Utilities|IsValid LaserThatHit
    (:Is%20Valid
      (Variables|Default|SetSpawnRef (Variables|/Game/Blueprints/Laser/BP_LaserParent.BP_LaserParent_C|GetSpawnRef LaserThatHit))
      (bind _output_get (Variables|Default|SetActive HitResponse))
      (if _output_get
        (bind _returnvalue (Game|SpawnActorfromClass "/Game/Blueprints/Laser/BP_LaserChild.BP_LaserChild_C" (Math|Transform|MakeTransform (Transformation|GetWorldLocation (Variables|Default|GetArrow)) (Math|Rotator|MakeRotfromX (Math|Vector|GetForwardVector (Variables|Default|GetArrow))) "1.000000,1.000000,1.000000") "Undefined" "MultiplyWithRoot" 0 (Default|UpdateID LaserThatHit "C") LaserThatHit (Variables|/Game/Blueprints/Laser/BP_LaserParent.BP_LaserParent_C|GetLinearColor LaserThatHit) (Variables|Default|GetSpawnRef) 0))
        (Transformation|AttachComponentToComponent _returnvalue (Variables|Default|GetSM_Visual) "None" "KeepWorld" "KeepWorld" "KeepRelative" false)
        (Utilities|Array|Add (Variables|Default|GetLasersAttached) _returnvalue)
        (Utilities|Array|Add (Variables|/Game/Blueprints/Laser/BP_LaserSpawn.BP_LaserSpawn_C|GetChild%20Lasers (Variables|Default|GetSpawnRef)) _returnvalue)
        (return _returnvalue)
        (else
          (CallFunction|ClearAllLasersAttached))))))