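; BP_LaserChild is a laser segment that updates every tick while its parent actor is valid, otherwise destroying itself.
; A forward box trace sets the beam length and stamps short-lived trail decals.
; New hits send BPI_Laser messages to obtain bounce lasers or damage actors named "Enemy", while repeated BP_ReflectLaser hits reposition the bounce.
; Changing or losing targets triggers cleanup through SpawnRef or the interface.
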(event EventBeginPlay)

(event EventTick
  (params (DeltaSeconds :type Float%20%28single-precision%29))
  ;[1 1 1] If parent is active keep updating else destroy //Omar
  (Utilities|IsValid (Variables|Default|GetParentActor)
    (:Is%20Valid
      (CallFunction|SetEndPoint))
    (:Is%20Not%20Valid
      (Actor|DestroyActor))))

(fn ConstructionScript
  (|CallParentFunction))

(fn SetEndPoint
  (bind _returnvalue (Transformation|GetActorLocation))
  (bind _returnvalue_2 (Transformation|GetActorForwardVector))
  (bind _returnvalue_3 (* _returnvalue_2 2.0))
  (bind _returnvalue_4 (+ _returnvalue _returnvalue_3))
  ;[1 1 1] Line cast for laser size //Omar
  (bind _outhit (Collision|BoxTraceByChannel _returnvalue_4 (+ _returnvalue_4 (* _returnvalue_2 (LocalVariables|GetL-Range))) "0.500000,0.500000,0.500000" "0, 0, 0" "TraceTypeQuery2" false 0 "None"))
  ;[1 1 1] Scales Laser to line case info, then calls a decal to spawn at hit location //Omar
  (bind _output_get (LocalVariables|SetL-HitInfo _outhit))
  (LocalVariables|SetL-HitActor (.HitActor (Collision|BreakHitResult _output_get)))
  (Utilities|FlowControl|Sequence
    (:then_0
      (Effects|Components|ParticleSystem|SetVectorParameter (Variables|Default|GetBeam%20FX) "Beam End" (Math|Vector|MakeVector 0.0 0.0 (Math|Float|SelectFloat (+ (.Distance (Collision|BreakHitResult _output_get)) -2.5e+02) (LocalVariables|GetL-Range) (.bBlockingHit (Collision|BreakHitResult _output_get)))))
      (LocalVariables|GetL-HitActor
        (:then
          (Utilities|FlowControl|Sequence
            (:then_0
              (if (== (Variables|Default|GetLastHitActor) (LocalVariables|GetL-HitActor))
                ;[1 1 1] If hit is reflection
                (bind _asbp_reflect_laser (Utilities|Casting|CastToBP_ReflectLaser (Variables|Default|GetLastHitActor)))
                (Transformation|SetActorLocation (Variables|Default|GetBounceLaser) (.ImpactPoint (Collision|BreakHitResult (LocalVariables|GetL-HitInfo))) false false)
                (Transformation|SetActorRotation (Variables|Default|GetBounceLaser) (Default|CalcRotation _asbp_reflect_laser (.ImpactPoint (Collision|BreakHitResult (LocalVariables|GetL-HitInfo))) (.ImpactNormal (Collision|BreakHitResult (LocalVariables|GetL-HitInfo))) (.TraceStart (Collision|BreakHitResult (LocalVariables|GetL-HitInfo)))))
                (else
                  ;[1 0 0.02061] If you wanted to add enemy hit functions call it from here, by adding a new does implement and add a BPI_enemy interface then call a take damage function I think that should work //Omar
                  (Utilities|FlowControl|Sequence
                    (:then_0
                      (if (Utilities|DoesObjectImplementInterface (Variables|Default|GetLastHitActor) "/Game/Blueprints/Laser/BPI_Laser.BPI_Laser_C")
                        (Default|RemoveFollowingLasers (Variables|Default|GetSpawnRef) self)))
                    (:then_1
                      ;[1 1 1] Call bounce if can //Omar
                      (if (Utilities|DoesObjectImplementInterface (LocalVariables|GetL-HitActor) "/Game/Blueprints/Laser/BPI_Laser.BPI_Laser_C")
                        (bind _new_laser (Class|BPILaser|LaserBounce(Message) (LocalVariables|GetL-HitActor) self true (LocalVariables|GetL-HitInfo) (Variables|Default|GetActors%20I've%20hit)))
                        (Variables|Default|SetBounceLaser _new_laser)))
                    (:then_2
                      (if (Utilities|String|Contains (Utilities|GetDisplayName (LocalVariables|GetL-HitActor)) "Enemy")
                        (Game|Damage|ApplyDamage (LocalVariables|GetL-HitActor) 5.0 0 (Components|GetOwner))))))))
            (:then_1
              (Variables|Default|SetLastHitActor (LocalVariables|GetL-HitActor)))))
        (:else
          ;[1 1 1] If new Position and uses interface bounce //Omar
          (Utilities|FlowControl|Sequence
            (:then_0
              (bind _lasthitactor (Variables|Default|GetLastHitActor)
                (:then
                  (if (Utilities|DoesObjectImplementInterface _lasthitactor "/Game/Blueprints/Laser/BPI_Laser.BPI_Laser_C")
                    (Class|BPILaser|LaserBounce(Message) (Variables|Default|GetLastHitActor) self false (LocalVariables|GetL-HitInfo) (Variables|Default|GetActors%20I've%20hit))))
                (:else)))
            (:then_1
              (Variables|Default|SetLastHitActor 0)
              (Variables|Default|SetBounceLaser 0))))))
    (:then_1
      (CallFunction|SpawnDecal (.ImpactPoint (Collision|BreakHitResult _output_get)) (Math|Conversions|RotationFromXVector (.Normal (Collision|BreakHitResult _output_get))) (.HitComponent (Collision|BreakHitResult _output_get))))))

(fn UpdateID
  (params (P-Append :type String))
  ;[1 1 1] Adds to Parent ID to make own //Omar
  (return (Utilities|String|Append (Variables|Default|GetLaser_ID) P-Append)))

(fn CancleTargetHit
  (params (Override :type Boolean))
  (Utilities|FlowControl|Sequence
    (:then_0
      (bind _lasthitactor (Variables|Default|GetLastHitActor)
        (:then
          ;[1 1 1] If uses interface call bounce //Omar
          (bind _asbp_laser_parent (Utilities|Casting|CastToBP_LaserParent _lasthitactor))
          (if (and (Utilities|DoesObjectImplementInterface _asbp_laser_parent "/Game/Blueprints/Laser/BPI_Laser.BPI_Laser_C") (Utilities|Array|IsEmpty (Variables|/Game/Blueprints/Laser/BP_LaserParent.BP_LaserParent_C|GetLasersAttached _asbp_laser_parent)))
            (Class|BPILaser|LaserBounce(Message) (Variables|Default|GetLastHitActor) self false)
            (else
              (Variables|/Game/Blueprints/Laser/BP_LaserParent.BP_LaserParent_C|SetActive _asbp_laser_parent false))))
        (:else)))
    (:then_1
      (if Override
        (return false)
        (else
          (Actor|DestroyActor)
          (return true))))))

(fn SpawnDecal
  (params (HitLocation :type Vector) (Hit%20normal :type Rotator) (ActorHit :type Primitive%20Component%20Object%20Reference))
  ;[1 1 1] Spawn Decal at attched location
  (Utilities|FlowControl|Sequence
    (:then_0
      _)
    (:then_1
      _)
    (:then_2
      _))
  (Class|GameplayStatics|SpawnDecalAttached "/Game/Materials/M_LaserTrailTest.M_LaserTrailTest" "15.000000,15.000000,15.000000" ActorHit "None" HitLocation Hit%20normal "KeepWorldPosition" 0.3))