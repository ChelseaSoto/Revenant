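; BP_Spawner1 is an enemy spawner that releases a test enemy when the player enters its trigger.
; The Box overlap event checks for the first player's pawn and passes through a DoOnce, so it fires a single time.
; It then calls the SpawnAI event, which spawns BP_TestEnemy at the Billboard component's location and rotation.
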(event OnComponentBeginOverlap(Box)
  (params (OverlappedComponent :type Primitive%20Component%20Object%20Reference) (OtherActor :type Actor%20Object%20Reference) (OtherComp :type Primitive%20Component%20Object%20Reference) (OtherBodyIndex :type Integer) (bFromSweep :type Boolean) (SweepResult :type Hit%20Result%20Structure%20%28by%20ref%29))
  (if (== OtherActor (Game|Player|GetPlayerPawn 0))
    (Utilities|FlowControl|DoOnce false
      (:Completed
        (CallFunction|SpawnAI)))))

(event Custom|SpawnAI
  (bind _billboard (Variables|Default|GetBillboard))
  (Utilities|FlowControl|Sequence
    (:then_0
      (AI|SpawnAIFromClass "/Game/Blueprints/Enemies/Blueprints/BP_TestEnemy.BP_TestEnemy_C" 0 (Transformation|GetWorldLocation _billboard) (Transformation|GetWorldRotation _billboard) false 0))))

(event EventBeginPlay)

(fn ConstructionScript)