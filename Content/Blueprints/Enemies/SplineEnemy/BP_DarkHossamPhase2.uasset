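; Phase 2 of the Dark Hossam boss, a child enemy Blueprint with a health bar and melee attacks.
; DogAttack alternates two timed attacks, checking one or two hitboxes before applying damage and a knockback launch to the player.
; Damaged updates the boss bar and fires one-shot calls by health band, while a separate macro randomly picks a combo or upward-attack montage.
; Death spawns smoke bursts and teleports the actor before running parent logic.
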(event Custom|Reset%20HP%20Bar
  (bind _maxhealth (Variables|Default|GetMaxHealth))
  (Default|UpdateHealthPercent (Variables|Default|GetBossHP) _maxhealth _maxhealth))

(event Custom|DogAttack
  (switch int (Variables|Default|GetNext%20attack)
    (:0
      (Variables|Default|SetisAttacking true)
      (Utilities|FlowControl|Delay 1.0)
      (bind _result (CallFunction|PlayerinHitBox (Variables|Default|GetNext%20attack)))
      (if _result
        (CallFunction|DealDamageKnockback))
      (Variables|Default|SetNext%20attack 1)
      (Default|CallAttackEnd))
    (:1
      (Utilities|FlowControl|Delay 0.5)
      (Variables|Default|SetisAttacking2 true)
      (Utilities|FlowControl|Delay 1.25)
      (bind _result_2 (CallFunction|PlayerinHitBox (Variables|Default|GetNext%20attack)))
      (if _result_2
        (CallFunction|DealDamageKnockback))
      (Variables|Default|SetNext%20attack 0)
      (Default|CallAttackEnd))))

(fn ConstructionScript
  (|CallParentFunction))

(fn Damaged
  (|CallParentFunction)
  (Utilities|FlowControl|Sequence
    (:then_0
      (Default|UpdateHealthPercent (Variables|Default|GetBossHP) (Variables|Default|GetHealth) (Variables|Default|GetMaxHealth)))
    (:then_1
      (if (<= (* (Variables|Default|GetMaxHealth) 0.8) (Variables|Default|GetHealth))
        (Utilities|FlowControl|DoOnce false
          (:Completed
            (Default|Call80%)))
        (elif (<= (* (Variables|Default|GetMaxHealth) 0.6) (Variables|Default|GetHealth))
          (Utilities|FlowControl|DoOnce false
            (:Completed
              (Default|Call60%)))
          (elif (<= (* (Variables|Default|GetMaxHealth) 0.5) (Variables|Default|GetHealth))
            (Utilities|FlowControl|DoOnce false
              (:Completed
                (Default|Call50%)))))))))

(fn PlayAttackAnimation
  (|CallParentFunction))

(fn DeathFunc
  (bind _returnvalue (Transformation|GetActorLocation))
  (Niagara|SpawnSystematLocation "/Game/VFX/FireVFX/NS_SethSmokeBurst.NS_SethSmokeBurst" (Math|Vector|MakeVector (.x _returnvalue) (.y _returnvalue) (.z _returnvalue)))
  (Niagara|SpawnSystematLocation "/Game/VFX/FireVFX/NS_SethSmokeBurst.NS_SethSmokeBurst" (Math|Vector|MakeVector (.x _returnvalue) (.y _returnvalue) (- (.z _returnvalue) 2e+02)))
  (Transformation|SetActorTransform (Math|Transform|MakeTransform "0, 0, 0" "0, 0, 0" "1.000000,1.000000,1.000000") false true)
  (|CallParentFunction))

(fn DealDamageKnockback
  (bind _returnvalue (Game|GetPlayerCharacter 0))
  (bind _self self)
  (bind _returnvalue_2 (Transformation|GetActorForwardVector _self))
  (Character|LaunchCharacter _returnvalue (* (Math|Vector|MakeVector (.x _returnvalue_2) (.y _returnvalue_2) (+ (.z _returnvalue_2) 1.0)) (Variables|Default|GetKnockback)) false false)
  (Game|Damage|ApplyDamage _returnvalue 2e+01 0 0))

(fn PlayerinHitBox
  (params (Attack :type Integer))
  (bind _returnvalue (Game|GetPlayerCharacter 0))
  (bind _hitbox (Variables|Default|GetHitBox))
  (bind _returnvalue_2 (Collision|IsOverlappingActor _hitbox _returnvalue :!class /Script/Engine.PrimitiveComponent))
  (switch int Attack
    (:0
      (Variables|Default|SetPlayerCheckOutput _returnvalue_2))
    (:1
      (Variables|Default|SetPlayerCheckOutput (or _returnvalue_2 (Collision|IsOverlappingActor (Variables|Default|GetHitBox2) (Game|GetPlayerCharacter 0) :!class /Script/Engine.PrimitiveComponent)))))
  (return (Variables|Default|GetPlayerCheckOutput)))