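; BP_DarkHossam is a sword-wielding enemy with health-based triggers that cycles through randomly chosen melee, shockwave and laser attacks.
; It spawns its sword on the mesh socket, feeds it to the trace component and destroys it on death.
; Montage-driven attack macros spawn projectiles on notifies, then reroll the next attack, its radius and idle time.
; Damage can randomly trigger stun or block, updates the health bar and fires one-time health-bracket calls.
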(event Custom|Blocked!_Event
  ;[1 1 1] Blocking
  (Variables|Default|SetBlocking%20State "NewEnumerator2")
  (Animation|Montage|PlayMontage (Variables|Character|GetMesh) "/Game/ArtPrototype/Rigs/Hossam/Animations/Fixed/AM_BlockImpact.AM_BlockImpact"
    (:OnCompleted
      _)
    (:OnInterrupted
      _))
  (CallFunction|EndBlock))

(event Custom|Stun%20Check
  ;[1 1 1] Stun
  (if (Variables|Default|GetcanStun)
    (Components|Movement|StopMovementImmediately (Variables|Character|GetCharacterMovement))
    (Animation|Montage|PlayMontage (Variables|Character|GetMesh) "/Game/ArtPrototype/Rigs/Hossam/Animations/New/AM_Stunned.AM_Stunned"
      (:OnCompleted
        (Variables|Default|SetcanStun false)
        (Variables|Default|SetIdlePlaying 5.0)
        (bind _output_get (Variables|Default|SetNext%20attack (Math|Random|RandomIntegerinRange 0 3)))
        (if (== _output_get 2)
          (Variables|Default|SetAttack%20Rad 5e+02)
          (else
            (Variables|Default|SetAttack%20Rad 1e+02)))
        (Default|CallOnAttackEnd)))))

(event Custom|CustomEvent
  (Actor|DestroyActor (Variables|Default|GetAs%20BP%20Base%20Sword)))

(event Custom|Clear
  (Utilities|Array|Clear (Variables|/Game/ThirdPerson/Equipment/TraceComponent_darkhossam.TraceComponent_darkhossam_C|GetActorsToIgnore (Variables|Default|GetTraceComponent_darkhossam))))

(event EventBeginPlay
  (|CallParentFunction)
  (Variables|Default|SetNext%20attack (Math|Random|RandomIntegerinRange 0 2))
  (bind _returnvalue (Game|SpawnActorfromClass "/Game/ThirdPerson/Equipment/BP_BaseSword.BP_BaseSword_C" (Transformation|GetSocketTransform (Variables|Character|GetMesh) "sword" "RTS_World") "Undefined" "MultiplyWithRoot" 0 0))
  (Rendering|SetCastShadow (Variables|/Game/ThirdPerson/Equipment/BP_BaseSword.BP_BaseSword_C|GetSkeletalMesh _returnvalue) false)
  (bind _output_get (Variables|Default|SetAs%20BP%20Base%20Sword _returnvalue))
  (Transformation|AttachComponentToComponent _output_get (Variables|Character|GetMesh) "sword" "SnapToTarget" "SnapToTarget" "SnapToTarget" true)
  (Variables|/Game/ThirdPerson/Equipment/TraceComponent_darkhossam.TraceComponent_darkhossam_C|Setswordref (Variables|Default|GetTraceComponent_darkhossam) (Variables|Default|GetAs%20BP%20Base%20Sword))
  (EventDispatchers|BindEventtoDeath (delegate Custom|CustomEvent)))

(event EventStartBlock
  ;[1 1 1] Blocking
  (Variables|Default|SetisBlocking? true)
  (Variables|Default|SetBlocking%20State "NewEnumerator1")
  (Animation|Montage|PlayMontage (Variables|Character|GetMesh) "/Game/ArtPrototype/Rigs/Hossam/Animations/Fixed/AM_Block.AM_Block"
    (:OnCompleted
      (CallFunction|EndBlock :!label _label))
    (:OnInterrupted
      (if (Utilities|Enum|NotEqual(Enum) (Variables|Default|GetBlocking%20State) "NewEnumerator2")
        (goto _label)))))

(event EventAttack
  (Variables|Default|SetcanStun true)
  (switch int (Variables|Default|GetNext%20attack)
    (:0
      (Utilities|RandomAttackAnim :!label _label
        (:Completed
          (Variables|Default|SetcanStun false :!label _label_2)
          (Variables|Default|SetIdlePlaying 5.0)
          (bind _output_get (Variables|Default|SetNext%20attack (Math|Random|RandomIntegerinRange 0 3)))
          (if (== _output_get 2)
            (Variables|Default|SetAttack%20Rad 5e+02)
            (else
              (Variables|Default|SetAttack%20Rad 1e+02)))
          (Default|CallOnAttackEnd))
        (:Interupped
          (CallFunction|StunCheck :!label _label_3))))
    (:1
      (goto _label))
    (:2
      (Variables|Default|SetIdlePlaying 4.9)
      (|ShockWave
        (:OnCompleted
          (goto _label_2))
        (:OnInterrupted
          (goto _label_3))))
    (:3
      (|SpawnLaser
        (:OnCompleted
          (goto _label_2))
        (:OnInterrupted
          (goto _label_3))))))

(fn ConstructionScript
  (|CallParentFunction))

(fn Damaged
  (|CallParentFunction)
  (Utilities|FlowControl|Sequence
    (:then_0
      (if (Math|Random|RandomBoolwithWeight 0.2)
        (CallFunction|StunCheck))
      (if (Math|Random|RandomBoolwithWeight 0.2)
        (CallFunction|StartBlock))
      (Default|UpdateHealthPercent (Variables|Default|GetHPBar) (Variables|Default|GetHealth) (Variables|Default|GetMaxHealth)))
    (:then_1
      (if (<= (* (Variables|Default|GetMaxHealth) 0.8) (Variables|Default|GetHealth))
        (Utilities|FlowControl|DoOnce false
          (:Completed
            (Default|Call80%)))
        (elif (<= (* (Variables|Default|GetMaxHealth) 0.6) (Variables|Default|GetHealth))
          (Utilities|FlowControl|DoOnce false
            (:Completed
              (Default|Call60%)))
          (elif (<= (* (Variables|Default|GetMaxHealth) 0.5) (Variables|Default|GetHealth))
            (Utilities|FlowControl|DoOnce false
              (:Completed
                (Default|Call50%)))))))))

(fn PlayAttackAnimation
  (|CallParentFunction))

(fn DeathFunc
  (|CallParentFunction)
  (Animation|PlayAnimMontage "/Game/Characters/Hossam/New_Anims/RT_Death_Montage.RT_Death_Montage" 1.0 "None"))