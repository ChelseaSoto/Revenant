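; Minotaur enemy that cycles through uppercut, stomp, sweep and kick attacks against the player.
; Each attack sets a state flag, waits for animation-matched delays, then checks hitbox overlap to deal damage, with knockback on all but stomp, before signalling attack end.
; Damage handling extends the parent with one-shot calls for 80, 60 and 50 percent health bands.
; A separate macro plays a weighted random attack montage.
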(event Custom|Kick
  ;[1 1 1] Logic for kick
  (Variables|Default|SetisKicking true)
  (Utilities|FlowControl|Delay 0.65)
  (bind _result (CallFunction|PlayerinHitbox))
  (if _result
    (CallFunction|DealDamageKnockback)
    (else
      (Development|PrintString "Player not hit")))
  (Utilities|FlowControl|Delay 1.5)
  (Variables|Default|SetisKicking false)
  (Default|CallMinotaurAttackEnd))

(event Custom|Sweep
  ;[1 1 1] Logic for the sweep
  (Variables|Default|SetisSweeping true)
  (Utilities|FlowControl|Delay 0.85)
  (bind _result (CallFunction|PlayerinHitbox))
  (if _result
    (CallFunction|DealDamageKnockback)
    (else
      (Development|PrintString "Player not hit")))
  ;;[1 1 1] Time until minotaur stands back up
  (Utilities|FlowControl|Delay 5.3)
  (Variables|Default|SetisSweeping false)
  (Default|CallMinotaurAttackEnd))

(event Custom|Stomp
  ;[1 1 1] Logic for the stomp
  (Variables|Default|SetisStomping true)
  (Utilities|FlowControl|Delay 0.9)
  (bind _result (CallFunction|PlayerinHitbox))
  (if _result
    (Game|Damage|ApplyDamage (Game|GetPlayerCharacter 0) 2e+01 0 self)
    (else
      (Development|PrintString "Player not hit")))
  (Utilities|FlowControl|Delay 1.0)
  (Variables|Default|SetisStomping false)
  (Default|CallMinotaurAttackEnd))

(event Custom|AttackEvent
  ;[1 1 1] Attack logic, cycles through each attack type
  (if (Variables|Default|GetCan%20Attack)
    (Variables|Default|SetCan%20Attack false)
    (bind _output_get (Variables|Default|SetAttack%20Index (+ (Variables|Default|GetAttack%20Index) 1)))
    (Development|PrintString (Utilities|String|ToString(Integer) (Math|Integer|%(Integer) _output_get 4)))
    (switch int (Math|Integer|%(Integer) _output_get 4)
      (:0
        (CallFunction|Uppercut))
      (:1
        (CallFunction|Stomp))
      (:2
        (CallFunction|Sweep))
      (:3
        (CallFunction|Kick)))))

(event Custom|Uppercut
  ;[1 1 1] Logic for the Uppercut
  (Variables|Default|SetisSwiping true)
  (if (not (Variables|Default|GetisCharging))
    ;;[1 1 1] based on anim timings
    (Utilities|FlowControl|Delay 1.1)
    (else
      (Utilities|FlowControl|Delay 0.66)))
  (bind _result (CallFunction|PlayerinHitbox))
  (if _result
    (CallFunction|DealDamageKnockback)
    (else
      (Development|PrintString "Player not hit!")))
  (Utilities|FlowControl|Delay 1.0)
  (Variables|Default|SetisSwiping false)
  (Default|CallMinotaurAttackEnd))

(fn ConstructionScript
  (Transformation|AttachComponentToComponent (Variables|Default|GetNiagara) (Variables|Character|GetMesh) "None" "SnapToTarget" "SnapToTarget" "KeepWorld" true))

(fn Damaged
  (|CallParentFunction)
  (Utilities|FlowControl|Sequence
    (:then_1
      (if (<= (* (Variables|Default|GetMaxHealth) 0.8) (Variables|Default|GetHealth))
        (Utilities|FlowControl|DoOnce false
          (:Completed
            (Default|Call80%)))
        (elif (<= (* (Variables|Default|GetMaxHealth) 0.6) (Variables|Default|GetHealth))
          (Utilities|FlowControl|DoOnce false
            (:Completed
              (Default|Call60%)))
          (elif (<= (* (Variables|Default|GetMaxHealth) 0.5) (Variables|Default|GetHealth))
            (Utilities|FlowControl|DoOnce false
              (:Completed
                (Default|Call50%)))))))))

(fn PlayAttackAnimation
  (|CallParentFunction))

(fn DeathFunc
  (|CallParentFunction)
  (Development|PrintString "dopa down" true true "(R=1.000000,G=0.000000,B=0.005617,A=1.000000)" 5.0))

(fn DealDamageKnockback
  (bind _returnvalue (Game|GetPlayerCharacter 0))
  (bind _self self)
  (bind _returnvalue_2 (Transformation|GetActorForwardVector _self))
  (Character|LaunchCharacter _returnvalue (* (Math|Vector|MakeVector (.x _returnvalue_2) (.y _returnvalue_2) (+ (.z _returnvalue_2) 1.0)) (Variables|Default|GetKnockback)) false false)
  (Game|Damage|ApplyDamage _returnvalue 2e+01 0 self))

(fn PlayerinHitbox
  (return (Collision|IsOverlappingActor (Variables|Default|GetAttackHitBox) (Game|GetPlayerCharacter 0) :!class /Script/Engine.PrimitiveComponent)))