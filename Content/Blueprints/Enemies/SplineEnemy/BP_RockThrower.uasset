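; BP_RockThrower is a ranged enemy that attacks by launching a burst of projectiles at the player.
; Attack turns an arrow component toward the player, spawns BP_Projectile instances from it with random cone spread, then signals attack end after a short delay.
; It also reports its attack and defend radii and maps a movement state to walk speed.
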(event EventBeginPlay)

(event Collision|EventActorBeginOverlap
  (params (OtherActor :type Actor%20Object%20Reference)))

(event EventTick
  (params (DeltaSeconds :type Float%20%28single-precision%29)))

(event EventAttack
  (bind _arrow1 (Variables|Default|GetArrow1))
  (bind _arrow1_2 (Variables|Default|GetArrow1))
  (Transformation|SetWorldRotation _arrow1 (Math|Rotator|FindLookatRotation (Transformation|GetWorldLocation _arrow1) (Transformation|GetActorLocation (Game|GetPlayerCharacter 0))) false false)
  (for _index (range 0 2)
    (Game|SpawnActorfromClass "/Game/Blueprints/Enemies/SplineEnemy/Weapons/BP_Projectile.BP_Projectile_C" (Math|Transform|MakeTransform (Transformation|GetWorldLocation _arrow1_2) (CallFunction|GetSpray (Math|Vector|GetForwardVector _arrow1_2) 4.0)) "AlwaysSpawn" "OverrideRootScale" 0 0))
  (Utilities|FlowControl|Delay 0.2)
  (Default|CallOnAttackEnd))

(fn ConstructionScript
  (|CallParentFunction))

(fn GetIdealRange
  (return (Variables|Default|GetAttack%20Rad) (Variables|Default|GetDefend%20Rad)))

(fn SetMovementSpeed
  (params (Speed :type E_MoveSpeed%20Enum :default "NewEnumerator0"))
  (bind _output_get (Variables|/Script/Engine.CharacterMovementComponent|SetMaxWalkSpeed (Variables|Character|GetCharacterMovement) (Utilities|Select :Index Speed :NewEnumerator0 (Variables|Default|GetIdle) :NewEnumerator1 (Variables|Default|GetWalking) :NewEnumerator2 (Variables|Default|GetJogging) :NewEnumerator3 (Variables|Default|GetSprinting))))
  (return _output_get))