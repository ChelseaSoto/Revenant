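; BP_HookedMonster is a four-legged enemy character with procedural foot placement and a hook melee attack.
; Alternating timers update diagonal foot pairs by tracing to the ground, playing a footstep sound when a target moves far enough.
; Attack pauses stepping, plays the hook animation, then restores the Animation Blueprint, clears the hook trace's ignore list and signals completion.
; It also supplies combat ranges and movement speeds, and passes sounds to its AI controller.
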(event Custom|Check%20Left
  (Utilities|Time|ClearandInvalidateTimerbyHandle (stale Custom|CheckRight _returnvalue))
  (bind _returnvalue (Utilities|Time|SetTimerbyEvent (delegate Custom|CheckRight) 0.2))
  (bind _newparam (CallFunction|FindFootPlacement (Variables|Default|GetFrontLeft) (Variables|Default|GetFRONTL)))
  (Variables|Default|SetFRONTL _newparam)
  (bind _newparam_2 (CallFunction|FindFootPlacement (Variables|Default|GetBackRight) (Variables|Default|GetBACKR)))
  (Variables|Default|SetBACKR _newparam_2))

(event Custom|CheckRight
  (Utilities|Time|ClearandInvalidateTimerbyHandle (stale Custom|Check%20Left _returnvalue))
  (bind _returnvalue (Utilities|Time|SetTimerbyEvent (delegate Custom|Check%20Left) 0.2))
  (bind _newparam (CallFunction|FindFootPlacement (Variables|Default|GetFrontRight) (Variables|Default|GetFRONTR)))
  (Variables|Default|SetFRONTR _newparam)
  (bind _newparam_2 (CallFunction|FindFootPlacement (Variables|Default|GetBackLeft) (Variables|Default|GetBACKL)))
  (Variables|Default|SetBACKL _newparam_2))

(event EventBeginPlay
  (CallFunction|SpawnEffect)
  (CallFunction|CheckLeft)
  (bind _asaic_enemy_base (Utilities|Casting|CastToAIC_Enemy_Base (AI|GetAIController self)))
  (bind _output_get (Variables|Default|SetAs%20AIC%20Enemy%20Base _asaic_enemy_base))
  (Variables|/Game/Blueprints/Enemies/SplineEnemy/AI/AIC_Enemy_Base.AIC_Enemy_Base_C|SetSoundFX _output_get (Variables|Default|GetSoundsToPlay))
  (Variables|Default|SetHealth (Variables|Default|GetMaxHealth))
  (Variables|/Game/ThirdPerson/Equipment/TraceComponent_Hook.TraceComponent_Hook_C|Sethook (Variables|Default|GetTraceComponent_Hook) self))

(event EventAttack
  (Utilities|Time|ClearandInvalidateTimerbyHandle (stale Custom|CheckRight _returnvalue))
  (Utilities|Time|ClearandInvalidateTimerbyHandle (stale Custom|Check%20Left _returnvalue))
  (Components|Animation|PlayAnimation (Variables|Character|GetMesh) "/Game/ArtPrototype/Rigs/HookedTerror/ATK_hook1.ATK_hook1" false)
  (Utilities|FlowControl|Delay 1.1)
  (Components|Animation|SetAnimationMode (Variables|Character|GetMesh) "AnimationBlueprint" true)
  (Utilities|Array|Clear (Variables|/Game/ThirdPerson/Equipment/TraceComponent_Hook.TraceComponent_Hook_C|GetActorsToIgnore (Variables|Default|GetTraceComponent_Hook)))
  (Default|CallOnAttackEnd)
  (CallFunction|CheckLeft))

(fn ConstructionScript
  (|CallParentFunction)
  (Utilities|FlowControl|Sequence
    (:then_0
      (bind _newparam (CallFunction|FindFootPlacement (Variables|Default|GetFrontLeft) (Variables|Default|GetFRONTL)))
      (Variables|Default|SetFRONTL _newparam)
      (bind _newparam_2 (CallFunction|FindFootPlacement (Variables|Default|GetBackRight) (Variables|Default|GetBACKR)))
      (Variables|Default|SetBACKR _newparam_2))
    (:then_1
      (bind _newparam_3 (CallFunction|FindFootPlacement (Variables|Default|GetFrontRight) (Variables|Default|GetFRONTR)))
      (Variables|Default|SetFRONTR _newparam_3)
      (bind _newparam_4 (CallFunction|FindFootPlacement (Variables|Default|GetBackLeft) (Variables|Default|GetBACKL)))
      (Variables|Default|SetBACKL _newparam_4))
    (:then_2
      (Variables|/Game/ThirdPerson/Equipment/TraceComponent_Hook.TraceComponent_Hook_C|Sethook (Variables|Default|GetTraceComponent_Hook) self))))

(fn GetIdealRange
  (return (Variables|Default|GetAttack%20Rad) (Variables|Default|GetDefend%20Rad)))

(fn SetMovementSpeed
  (params (Speed :type E_MoveSpeed%20Enum :default "NewEnumerator0"))
  (bind _output_get (Variables|/Script/Engine.CharacterMovementComponent|SetMaxWalkSpeed (Variables|Character|GetCharacterMovement) (Utilities|Select :Index Speed :NewEnumerator0 (Variables|Default|GetIdle) :NewEnumerator1 (Variables|Default|GetWalking) :NewEnumerator2 (Variables|Default|GetJogging) :NewEnumerator3 (Variables|Default|GetSprinting))))
  (return _output_get))

(fn FindFootPlacement
  (params (Target :type Scene%20Component%20Object%20Reference) (Currlocation :type Vector))
  (bind _returnvalue (Transformation|GetWorldLocation Target))
  (bind (_outhit _returnvalue_2) (Collision|LineTraceByChannel (Transformation|GetWorldLocation Target) (Math|Vector|MakeVector (.x _returnvalue) (.y _returnvalue) (- (.z _returnvalue) 5e+02)) "TraceTypeQuery1" false (Utilities|Array|MakeArray self (Game|GetPlayerCharacter 0)) "None"))
  (if _returnvalue_2
    (if (> (Math|Vector|Distance(Vector) Currlocation (.location _outhit)) 1.5e+02)
      (Audio|PlaySoundatLocation "/Game/Audio/Footsteps/Default/SQ_FootDefault.SQ_FootDefault" (.location _outhit) "0, 0, 0" 1.0 1.0 0.0 0 0 0 0)
      (return (.location _outhit))
      (else
        (return (.location _outhit))))))

(fn DeathFunc
  (|CallParentFunction))