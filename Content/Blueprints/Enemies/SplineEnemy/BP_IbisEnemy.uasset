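; Ibis enemy Blueprint that attacks by lunging at the player, extending a parent enemy class.
; After a short wind-up it launches toward the player, applies damage if its hitbox overlaps them, then signals attack end.
; Damage handling adds one-shot calls for health bands bounded at 80, 60 and 50 percent.
; A random montage macro favors the full combo over the upward attack; death adds a debug print.
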(event Custom|Calculate%20Direction
  (bind _output_get (Variables|Default|SetplayerPos (Transformation|GetActorLocation (Game|GetPlayerCharacter 0))))
  (bind _output_get_2 (Variables|Default|SetcurrentPos (Transformation|GetActorLocation)))
  (Variables|Default|SettargetDirection (Math|Vector|Normalize (- _output_get _output_get_2))))

(event Custom|AttackEvent
  ;[1 1 1] Attack
  (Variables|Default|SetCan%20Attack false)
  (Utilities|FlowControl|Delay 1.2)
  (CallFunction|CalculateDirection)
  (Character|LaunchCharacter (* (Variables|Default|GettargetDirection) (Variables|Default|GetlaunchStrength)) false false)
  (Utilities|FlowControl|Delay 0.2)
  (bind _result (CallFunction|PlayerinHitbox))
  (if _result
    (Game|Damage|ApplyDamage (Game|GetPlayerCharacter 0) 15.0 0 self))
  (Default|CallIbisAttackEnd))

(fn ConstructionScript)

(fn Damaged
  (|CallParentFunction)
  (Utilities|FlowControl|Sequence
    (:then_1
      (if (<= (* (Variables|Default|GetMaxHealth) 0.8) (Variables|Default|GetHealth))
        (Utilities|FlowControl|DoOnce false
          (:Completed
            (Default|Call80%)))
        (elif (<= (* (Variables|Default|GetMaxHealth) 0.6) (Variables|Default|GetHealth))
          (Utilities|FlowControl|DoOnce false
            (:Completed
              (Default|Call60%)))
          (elif (<= (* (Variables|Default|GetMaxHealth) 0.5) (Variables|Default|GetHealth))
            (Utilities|FlowControl|DoOnce false
              (:Completed
                (Default|Call50%)))))))))

(fn PlayAttackAnimation
  (|CallParentFunction))

(fn DeathFunc
  (|CallParentFunction)
  (Development|PrintString "dopa down" true true "(R=1.000000,G=0.000000,B=0.005617,A=1.000000)" 5.0))

(fn PlayerinHitbox
  (return (Collision|IsOverlappingActor (Variables|Default|GetHitBox) (Game|GetPlayerCharacter 0) :!class /Script/Engine.PrimitiveComponent)))