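; Boss hand slam attack actor that materializes, telegraphs, then slams toward the player's captured position.
; A looping timer turns the mesh toward the player while a timeline fades it in through a material mask.
; After a delay it locks the aim location, shakes, then lunges with a camera shake and fades out by reversing that timeline as its lifespan runs out.
; The first mesh hit applies damage, gated by DoOnce.
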(event OnComponentHit(StaticMesh)
  (params (HitComponent :type Primitive%20Component%20Object%20Reference) (OtherActor :type Actor%20Object%20Reference) (OtherComp :type Primitive%20Component%20Object%20Reference) (NormalImpulse :type Vector :default "0, 0, 0") (Hit :type Hit%20Result%20Structure%20%28by%20ref%29))
  (Utilities|FlowControl|DoOnce false
    (:Completed
      (Game|Damage|ApplyDamage OtherActor 45.0 0 0 "/Script/Engine.DamageType"))))

(event Custom|Fade%20In
  ;[1 1 1] material fade in
  (bind _mask (Timeline|fadeIn PlayFromStart)
    (:Update
      (Rendering|Material|SetScalarParameterValueonMaterials (Variables|Default|GetStaticMesh) "mask" _mask))
    (:Finished
      (Utilities|FlowControl|Delay 2.0)
      (Utilities|FlowControl|Sequence
        (:then_0
          (bind _output_get (Variables|Default|SetAim%20Location (Transformation|GetActorLocation (Game|GetPlayerCharacter 0))))
          (Utilities|Time|ClearandInvalidateTimerbyHandle (Variables|Default|GetLookTowards%20Handle))
          (bind _newtrack_0 (Timeline|Shake Play)
            (:Update
              (Transformation|AddLocalOffset (Variables|Default|GetStaticMesh) (Math|Vector|Lerp(Vector) "0, 0, 0" "15.000000,0.000000,0.000000" _newtrack_0) false false))))
        (:then_1
          (Utilities|FlowControl|Delay 1.5)
          (Utilities|FlowControl|Sequence
            (:then_0
              (Timeline|Shake Stop))
            (:then_1
              (Components|MoveComponentTo (Variables|Default|GetStaticMesh) _output_get "0, 0, 0" true true 0.3 false)
              (Default|CameraShake (CallFunction|GetMyPlayerCharacter) true)
              (CallFunction|FadeOut))))))))

(event Custom|Turn%20Towards%20player
  (bind _staticmesh (Variables|Default|GetStaticMesh))
  (Components|MoveComponentTo _staticmesh (Variables|/Script/Engine.SceneComponent|GetRelativeLocation _staticmesh) (Math|Rotator|MakeRotator 0.0 0.0 (+ (.yaw (Math|Rotator|FindLookatRotation (Transformation|GetActorLocation) (Transformation|GetActorLocation (Game|GetPlayerCharacter 0)))) 9e+01)) true true 0.2 false))

(event Custom|Fade%20Out
  ;[1 1 1] material fade in
  (Actor|SetLifeSpan 5.0)
  (bind _mask (Timeline|fadeIn ReverseFromEnd)
    (:Update
      (Rendering|Material|SetScalarParameterValueonMaterials (Variables|Default|GetStaticMesh) "mask" _mask))
    (:Finished
      (Utilities|FlowControl|Delay 2.0)
      (Utilities|FlowControl|Sequence
        (:then_0
          (bind _output_get (Variables|Default|SetAim%20Location (Transformation|GetActorLocation (Game|GetPlayerCharacter 0))))
          (Utilities|Time|ClearandInvalidateTimerbyHandle (Variables|Default|GetLookTowards%20Handle))
          (bind _newtrack_0 (Timeline|Shake Play)
            (:Update
              (Transformation|AddLocalOffset (Variables|Default|GetStaticMesh) (Math|Vector|Lerp(Vector) "0, 0, 0" "15.000000,0.000000,0.000000" _newtrack_0) false false))))
        (:then_1
          (Utilities|FlowControl|Delay 1.5)
          (Utilities|FlowControl|Sequence
            (:then_0
              (Timeline|Shake Stop))
            (:then_1
              (Components|MoveComponentTo (Variables|Default|GetStaticMesh) _output_get "0, 0, 0" true true 0.3 false)
              (Default|CameraShake (CallFunction|GetMyPlayerCharacter) true)
              (CallFunction|FadeOut))))))))

(event EventBeginPlay
  (CallFunction|Fadein)
  (bind _returnvalue (Utilities|Time|SetTimerbyEvent (delegate Custom|Turn%20Towards%20player) 0.5 true))
  (Variables|Default|SetLookTowards%20Handle _returnvalue))

(fn ConstructionScript)