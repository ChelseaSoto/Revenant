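; Boss attack base actor, in the Bosshand enemy folder, that fades in, slams toward the player and removes itself.
; A looping timer turns it toward the player until the strike, when component moves rotate the mesh and root with a camera shake.
; The mesh deals damage on its first hit.
; One timeline drives the material mask both ways; its Finished pin launches the attack, then destroys the actor after fade-out via a resettable DoOnce.
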(event OnComponentHit(StaticMesh)
  (params (HitComponent :type Primitive%20Component%20Object%20Reference) (OtherActor :type Actor%20Object%20Reference) (OtherComp :type Primitive%20Component%20Object%20Reference) (NormalImpulse :type Vector :default "0, 0, 0") (Hit :type Hit%20Result%20Structure%20%28by%20ref%29))
  (Utilities|FlowControl|DoOnce false
    (:Completed
      (Game|Damage|ApplyDamage OtherActor 45.0 0 0 "/Script/Engine.DamageType"))))

(event Custom|Fade%20In
  ;[1 1 1] material fade in
  (bind _mask (Timeline|fadeIn PlayFromStart)
    (:Update
      (Rendering|Material|SetScalarParameterValueonMaterials (Variables|Default|GetStaticMesh) "mask" _mask))
    (:Finished
      (CallFunction|LaunchAttack)
      (Utilities|FlowControl|DoOnce true
        (:Completed
          (Actor|DestroyActor))))))

(event Custom|LaunchAttack
  (bind _staticmesh (Variables|Default|GetStaticMesh))
  (bind _defaultsceneroot (Variables|Default|GetDefaultSceneRoot))
  (bind _relativelocation (Variables|/Script/Engine.SceneComponent|GetRelativeLocation _staticmesh))
  (Utilities|FlowControl|Delay 0.75)
  (Components|MoveComponentTo _staticmesh _relativelocation (Math|Rotator|MakeRotator 9e+01 0.0 (+ (.yaw (Math|Rotator|FindLookatRotation _relativelocation (Transformation|GetActorLocation (Game|GetPlayerCharacter 0)))) 45.0)) true true 0.5 false)
  (Utilities|FlowControl|Sequence
    (:then_0
      (Utilities|FlowControl|Delay 0.5)
      (Utilities|Time|ClearandInvalidateTimerbyHandle (Variables|Default|GetLookTowards%20Handle))
      (Components|MoveComponentTo _defaultsceneroot (Variables|/Script/Engine.SceneComponent|GetRelativeLocation _defaultsceneroot) (Math|Rotator|MakeRotator 0.0 -9e+01 (- (.yaw (Transformation|GetActorRotation)) 9e+01)) true true 0.2 false)
      (Default|CameraShake (CallFunction|GetMyPlayerCharacter) true)
      (Utilities|FlowControl|Delay 1.2)
      (CallFunction|FadeOut))
    (:then_1
      (Utilities|FlowControl|DoOnce true) ; enters at Reset
    )))

(event Custom|Turn%20Towards%20player
  (Transformation|SetActorRotation (Math|Rotator|MakeRotator 0.0 0.0 (+ (.yaw (Math|Rotator|FindLookatRotation (Transformation|GetActorLocation) (Transformation|GetActorLocation (Game|GetPlayerCharacter 0)))) 9e+01))))

(event Custom|Fade%20Out
  ;[1 1 1] material fade in
  (bind _mask (Timeline|fadeIn ReverseFromEnd)
    (:Update
      (Rendering|Material|SetScalarParameterValueonMaterials (Variables|Default|GetStaticMesh) "mask" _mask))
    (:Finished
      (CallFunction|LaunchAttack)
      (Utilities|FlowControl|DoOnce true
        (:Completed
          (Actor|DestroyActor))))))

(event EventBeginPlay
  (CallFunction|Fadein)
  (bind _returnvalue (Utilities|Time|SetTimerbyEvent (delegate Custom|Turn%20Towards%20player) 0.75 true))
  (Variables|Default|SetLookTowards%20Handle _returnvalue))

(fn ConstructionScript)