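; Boss hand slam enemy that fades in via a material mask, tracks the player's yaw, then shakes and lunges through their last sampled position before fading out.
; A fast looping timer runs sphere traces at the hand socket to damage the player, gated by CanHurt.
; Damaging the socket-attached child actor cancels tracking and triggers a shake and fade-out death.
; Hit-stop functions briefly freeze the actor's time dilation with a camera shake.
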(event OnComponentBeginOverlap(SkeletalMesh)
  (params (OverlappedComponent :type Primitive%20Component%20Object%20Reference) (OtherActor :type Actor%20Object%20Reference) (OtherComp :type Primitive%20Component%20Object%20Reference) (OtherBodyIndex :type Integer) (bFromSweep :type Boolean) (SweepResult :type Hit%20Result%20Structure%20%28by%20ref%29)))

(event Custom|Fade%20In
  ;[1 1 1] material fade in
  (bind _mask (Timeline|fadeIn PlayFromStart)
    (:Update
      (Rendering|Material|SetScalarParameterValueonMaterials (Variables|Default|GetSkeletalMesh) "mask" _mask))
    (:Finished
      (Utilities|FlowControl|Delay 2.0)
      (Utilities|FlowControl|Sequence
        (:then_0
          (Variables|Default|SetAim%20Location (Transformation|GetActorLocation (Game|GetPlayerCharacter 0)))
          (Utilities|Time|ClearandInvalidateTimerbyHandle (Variables|Default|GetLookTowards%20Handle))
          (bind _newtrack_0 (Timeline|Shake Play)
            (:Update
              (Transformation|AddLocalOffset (Variables|Default|GetSkeletalMesh) (Math|Vector|Lerp(Vector) "0, 0, 0" "15.000000,0.000000,0.000000" _newtrack_0) false false))))
        (:then_1
          (Utilities|FlowControl|Delay 0.75)
          (Utilities|FlowControl|Sequence
            (:then_0
              (Timeline|Shake Stop))
            (:then_1
              (Variables|Default|Setattack? true)
              (Components|MoveComponentTo (Variables|Default|GetSkeletalMesh) (+ (* (Math|Vector|GetUnitDirection(Vector) (Transformation|GetWorldLocation (Variables|Default|GetSkeletalMesh)) (Variables|Default|GetAim%20Location)) 2e+02) (Variables|Default|GetAim%20Location)) (Transformation|GetWorldRotation (Variables|Default|GetSkeletalMesh)) true false 1.5 false)
              (Default|CameraShake (CallFunction|GetMyPlayerCharacter) true)
              (CallFunction|FadeOut)
              (Variables|Default|SetcanHurt? false))))))))

(event Custom|Death
  (params (DamagedActor :type Actor%20Object%20Reference) (Damage :type Float%20%28single-precision%29) (DamageType :type Damage%20Type%20Object%20Reference) (InstigatedBy :type Controller%20Object%20Reference) (DamageCauser :type Actor%20Object%20Reference))
  (Utilities|Time|ClearandInvalidateTimerbyHandle (Variables|Default|GetLookTowards%20Handle))
  (CallFunction|FadeOut)
  (bind _newtrack_0 (Timeline|Shake PlayFromStart)
    (:Update
      (Transformation|AddLocalOffset (Variables|Default|GetSkeletalMesh) (Math|Vector|Lerp(Vector) "0, 0, 0" "15.000000,0.000000,0.000000" _newtrack_0) false false))))

(event Custom|Turn%20Towards%20player
  (bind _skeletalmesh (Variables|Default|GetSkeletalMesh))
  (Components|MoveComponentTo _skeletalmesh (Variables|/Script/Engine.SceneComponent|GetRelativeLocation _skeletalmesh) (Math|Rotator|MakeRotator 0.0 0.0 (- (.yaw (Math|Rotator|FindLookatRotation (Transformation|GetActorLocation) (Transformation|GetActorLocation (Game|GetPlayerCharacter 0)))) 9e+01)) true true 0.2 false))

(event Custom|Fade%20Out
  ;[1 1 1] material fade in
  (Actor|SetLifeSpan self 5.0)
  (bind _mask (Timeline|fadeIn ReverseFromEnd)
    (:Update
      (Rendering|Material|SetScalarParameterValueonMaterials (Variables|Default|GetSkeletalMesh) "mask" _mask))
    (:Finished
      (Utilities|FlowControl|Delay 2.0)
      (Utilities|FlowControl|Sequence
        (:then_0
          (Variables|Default|SetAim%20Location (Transformation|GetActorLocation (Game|GetPlayerCharacter 0)))
          (Utilities|Time|ClearandInvalidateTimerbyHandle (Variables|Default|GetLookTowards%20Handle))
          (bind _newtrack_0 (Timeline|Shake Play)
            (:Update
              (Transformation|AddLocalOffset (Variables|Default|GetSkeletalMesh) (Math|Vector|Lerp(Vector) "0, 0, 0" "15.000000,0.000000,0.000000" _newtrack_0) false false))))
        (:then_1
          (Utilities|FlowControl|Delay 0.75)
          (Utilities|FlowControl|Sequence
            (:then_0
              (Timeline|Shake Stop))
            (:then_1
              (Variables|Default|Setattack? true)
              (Components|MoveComponentTo (Variables|Default|GetSkeletalMesh) (+ (* (Math|Vector|GetUnitDirection(Vector) (Transformation|GetWorldLocation (Variables|Default|GetSkeletalMesh)) (Variables|Default|GetAim%20Location)) 2e+02) (Variables|Default|GetAim%20Location)) (Transformation|GetWorldRotation (Variables|Default|GetSkeletalMesh)) true false 1.5 false)
              (Default|CameraShake (CallFunction|GetMyPlayerCharacter) true)
              (CallFunction|FadeOut)
              (Variables|Default|SetcanHurt? false))))))))

(event Custom|StartAttack
  (CallFunction|Fadein)
  (bind _returnvalue (Utilities|Time|SetTimerbyEvent (delegate Custom|Turn%20Towards%20player) 0.5 true))
  (Variables|Default|SetLookTowards%20Handle _returnvalue)
  (EventDispatchers|BindEventtoOnTakeAnyDamage (Variables|/Script/Engine.ChildActorComponent|GetChildActor (Variables|Default|GetChildActor)) (delegate Custom|Death)))

(event Custom|Trace
  (bind _returnvalue (Game|Player|GetPlayerPawn 0))
  (bind _skeletalmesh (Variables|Default|GetSkeletalMesh))
  (bind _returnvalue_2 (Transformation|GetSocketTransform _skeletalmesh "Slot" "RTS_World"))
  (bind (_outhits _returnvalue_3) (Collision|MultiSphereTraceForObjects (.location _returnvalue_2) (.location _returnvalue_2) 2e+02 (Utilities|Array|MakeArray "ObjectTypeQuery3") false 0 "None"))
  (if _returnvalue_3
    (for _array_element _outhits
      (if (and (== (.hitactor _array_element) _returnvalue) (Variables|Default|GetcanHurt?))
        (Variables|Default|SetcanHurt? false)
        (Utilities|FlowControl|DoOnce false
          (:Completed
            (Game|Damage|ApplyDamage _returnvalue 2e+01 0 self "/Script/Engine.DamageType")))))))

(event EventBeginPlay
  (Transformation|AttachComponentToComponent (Variables|Default|GetChildActor) (Variables|Default|GetSkeletalMesh) "slot" "SnapToTarget" "SnapToTarget" "KeepRelative" true))

(event EventStartAttack
  (bind _returnvalue (Utilities|Time|SetTimerbyEvent (delegate Custom|Trace) 0.001 true))
  (Variables|Default|SetTra _returnvalue))

(event EventEndAttack
  (Utilities|Time|ClearandInvalidateTimerbyHandle (Variables|Default|GetTra)))

(fn ConstructionScript)

(fn StartHitStop
  (Camera|PlayWorldCameraShake "/Game/Blueprints/Player/Effects/BP_CamShakeSmall.BP_CamShakeSmall_C" (Transformation|GetWorldLocation (Variables|/Script/Engine.Character|GetMesh (CallFunction|GetMyPlayerCharacter))) 0.0 1e+03)
  (Variables|Default|SetCustomTimeDilation 0.0)
  (Utilities|Time|SetTimerbyFunctionName 0 "End Hit Stop" 0.0 false 0.1 0.08))

(fn EndHitStop
  (Variables|Default|SetCustomTimeDilation 1.0))