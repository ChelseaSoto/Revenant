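; Seth boss enemy that chases the player, summons shadow minions and removes them in smoke bursts on death.
; Damage below a threshold under its regen cap triggers a timed bubble that blocks damage, regenerates health and halts new move orders, followed by a cooldown.
; Each bubble spawns mage or melee adds at mirrored offsets, balancing types up to an enemy limit.
; Tick drives both movement and regeneration; CurrentPhase is set but never read.
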(event Custom|Make%20Smoke
  (params (Child%20Location :type Vector))
  (Niagara|SpawnSystematLocation "/Game/VFX/FireVFX/NS_SethSmokeBurst.NS_SethSmokeBurst" Child%20Location))

(event Custom|Move
  ;[1 1 1] Movement
  (AI|AIMoveTo self "0, 0, 0" (Game|GetPlayerCharacter 0) 1.5e+02 false))

(event EventBeginPlay
  (Variables|Default|SetCurrentPhase "NewEnumerator1"))

(event EventTick
  (params (DeltaSeconds :type Float%20%28single-precision%29))
  ;[1 1 1] Checking if conditions are met to bubble
  (if (Variables|Default|GetInBubble)
    (CallFunction|RegenerateHealth)
    (else
      (CallFunction|Move))))

(event Game|Damage|EventAnyDamage
  (params (Damage :type Float%20%28single-precision%29) (DamageType :type Damage%20Type%20Object%20Reference) (InstigatedBy :type Controller%20Object%20Reference) (DamageCauser :type Actor%20Object%20Reference))
  ;[1 1 1] When taking damage
  (if (Variables|Default|GetInBubble)
    (Development|PrintString "Shielded damage")
    (else
      (bind _output_get (Variables|Default|SetHealth (- (Variables|Default|GetHealth) Damage)))
      (if (>= _output_get 0.0)
        (if (and (Variables|Default|GetCanBubble) (< (Variables|Default|GetHealth) (- (Variables|Default|GetHealthRegenCap) 2e+01)))
          (CallFunction|Bubble)
          (Variables|Default|SetCanBubble false)
          (else
            (Development|PrintString "Current health: ")
            (Development|PrintString (Utilities|String|ToString(Float) (Variables|Default|GetHealth)))))
        (else
          (Utilities|FlowControl|DoOnce false
            (:Completed
              (for _array_element (Variables|Default|GetSpawnedEnemies)
                (CallFunction|MakeSmoke (Transformation|GetActorLocation _array_element))
                (Actor|DestroyActor _array_element))
              (Actor|DestroyActor))))))))

(event Custom|Bubble
  ;[1 1 1] Bubble and health recovery
  (Variables|Default|SetInBubble true)
  (Development|PrintString "In Bubble" true true "(R=0.552997,G=0.000000,B=1.000000,A=1.000000)")
  (CallFunction|SpawnAdds)
  (Utilities|FlowControl|Delay 3.0)
  (Variables|Default|SetInBubble false)
  (Development|PrintString "Bubble Complete" true true "(R=0.261148,G=1.000000,B=0.000000,A=1.000000)")
  (Utilities|FlowControl|Delay 5.0)
  (Variables|Default|SetCanBubble true)
  (Development|PrintString "Can Bubble!" true true "(R=1.000000,G=0.000000,B=0.099285,A=1.000000)"))

(event Custom|RegenerateHealth
  ;[1 1 1] Handling health regeneration when in bubble
  (bind _output_get (Variables|Default|SetHealth (Math|Interpolation|FInterptoConstant (Variables|Default|GetHealth) (Variables|Default|GetHealthRegenCap) (Utilities|Time|GetWorldDeltaSeconds) (Variables|Default|GetHealthRecoveryRate))))
  (Development|PrintString (Utilities|String|ToString(Float) _output_get) true true "(R=0.658308,G=1.000000,B=0.701410,A=1.000000)"))

(event Custom|Spawn%20Adds
  (bind _maxenemies (Variables|Default|GetMaxEnemies))
  (bind _magecount (Variables|Default|GetMageCount))
  (bind _meleecount (Variables|Default|GetMeleeCount))
  (bind _returnvalue (+ _magecount _meleecount))
  ;[1 1 1] Spawns two enemies when entering bubble
  ;;[1 1 1] ???
  (if (not (>= _returnvalue _maxenemies))
    (if (== _returnvalue (- _maxenemies 2))
      (CallFunction|SpawnMage)
      (CallFunction|SpawnMelee)
      (elif (> (Variables|Default|GetMageCount) (Variables|Default|GetMeleeCount))
        (CallFunction|SpawnMelee)
        (else
          (CallFunction|SpawnMage))))))

(event Custom|Spawn%20Mage
  (bind _returnvalue (Transformation|GetActorTransform))
  ;[1 1 1] Spawns mage enemy
  (bind _returnvalue_2 (Game|SpawnActorfromClass "/Game/Blueprints/Enemies/Blueprints/BP_ShadowMage.BP_ShadowMage_C" (Math|Transform|MakeTransform (+ (.location _returnvalue) (Variables|Default|GetLocationOffset)) (.rotation _returnvalue) "1.000000,1.000000,1.000000") "Undefined" "MultiplyWithRoot" self 0))
  (Utilities|Array|Add (Variables|Default|GetSpawnedEnemies) _returnvalue_2)
  (Pawn|SpawnDefaultController _returnvalue_2)
  (bind _result (Math|Integer|IncrementInt (Variables|Default|GetMageCount))
    (:%20%20
      (Variables|Default|SetMageCount _result))))

(event Custom|Spawn%20Melee
  (bind _returnvalue (Transformation|GetActorTransform))
  (bind _locationoffset (Variables|Default|GetLocationOffset))
  ;[1 1 1] Spawns melee enemy
  (bind _returnvalue_2 (Game|SpawnActorfromClass "/Game/Blueprints/Enemies/Blueprints/BP_ShadowMelee.BP_ShadowMelee_C" (Math|Transform|MakeTransform (+ (.location _returnvalue) (Math|Vector|MakeVector (* (.x _locationoffset) -1.0) (* (.y _locationoffset) -1.0) (.z _locationoffset))) (.rotation _returnvalue) "1.000000,1.000000,1.000000") "Undefined" "MultiplyWithRoot" self 0))
  (Utilities|Array|Add (Variables|Default|GetSpawnedEnemies) _returnvalue_2)
  (Pawn|SpawnDefaultController _returnvalue_2)
  (bind _result (Math|Integer|IncrementInt (Variables|Default|GetMeleeCount))
    (:%20%20
      (Variables|Default|SetMeleeCount _result))))

(fn ConstructionScript)