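; Projectile for the mage enemy that damages the player on contact.
; On BeginPlay it sets a five-second lifespan and launches along its owner's forward vector by setting the ProjectileMovement velocity directly.
; Overlapping the player deals damage proportional to their health, half of it clamped to a fixed range, through PlayerTakeDamage, then destroys the projectile.
; Other overlapping actors are ignored.
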(event EventBeginPlay
  ;[1 1 1] This works to set the speed of the projectile in the correct direction but I don't really like it
  (Actor|SetLifeSpan 5.0)
  (Variables|/Script/Engine.MovementComponent|SetVelocity (Variables|Default|GetProjectileMovement) (* (Transformation|GetActorForwardVector (Components|GetOwner)) (Variables|Default|GetProjectileSpeedFix))))

(event Collision|EventActorBeginOverlap
  (params (OtherActor :type Actor%20Object%20Reference))
  (bind _returnvalue (Game|GetPlayerCharacter 0))
  (if (== OtherActor _returnvalue)
    (bind _asbp_third_person_character (Utilities|Casting|CastToBP_ThirdPersonCharacter _returnvalue))
    (Default|PlayerTakeDamage _asbp_third_person_character (Math|Float|Clamp(Float) (/ (Variables|/Game/ThirdPerson/Blueprints/BP_ThirdPersonCharacter.BP_ThirdPersonCharacter_C|GetHealth _asbp_third_person_character) 2.0) 1e+01 5e+01))
    (Actor|DestroyActor)))

(fn ConstructionScript)