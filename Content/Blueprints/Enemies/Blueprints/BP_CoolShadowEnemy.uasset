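; BP_CoolShadowEnemy is an enemy that chases the player and jitters erratically once its PawnSensing detects a pawn.
; Each sighting sets IsSeeingPlayer, which this graph never clears, and calls FollowPlayer to issue an AI MoveTo toward player 0.
; FreakMode fires as soon as that move request is issued, not on arrival, teleporting the enemy by a random horizontal offset.
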(event OnSeePawn(PawnSensing)
  (params (Pawn :type Pawn%20Object%20Reference))
  (Variables|Default|SetisSeeingPlayer? true)
  (CallFunction|FollowPlayer))

(event Custom|Follow%20Player
  (if (Variables|Default|GetisSeeingPlayer?)
    (AI|AIMoveTo self "0, 0, 0" (Game|GetPlayerCharacter 0) 5.0 false
      (:then
        (CallFunction|FreakMode)))))

(event Custom|Freak%20Mode
  (Transformation|AddActorWorldOffset (Math|Vector|MakeVector (Math|Random|RandomFloatinRange -1e+02 1e+02) (Math|Random|RandomFloatinRange -1e+02 1e+02) 0.0) false true))

(event EventBeginPlay)

(event Collision|EventActorBeginOverlap
  (params (OtherActor :type Actor%20Object%20Reference)))

(event EventTick
  (params (DeltaSeconds :type Float%20%28single-precision%29)))

(fn ConstructionScript)