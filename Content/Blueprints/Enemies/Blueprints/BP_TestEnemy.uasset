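; BP_TestEnemy is a sword-wielding skeleton enemy that runs BT_Skeleton and supports player lock-on.
; Pawn sensing, damage and leaving the sphere overlap set a behavior enum, mirrored to the Blackboard.
; Damage triggers hit stop through custom time dilation and camera shake, plus a hit reaction with delayed return to combat.
; Death stops AI logic, plays a montage, then ragdolls and releases lock-on; attacks play random montages.
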(event OnSeePawn(PawnSensing)
  (params (Pawn :type Pawn%20Object%20Reference))
  ;[1 1 1] Detect the player with PawnSensing. // Antonio
  (if (and (== Pawn (Game|GetPlayerCharacter 0)) (Utilities|Enum|NotEqual(Enum) (Variables|Default|GetBehavior) "NewEnumerator0"))
    (Variables|Default|SetBehavior "NewEnumerator3")
    (AI|Components|Blackboard|SetValueasEnum (AI|GetBlackboard 0) (Utilities|Name|MakeLiteralName "EBehavior") (Variables|Default|GetBehavior))))

(event OnComponentEndOverlap(Sphere)
  (params (OverlappedComponent :type Primitive%20Component%20Object%20Reference) (OtherActor :type Actor%20Object%20Reference) (OtherComp :type Primitive%20Component%20Object%20Reference) (OtherBodyIndex :type Integer))
  ;[1 1 1] If the Player is too far away from the Enemy, the Enemy enters Idle state. // Antonio
  (Utilities|Casting|CastToBP_ThirdPersonCharacter OtherActor)
  (Variables|Default|SetBehavior "NewEnumerator1")
  (AI|Components|Blackboard|SetValueasEnum (AI|GetBlackboard 0) (Utilities|Name|MakeLiteralName "EBehavior") (Variables|Default|GetBehavior)))

(event Custom|Attack
  ;[1 1 1] Play a random attack animation montage. // Antonio
  (bind _returnvalue (Animation|PlayAnimMontage (.OutItem (Utilities|Array|Random (Variables|Default|GetAttackAnimations))) 1.0 "None"))
  (Variables|Default|SetAttackLength _returnvalue))

(event Custom|Clear%20Hit%20Actors
  (Utilities|Array|Clear (Variables|/Game/ThirdPerson/Equipment/TraceComponent.TraceComponent_C|GetActorsToIgnore (Variables|Default|GetTraceComponent))))

(event Custom|ShakeMesh
  (bind _mesh (Variables|Character|GetMesh))
  (bind _relativelocation (Variables|/Script/Engine.SceneComponent|GetRelativeLocation _mesh))
  (bind _isa (Utilities|FlowControl|FlipFlop)
    (:A
      _)
    (:B
      _))
  (Transformation|SetRelativeLocation (Variables|Character|GetMesh) (Math|Vector|MakeVector (+ (.x _relativelocation) (Math|Float|SelectFloat (* -1.0 0.0) 0.0 _isa)) (+ (.y _relativelocation) (Math|Float|SelectFloat (* -1.0 0.0) 0.0 _isa)) (.z _relativelocation)) false false))

(event EventBeginPlay
  ;[1 1 1] Set up Enemy and start up Behavior Tree. // Antonio
  (Rendering|SetVisibility (Variables|Default|GetLock-on) false false)
  (AI|RunBehaviorTree (AI|GetAIController self) "/Game/Blueprints/Enemies/BehaviorTree/BT_Skeleton.BT_Skeleton")
  (bind _returnvalue (Game|SpawnActorfromClass (Variables|Default|Getsword) (Transformation|GetSocketTransform (Variables|Character|GetMesh) "sword" "RTS_World") "Undefined" "MultiplyWithRoot" 0 0))
  (bind _asbp_base_sword (Utilities|Casting|CastToBP_BaseSword _returnvalue))
  (bind _output_get (Variables|Default|SetSwordReference _asbp_base_sword))
  (Transformation|AttachComponentToComponent _output_get (Variables|Character|GetMesh) "sword" "SnapToTarget" "SnapToTarget" "SnapToTarget" true)
  (Variables|/Game/ThirdPerson/Equipment/TraceComponent.TraceComponent_C|Setswordref (Variables|Default|GetTraceComponent) (Variables|Default|GetSwordReference))
  (bind _asbp_third_person_character (Utilities|Casting|CastToBP_ThirdPersonCharacter (Game|GetPlayerCharacter 0)))
  (Variables|Default|SetPlayerReference _asbp_third_person_character)
  (AI|Components|Blackboard|SetValueasEnum (AI|GetBlackboard 0) (Utilities|Name|MakeLiteralName "EBehavior") (Variables|Default|GetBehavior))
  (Variables|/Game/ThirdPerson/Equipment/RotatingComponent.RotatingComponent_C|Settarget (Variables|Default|GetRotatingComponent) (Game|GetPlayerCharacter 0))
  (bind _outactors (Actor|GetAllActorswithTag "enemy"))
  (Variables|/Game/ThirdPerson/Equipment/TraceComponent.TraceComponent_C|Setenemy (Variables|Default|GetTraceComponent) _outactors))

(event Collision|EventActorBeginOverlap
  (params (OtherActor :type Actor%20Object%20Reference))
  ;[1 1 1] Set up Enemy and start up Behavior Tree. // Antonio
)

(event Game|Damage|EventAnyDamage
  (params (Damage :type Float%20%28single-precision%29) (DamageType :type Damage%20Type%20Object%20Reference) (InstigatedBy :type Controller%20Object%20Reference) (DamageCauser :type Actor%20Object%20Reference))
  (bind _my_player_character (CallFunction|GetMyPlayerCharacter))
  (bind _playerreference (Variables|Default|GetPlayerReference))
  (bind _targetactor (Variables|/Game/ThirdPerson/Blueprints/BP_ThirdPersonCharacter.BP_ThirdPersonCharacter_C|GetTargetActor _playerreference))
  ;[1 1 1] Enemy Takes Damage System. // Antonio
  (if (Utilities|String|Contains (Utilities|GetDisplayName DamageCauser) "ThirdPerson")
    (Default|StartHitStop _my_player_character 0.1)
    (Default|CameraShake _my_player_character false))
  (Default|CallDamageDispatch Damage)
  (Variables|Default|SetBehavior "NewEnumerator0")
  (AI|Components|Blackboard|SetValueasEnum (AI|GetBlackboard 0) (Utilities|Name|MakeLiteralName "EBehavior") (Variables|Default|GetBehavior))
  (bind _output_get (Variables|Default|Sethealth (- (Variables|Default|Gethealth) Damage)))
  (if (<= _output_get 0.0)
    (Utilities|FlowControl|DoOnce false
      (:Completed
        (Default|CallDeathDispatch)
        (AI|Logic|StopLogic (Variables|/Script/AIModule.AIController|GetBrainComponent (AI|GetAIController self)) "die")
        (Animation|PlayAnimMontage "/Game/Blueprints/Enemies/Animations/SkeletonEnemyExample/SkeleDeath_Montage.SkeleDeath_Montage" 1.0 "None")
        (Actor|SetLifeSpan 1e+01)
        (Utilities|FlowControl|RetriggerableDelay 1.5)
        (Animation|StopAnimMontage "/Game/Blueprints/Enemies/Animations/SkeletonEnemyExample/SkeleDeath_Montage.SkeleDeath_Montage")
        (Physics|SetSimulatePhysics (Variables|Character|GetMesh) true)
        (Variables|Default|SetEnemyDead? true)
        (Utilities|IsValid _targetactor
          (:Is%20Valid
            (if (== _targetactor self)
              (Default|DisengageLock-on (Variables|Default|GetPlayerReference)))))))
    (else
      (Components|Movement|StopMovementImmediately (Variables|Character|GetCharacterMovement))
      ;[1 1 1] Once the enemy is damaged, the enemy returns to combat mode after a set delay. // Antonio
      (Animation|PlayAnimMontage "/Game/Blueprints/Enemies/Animations/SkeletonEnemyExample/Skele_Hit_Montage.Skele_Hit_Montage" 1.0 "None")
      (Utilities|FlowControl|Sequence
        (:then_0
          (Utilities|FlowControl|RetriggerableDelay (Variables|Default|GetDamageTime))
          (Variables|Default|SetBehavior "NewEnumerator3")
          (AI|Components|Blackboard|SetValueasEnum (AI|GetBlackboard 0) (Utilities|Name|MakeLiteralName "EBehavior") (Variables|Default|GetBehavior)))
        (:then_1
          (if (> Damage 1e+01)
            (CallFunction|StartHitStop 0.2)
            (else
              (CallFunction|StartHitStop 0.1))))))))

(event EventOnSelected
  ;[1 1 1] Handle lock-on. // Antonio
  (Rendering|SetVisibility (Variables|Default|GetLock-on) true false))

(event EventOnDeselected
  ;[1 1 1] Handle lock-on. // Antonio
  (Rendering|SetVisibility (Variables|Default|GetLock-on) false false))

(fn ConstructionScript)

(fn StartHitStop
  (params (Time :type Float%20%28single-precision%29))
  (Camera|PlayWorldCameraShake "/Game/Blueprints/Player/Effects/BP_CamShakeSmall.BP_CamShakeSmall_C" (Transformation|GetWorldLocation (Variables|/Script/Engine.Character|GetMesh (CallFunction|GetMyPlayerCharacter))) 0.0 1e+03)
  (Variables|Default|SetCustomTimeDilation 0.0)
  (Utilities|Time|SetTimerbyFunctionName 0 "End Hit Stop" Time false 0.1 0.08))

(fn EndHitStop
  (Variables|Default|SetCustomTimeDilation 1.0))

(fn IsDead
  (return (Variables|Default|GetEnemyDead?)))