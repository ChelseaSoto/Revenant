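; Bird Vessel enemy that carries two swords and fires a Ray of Feathers attack at the player.
; BeginPlay spawns and attaches the swords to hand sockets and passes them to its trace component, along with actors tagged "enemy".
; Reported damage triggers a health check that, at zero, stops AI logic, releases player lock-on, schedules cleanup and switches to ragdoll.
; Helper functions supply movement speeds, attack and defend ranges, death state and random attack selection.
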(event Custom|TakeDamage
  (bind _playerref (Variables|Default|GetPlayerRef))
  (bind _targetactor (Variables|/Game/ThirdPerson/Blueprints/BP_ThirdPersonCharacter.BP_ThirdPersonCharacter_C|GetTargetActor _playerref))
  (if (<= (Variables|Default|GetHealth) 0.0)
    (Variables|Default|SetIsDead? true)
    (Collision|SetCollisionEnabled (Variables|Default|GetCapsuleComponent) "NoCollision")
    (Utilities|FlowControl|DoOnce false
      (:Completed
        (AI|Logic|StopLogic (Variables|/Script/AIModule.AIController|GetBrainComponent (AI|GetAIController self)) "die")
        (Variables|Default|SetEnemyDead? true)
        (Utilities|IsValid _targetactor
          (:Is%20Valid
            (if (== _targetactor self)
              (Default|DisengageLock-on (Variables|Default|GetPlayerRef) :!label _label)
              (Actor|SetLifeSpan 5.0)
              (Actor|SetLifeSpan (Variables|Default|Getswordreference2) 5.0)
              (Actor|SetLifeSpan (Variables|Default|Getswordreference3) 5.0)
              (Utilities|IsValid (Variables|Default|GetRayOfFeathersActor)
                (:Is%20Valid
                  (Actor|DestroyActor (Variables|Default|GetRayOfFeathersActor)))
                (:Is%20Not%20Valid
                  _))
              (Collision|SetCollisionResponsetoChannel (Variables|Character|GetMesh) "ECC_Pawn" "ECR_Ignore")
              (Collision|SetCollisionResponsetoChannel (Variables|Default|GetCapsuleComponent) "ECC_Pawn" "ECR_Ignore")
              (Utilities|FlowControl|RetriggerableDelay 2.2)
              (Animation|StopAnimMontage "/Game/ArtPrototype/Rigs/BirdVessel/Cleaned/Death/Bird_Vessel_Death_V2_Montage.Bird_Vessel_Death_V2_Montage")
              (Physics|SetSimulatePhysics (Variables|Character|GetMesh) true)))
          (:Is%20Not%20Valid
            (goto _label)))))))

(event Custom|Clear%20Hit%20Actors
  (Utilities|Array|Clear (Variables|/Game/ThirdPerson/Equipment/TraceComponent.TraceComponent_C|GetActorsToIgnore (Variables|Default|GetTraceComponent_BirdVessel))))

(event Custom|RayOfFeathersAttack
  (bind _returnvalue (Transformation|GetActorLocation))
  (Transformation|SetActorLocationAndRotation _returnvalue (Math|Rotator|FindLookatRotation _returnvalue (Transformation|GetActorLocation (Game|Player|GetPlayerPawn 0))))
  (Utilities|FlowControl|Delay 0.2)
  (bind _returnvalue_2 (Game|SpawnActorfromClass "/Game/Blueprints/Enemies/JackalEnemyAI/BirdVesselEnemyAI/BP_RayOfFeathers.BP_RayOfFeathers_C" (Transformation|GetWorldTransform (Variables|Default|GetArrow1)) "AlwaysSpawn" "MultiplyWithRoot" 0 0))
  (bind _output_get (Variables|Default|SetRayOfFeathersActor _returnvalue_2))
  (Actor|SetLifeSpan _output_get 8.0))

(event EventBeginPlay
  (Collision|SetCollisionResponsetoChannel (Variables|Default|GetCapsuleComponent) "ECC_Pawn" "ECR_Block")
  (bind _asbp_third_person_character (Utilities|Casting|CastToBP_ThirdPersonCharacter (Game|GetPlayerCharacter 0)))
  (Variables|Default|SetPlayerRef _asbp_third_person_character)
  (bind _returnvalue (Game|SpawnActorfromClass (Variables|Default|Getswordclassref) (Transformation|GetSocketTransform (Variables|Character|GetMesh) "SwordRight" "RTS_World") "Undefined" "MultiplyWithRoot" 0 0))
  (bind _output_get (Variables|Default|Setswordreference2 _returnvalue))
  (Transformation|AttachComponentToComponent _output_get (Variables|Character|GetMesh) "SwordRight" "SnapToTarget" "SnapToTarget" "SnapToTarget" true)
  (Variables|/Game/ThirdPerson/Equipment/TraceComponent.TraceComponent_C|Setswordref (Variables|Default|GetTraceComponent_BirdVessel) (Variables|Default|Getswordreference2))
  (bind _returnvalue_2 (Game|SpawnActorfromClass (Variables|Default|Getswordclassref) (Transformation|GetSocketTransform (Variables|Character|GetMesh) "SwordLeft" "RTS_World") "Undefined" "MultiplyWithRoot" 0 0))
  (bind _output_get_2 (Variables|Default|Setswordreference3 _returnvalue_2))
  (Transformation|AttachComponentToComponent _output_get_2 (Variables|Character|GetMesh) "SwordLeft" "SnapToTarget" "SnapToTarget" "SnapToTarget" true)
  (Variables|/Game/ThirdPerson/Equipment/TraceComponent.TraceComponent_C|Setswordrefalt (Variables|Default|GetTraceComponent_BirdVessel) (Variables|Default|Getswordreference3))
  (bind _outactors (Actor|GetAllActorswithTag "enemy"))
  (Variables|/Game/ThirdPerson/Equipment/TraceComponent.TraceComponent_C|Setenemy (Variables|Default|GetTraceComponent_BirdVessel) _outactors))

(event Collision|EventActorBeginOverlap
  (params (OtherActor :type Actor%20Object%20Reference)))

(event EventTick
  (params (DeltaSeconds :type Float%20%28single-precision%29)))

(fn ConstructionScript
  (|CallParentFunction))

(fn SetMovementSpeed
  (params (Speed :type E_MoveSpeed%20Enum :default "NewEnumerator0"))
  (bind _output_get (Variables|/Script/Engine.CharacterMovementComponent|SetMaxWalkSpeed (Variables|Character|GetCharacterMovement) (Utilities|Select :Index Speed :NewEnumerator0 (Variables|Default|GetIdle) :NewEnumerator1 (Variables|Default|GetWalking) :NewEnumerator2 (Variables|Default|GetJogging) :NewEnumerator3 (Variables|Default|GetSprinting))))
  (return _output_get))

(fn GetIdealRange
  (return (Variables|Default|GetAttack%20Rad_0) (Variables|Default|GetDefend%20Rad_0)))

(fn IsDead
  (return (Variables|Default|GetEnemyDead?)))

(fn ReportDamage
  (params (Damage%20Amount%20Taken :type Float%20%28single-precision%29) (Instigator :type Actor%20Object%20Reference))
  (bind _damage_taken (|CallParentFunction Damage%20Amount%20Taken Instigator))
  (bind _output_get (Variables|Default|SetDamage%20Taken _damage_taken))
  (CallFunction|TakeDamage)
  (return _output_get))

(fn DeathFunc
  (|CallParentFunction))

(fn GetRandomAttackNum
  (bind _output_get (LocalVariables|SetC (Math|Float|SelectFloat (LocalVariables|GetA) (LocalVariables|GetB) (Math|Random|RandomBool))))
  (Development|PrintString (Utilities|String|ToString(Float) _output_get))
  (return (LocalVariables|GetC)))