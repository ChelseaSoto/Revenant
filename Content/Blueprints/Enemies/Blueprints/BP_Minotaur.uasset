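; Minotaur melee enemy that cycles uppercut, stomp, sweep and kick attacks, and has a wind-up charge toward the player's last sampled position.
; Attacks set state flags, use timed delays for hitbox checks, then deal damage, mostly with knockback, and re-arm DoOnce gates.
; Player hits trigger camera shake and hit-stop through time dilation; zero health destroys it.
; The pawn-sensing event is empty, leaving the chase-or-charge decision logic disconnected.
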(event OnSeePawn(PawnSensing)
  (params (Pawn :type Pawn%20Object%20Reference))
  ;[1 1 1] When player is visible, calculate distance and start actions. If player is too far minotaur will start to charge
)

(event Custom|Distance%20to%20player
  ;[1 1 1] Updates the location, playerlocation, and distancetoplayer variables
  (bind _output_get (Variables|BasicStuff|SetLocation (Transformation|GetWorldLocation (Variables|Collision|GetCapsuleComponent self))))
  (bind _output_get_2 (Variables|BasicStuff|SetPlayerLocation (Transformation|GetWorldLocation (Variables|/Script/Engine.Character|GetCapsuleComponent (Game|GetPlayerCharacter 0)))))
  (Variables|BasicStuff|SetDistanceToPlayer (Math|Vector|Distance(Vector) _output_get _output_get_2)))

(event Custom|Fix%20Rotation
  ;[1 1 1] Makes enemy face player
  (CallFunction|DistancetoPlayer)
  (Transformation|SetActorRotation (Math|Rotator|FindLookatRotation (Variables|BasicStuff|GetLocation) (Variables|BasicStuff|GetPlayerLocation))))

(event Custom|Kick
  ;[1 1 1] Logic for kick
  (Development|PrintString "Play kick animation")
  (Variables|Default|SetisKicking true)
  (Utilities|FlowControl|Delay 0.65)
  (bind _result (CallFunction|PlayerinHitbox))
  (if _result
    (CallFunction|DealDamageKnockback)
    (else
      (Development|PrintString "Player not hit")))
  (Utilities|FlowControl|Delay 1.5)
  (Variables|Default|SetisKicking false)
  (Variables|AttackStats|SetCan%20Attack true)
  (CallFunction|ResetAttack))

(event Custom|Reset%20Attack%202
  ;[1 1 1] Movement that calls attack when close enough
  (Utilities|FlowControl|DoOnce false) ; enters at Reset
)

(event Custom|Sweep
  ;[1 1 1] Logic for the sweep
  (Development|PrintString "Play sweep animation")
  (Variables|Default|SetisSweeping true)
  (Utilities|FlowControl|Delay 0.85)
  (bind _result (CallFunction|PlayerinHitbox))
  (if _result
    (CallFunction|DealDamageKnockback)
    (else
      (Development|PrintString "Player not hit")))
  ;;[1 1 1] Time until minotaur stands back up
  (Utilities|FlowControl|Delay 5.3)
  (Variables|Default|SetisSweeping false)
  (Variables|AttackStats|SetCan%20Attack true)
  (CallFunction|ResetAttack))

(event Custom|Stomp
  ;[1 1 1] Logic for the stomp
  (Variables|Default|SetisStomping true)
  (Utilities|FlowControl|Delay 0.9)
  (bind _result (CallFunction|PlayerinHitbox))
  (if _result
    (bind _asbp_third_person_character (Utilities|Casting|CastToBP_ThirdPersonCharacter (Game|GetPlayerCharacter 0)))
    (Default|PlayerTakeDamage _asbp_third_person_character 2e+01)
    (else
      (Development|PrintString "Player not hit")))
  (Utilities|FlowControl|Delay 1.0)
  (Variables|Default|SetisStomping false)
  (Variables|AttackStats|SetCan%20Attack true)
  (CallFunction|ResetAttack))

(event Custom|Attack
  ;[1 1 1] Attack logic, cycles through each attack type
  (if (Variables|AttackStats|GetCan%20Attack)
    (Variables|AttackStats|SetCan%20Attack false)
    (bind _output_get (Variables|AttackStats|SetAttack%20Index (+ (Variables|AttackStats|GetAttack%20Index) 1)))
    (switch int (Math|Integer|%(Integer) _output_get 5)
      (:0
        (CallFunction|Uppercut :!label _label))
      (:1
        (CallFunction|Stomp))
      (:2
        (CallFunction|Sweep))
      (:3
        (goto _label))
      (:4
        (CallFunction|Kick)))))

(event Custom|Move
  (bind _self self)
  (bind _ischarging (Variables|ChargeAttack|GetisCharging))
  ;[1 1 1] Movement that calls attack when close enough
  (if (and (Variables|AttackStats|GetCan%20Attack) (not _ischarging))
    (if _ischarging
      (AI|AIMoveTo _self (Variables|ChargeAttack|GetChargeLocation) 0 2e+02 false :!label _label
        (:OnSuccess
          (Utilities|FlowControl|DoOnce false
            (:Completed
              (CallFunction|Uppercut)
              (CallFunction|ResetCharge)
              (Development|PrintString "charge attack")
              (Utilities|FlowControl|Delay 2.0)
              (CallFunction|ResetAttack2)))))
      (else
        (AI|AIMoveTo _self "0, 0, 0" (Game|GetPlayerCharacter 0) 2e+02 false
          (:OnSuccess
            (Utilities|FlowControl|DoOnce false
              (:Completed
                (CallFunction|Attack)
                (Development|PrintString "not charge attack")))))))
    (else
      (goto _label))))

(event Custom|Uppercut
  ;[1 1 1] Logic for the Uppercut
  (Variables|AttackStats|SetisSwiping true)
  (if (not (Variables|ChargeAttack|GetisCharging))
    ;;[1 1 1] based on anim timings
    (Utilities|FlowControl|Delay 1.1)
    (else
      (Utilities|FlowControl|Delay 0.66)))
  (bind _result (CallFunction|PlayerinHitbox))
  (if _result
    (CallFunction|DealDamageKnockback)
    (else
      (Development|PrintString "Player not hit!")))
  (Utilities|FlowControl|Delay 1.0)
  (Variables|AttackStats|SetisSwiping false)
  (Variables|AttackStats|SetCan%20Attack true)
  (CallFunction|ResetAttack))

(event Custom|Charge
  (bind _charactermovement (Variables|Character|GetCharacterMovement))
  ;[1 1 1] Logic for the charge
  (Variables|ChargeAttack|SetwindUp true)
  (Utilities|FlowControl|Delay 2.6)
  (Variables|ChargeAttack|SetwindUp false)
  (CallFunction|DistancetoPlayer)
  (Variables|ChargeAttack|SetChargeLocation (Variables|BasicStuff|GetPlayerLocation))
  (Variables|ChargeAttack|SetisCharging true)
  (Variables|/Script/Engine.CharacterMovementComponent|SetMaxWalkSpeed _charactermovement 1.25e+03)
  (Variables|/Script/Engine.CharacterMovementComponent|SetMaxAcceleration _charactermovement 3e+03)
  (if true
    ;;[1 1 1] How long he should charge for
    (Utilities|FlowControl|Delay 3.5)
    (CallFunction|ResetCharge)
    (CallFunction|ResetAttack)))

(event Custom|ResetCharge
  (bind _charactermovement (Variables|Character|GetCharacterMovement))
  (Variables|ChargeAttack|SetisCharging false)
  (Variables|/Script/Engine.CharacterMovementComponent|SetMaxWalkSpeed _charactermovement 3e+02)
  (Variables|/Script/Engine.CharacterMovementComponent|SetMaxAcceleration _charactermovement 1e+03)
  ;[1 1 1] When player is visible, calculate distance and start actions. If player is too far minotaur will start to charge
  (Utilities|FlowControl|DoOnce false) ; enters at Reset
)

(event Custom|Reset%20Attack
  ;[1 1 1] Movement that calls attack when close enough
  (Utilities|FlowControl|DoOnce false) ; enters at Reset
)

(event Game|Damage|EventAnyDamage
  (params (Damage :type Float%20%28single-precision%29) (DamageType :type Damage%20Type%20Object%20Reference) (InstigatedBy :type Controller%20Object%20Reference) (DamageCauser :type Actor%20Object%20Reference))
  ;[1 1 1] Minotaur getting hit
  (bind _output_get (Variables|BasicStuff|SetHealth (- (Variables|BasicStuff|GetHealth) Damage)))
  (if (> _output_get 0.0)
    (if (== DamageCauser (Game|Player|GetPlayerPawn 0))
      (CallFunction|HitStop 0.1))
    (else
      (Actor|DestroyActor))))

(event EventOnSelected
  ;[1 1 1] Handles lock-on
  (Rendering|SetVisibility (Variables|Default|GetLockOn) true false))

(event EventOnDeselected
  ;[1 1 1] Handles lock-on
  (Rendering|SetVisibility (Variables|Default|GetLockOn) false false))

(fn ConstructionScript
  (Transformation|AttachComponentToComponent (Variables|Default|GetNiagara) (Variables|Character|GetMesh) "JawSocket" "SnapToTarget" "SnapToTarget" "KeepWorld" true))

(fn PlayerinHitbox
  (return (Collision|IsOverlappingActor (Variables|Default|GetAttackHitBox) (Game|GetPlayerCharacter 0) :!class /Script/Engine.PrimitiveComponent)))

(fn DealDamageKnockback
  (bind _returnvalue (Game|GetPlayerCharacter 0))
  (bind _self self)
  (bind _returnvalue_2 (Transformation|GetActorForwardVector _self))
  (Character|LaunchCharacter _returnvalue (* (Math|Vector|MakeVector (.x _returnvalue_2) (.y _returnvalue_2) (+ (.z _returnvalue_2) 1.0)) (Variables|AttackStats|GetKnockback%20Strength)) false false)
  (bind _asbp_third_person_character (Utilities|Casting|CastToBP_ThirdPersonCharacter _returnvalue))
  (Default|PlayerTakeDamage _asbp_third_person_character 2e+01))

(fn HitStop
  (params (Time :type Float%20%28single-precision%29))
  (Camera|PlayWorldCameraShake "/Game/Blueprints/Player/Effects/BP_CamShakeSmall.BP_CamShakeSmall_C" (Transformation|GetWorldLocation (Variables|/Script/Engine.Character|GetMesh (CallFunction|GetMyPlayerCharacter))) 0.0 1e+03)
  (Variables|Default|SetCustomTimeDilation 0.0)
  (Utilities|Time|SetTimerbyFunctionName 0 "EndHitStop" Time false 0.1 0.08))

(fn EndHitStop
  (Variables|Default|SetCustomTimeDilation 1.0))

(fn IsDead
  (return false))