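; Shadow mage enemy that fights the player with delayed projectiles and smoke-puff teleports.
; PawnSensing sightings drive it by distance: mid range triggers a cooldown-gated attack, while too far teleports it a random fraction closer and too near teleports it away, ignoring terrain.
; When health drops below zero it fires a death dispatch, decrements Seth's mage count and dissolves on a timer before destruction.
; Selection events toggle its widget.
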(event OnSeePawn(PawnSensing)
  (params (Pawn :type Pawn%20Object%20Reference))
  ;[1 1 1] When player is visible, calculate distance and start actions
  (if (== Pawn (Game|GetPlayerCharacter 0))
    (Variables|Default|SetisSeeingPlayer? true)
    (CallFunction|FixRotation)
    (if (>= (Variables|Default|GetDistanceToPlayer) 1.5e+03)
      (Variables|Default|SetPlayerTooClose false)
      (CallFunction|FreakMode)
      (elif (<= (Variables|Default|GetDistanceToPlayer) 5e+02)
        (Variables|Default|SetPlayerTooClose true)
        (CallFunction|FreakMode)
        (else
          (Variables|Default|SetPlayerTooClose false)
          (CallFunction|Attack))))))

(event Custom|Distance%20to%20player
  ;[1 1 1] Updates the location, playerlocation, and distancetoplayer variables
  (bind _output_get (Variables|Default|SetLocation (Transformation|GetWorldLocation (Variables|Collision|GetCapsuleComponent self))))
  (bind _output_get_2 (Variables|Default|SetPlayerLocation (Transformation|GetWorldLocation (Variables|/Script/Engine.Character|GetCapsuleComponent (Game|GetPlayerCharacter 0)))))
  (Variables|Default|SetDistanceToPlayer (Math|Vector|Distance(Vector) _output_get _output_get_2)))

(event Custom|Fix%20Rotation
  ;[1 1 1] Makes enemy face player
  (CallFunction|DistancetoPlayer)
  (Transformation|SetActorRotation (Math|Rotator|FindLookatRotation (Variables|Default|GetLocation) (Variables|Default|GetPlayerLocation))))

(event Custom|Fade
  (bind _output_get (Variables|Default|SetValue (+ (Variables|Default|GetValue) 0.01)))
  (Rendering|Material|SetScalarParameterValueonMaterials (Variables|Character|GetMesh) "Dissolve" (Math|Interpolation|Ease "EaseIn" _output_get (Math|Float|MakeLiteralFloat -0.4) 0.0 2.0)))

(event Custom|Make%20Smoke
  ;[1 1 1] Teleport VFX
  (Niagara|SpawnSystemAttached "/Game/VFX/FireVFX/NS_SethSmokeBurst.NS_SethSmokeBurst" (Variables|Character|GetMesh) "None" "0, 0, 0" "0, 0, 0" "KeepRelativeOffset" true))

(event Custom|Attack
  ;[1 1 1] Attack logic; looks at player and spawns projectile
  (if (Variables|Default|GetCan%20Attack)
    (Variables|Default|SetshouldIdle false)
    (CallFunction|FixRotation)
    (Variables|Default|SetCan%20Attack false)
    (CallFunction|DistancetoPlayer)
    (Utilities|FlowControl|Delay 2.0)
    (Game|SpawnActorfromClass "/Game/Blueprints/Enemies/Blueprints/BP_MageProjectile.BP_MageProjectile_C" (Math|Transform|MakeTransform (+ (Variables|Default|GetLocation) (Transformation|GetActorForwardVector)) "0, 0, 0" "1.000000,1.000000,1.000000") "Undefined" "MultiplyWithRoot" self 0)
    (Utilities|FlowControl|Delay 1.5)
    (Variables|Default|SetshouldIdle true)
    (Utilities|FlowControl|Delay 4.0)
    (Variables|Default|SetCan%20Attack true)))

(event Custom|Freak%20Mode
  (bind _location (Variables|Default|GetLocation))
  (bind _playerlocation (Variables|Default|GetPlayerLocation))
  (bind _location_2 (Variables|Default|GetLocation))
  (bind _verticaloffset (Variables|Default|GetVerticalOffset))
  (bind _returnvalue (+ _location_2 _verticaloffset))
  (bind _returnvalue_2 (- _playerlocation _location))
  ;[1 1 1] Teleport to a random location between themself and the player if too far, or backwards if player is too close (ignores terrain atm)
  (Variables|Default|SetOffset (Math|Random|RandomFloatinRange 0.2 0.5))
  (CallFunction|MakeSmoke)
  (if (Variables|Default|GetPlayerTooClose)
    (Transformation|SetActorLocation (+ (* (* (+ (Variables|Default|GetOffset) 1.0) -1.0) _returnvalue_2) _returnvalue) false true)
    (else
      (Transformation|SetActorLocation (+ _returnvalue (* (Variables|Default|GetOffset) _returnvalue_2)) false true)))
  (CallFunction|MakeSmoke)
  (CallFunction|FixRotation))

(event EventBeginPlay
  (CallFunction|MakeSmoke)
  (CallFunction|FixRotation))

(event EventOnSelected
  (Rendering|SetVisibility (Variables|Default|GetWidget) true false))

(event EventOnDeselected
  (Rendering|SetVisibility (Variables|Default|GetWidget) false false))

(event Game|Damage|EventAnyDamage
  (params (Damage :type Float%20%28single-precision%29) (DamageType :type Damage%20Type%20Object%20Reference) (InstigatedBy :type Controller%20Object%20Reference) (DamageCauser :type Actor%20Object%20Reference))
  (bind _output_get (Variables|Default|SetHealth (- (Variables|Default|GetHealth) Damage)))
  (if (not (>= _output_get 0.0))
    (Variables|Default|SetIsDead? true)
    (Default|CallShadowMageDeathDispatch)
    (Utilities|FlowControl|DoOnce false
      (:Completed
        (CallFunction|MakeSmoke)
        (Default|SubtractMage (Variables|Default|GetSeth))
        (Utilities|Time|SetTimerbyEvent (delegate Custom|Fade) 0.01 true)
        (Utilities|FlowControl|Delay 2.0)
        (Actor|DestroyActor)))))

(fn ConstructionScript)

(fn IsDead
  (return (Variables|Default|GetIsDead?)))