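; BP_ShadowMelee is a shadow melee enemy that can be spawned as a child actor of the Seth boss fight.
; Seeing the player via PawnSensing makes it turn and chase with AIMoveTo.
; A placeholder Attack, whose only call is disconnected, would trigger FreakMode, a smoke-wrapped teleport overshooting the player along the line between them, ignoring terrain.
; Lethal damage spawns smoke, decrements the boss's MeleeCount when parented, and destroys it.
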(event OnSeePawn(PawnSensing)
  (params (Pawn :type Pawn%20Object%20Reference))
  ;[1 1 1] When player is visible, calculate distance and start actions
  (if (== Pawn (Game|GetPlayerCharacter 0))
    (Variables|Default|SetisSeeingPlayer? true)
    (CallFunction|Move)
    (CallFunction|FixRotation)))

(event Custom|Distance%20to%20player
  ;[1 1 1] Updates the location, playerlocation, and distancetoplayer variables
  (bind _output_get (Variables|Default|SetLocation (Transformation|GetWorldLocation (Variables|Collision|GetCapsuleComponent self))))
  (bind _output_get_2 (Variables|Default|SetPlayerLocation (Transformation|GetWorldLocation (Variables|/Script/Engine.Character|GetCapsuleComponent (Game|GetPlayerCharacter 0)))))
  (Variables|Default|SetDistanceToPlayer (Math|Vector|Distance(Vector) _output_get _output_get_2)))

(event Custom|Fix%20Rotation
  ;[1 1 1] Makes enemy face player
  (CallFunction|DistancetoPlayer)
  (Transformation|SetActorRotation (Math|Rotator|FindLookatRotation (Variables|Default|GetLocation) (Variables|Default|GetPlayerLocation))))

(event Custom|Freak%20Mode
  ;[1 1 1] Teleport to a random location between themself and the player if too far, or backwards if player is too close (ignores terrain atm)
  (CallFunction|DistancetoPlayer)
  (bind _output_get (Variables|Default|SetOffset (Math|Random|RandomFloatinRange 3.0 4.0)))
  (CallFunction|MakeSmoke)
  (Transformation|SetActorLocation (+ (* _output_get (- (Variables|Default|GetPlayerLocation) (Variables|Default|GetLocation))) (+ (Variables|Default|GetLocation) (Variables|Default|GetVerticalOffset))) false true)
  (CallFunction|MakeSmoke)
  (CallFunction|FixRotation))

(event Custom|Make%20Smoke
  ;[1 1 1] Teleport VFX
  (Niagara|SpawnSystemAttached "/Game/VFX/FireVFX/NS_SethSmokeBurst.NS_SethSmokeBurst" (Variables|Character|GetMesh) "None" "0, 0, 0" "0, 0, 0" "KeepRelativeOffset" true))

(event Custom|Attack
  ;[1 1 1] Attack logic; attacks and then calls teleport behind player
  (if (Variables|Default|GetCan%20Attack)
    (Variables|Default|SetCan%20Attack false)
    ;[1 1 1] Would just make a hitbox or something but would rather do how antonio's skeleton works
    (Development|PrintString "do an attack here")
    (CallFunction|FreakMode)
    (Utilities|FlowControl|Delay 1.0)
    (Variables|Default|SetCan%20Attack true)))

(event Custom|Move
  ;[1 1 1] Movement that calls attack when close enough
  (AI|AIMoveTo self "0, 0, 0" (Game|GetPlayerCharacter 0) 1.5e+02 false))

(event EventBeginPlay
  (CallFunction|MakeSmoke)
  (CallFunction|FixRotation))

(event Game|Damage|EventAnyDamage
  (params (Damage :type Float%20%28single-precision%29) (DamageType :type Damage%20Type%20Object%20Reference) (InstigatedBy :type Controller%20Object%20Reference) (DamageCauser :type Actor%20Object%20Reference))
  (bind _output_get (Variables|Default|SetHealth (- (Variables|Default|GetHealth) Damage)))
  (if (not (>= _output_get 0.0))
    (Utilities|FlowControl|DoOnce false
      (:Completed
        (CallFunction|MakeSmoke)
        (if (Class|Actor|IsChildActor)
          (bind _asbp_seth_boss_fight (Utilities|Casting|CastToBP_SethBossFight (Actor|GetParentActor)))
          (bind _result (Math|Integer|DecrementInt (Variables|/Game/Blueprints/Enemies/Blueprints/BP_SethBossFight.BP_SethBossFight_C|GetMeleeCount _asbp_seth_boss_fight))
            (:%20%20
              (Variables|/Game/Blueprints/Enemies/Blueprints/BP_SethBossFight.BP_SethBossFight_C|SetMeleeCount _asbp_seth_boss_fight _result))))
        (Actor|DestroyActor)))))

(fn ConstructionScript)