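; Jackal melee enemy built on a parent enemy class, exposing movement speed, attack/defend ranges and death state.
; On BeginPlay it attaches a spawned sword to a mesh socket and passes it, plus all "enemy"-tagged actors, to its trace component.
; Reported damage triggers a health check; death runs once, stopping AI logic and destroying the capsule.
; Lock-on release and timed removal follow only if the player's target is this enemy or invalid.
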(event Custom|TakeDamage
  (bind _playerref (Variables|Default|GetPlayerRef))
  (bind _targetactor (Variables|/Game/ThirdPerson/Blueprints/BP_ThirdPersonCharacter.BP_ThirdPersonCharacter_C|GetTargetActor _playerref))
  (if (<= (Variables|Default|GetHealth) 0.0)
    (Variables|Default|SetIsDead? true)
    (Collision|SetCollisionEnabled (Variables|Character|GetMesh) "QueryAndPhysics")
    (Collision|SetCollisionEnabled (Variables|Default|GetCapsuleComponent) "NoCollision")
    (Utilities|FlowControl|DoOnce false
      (:Completed
        (AI|Logic|StopLogic (Variables|/Script/AIModule.AIController|GetBrainComponent (AI|GetAIController self)) "die")
        (Components|DestroyComponent (Variables|Default|GetCapsuleComponent))
        (Variables|Default|SetEnemyDead? true)
        (Utilities|IsValid _targetactor
          (:Is%20Valid
            (if (== _targetactor self)
              (Default|DisengageLock-on (Variables|Default|GetPlayerRef) :!label _label)
              (Actor|SetLifeSpan 4.0)
              (Actor|SetLifeSpan (Variables|Default|Getswordreference4) 4.0)
              (Collision|SetCollisionResponsetoChannel (Variables|Character|GetMesh) "ECC_Pawn" "ECR_Ignore")))
          (:Is%20Not%20Valid
            (goto _label)))))))

(event Custom|Clear%20Hit%20Actors
  (Utilities|Array|Clear (Variables|/Game/ThirdPerson/Equipment/TraceComponent.TraceComponent_C|GetActorsToIgnore (Variables|Default|GetTraceComponent_Jackal))))

(event EventBeginPlay
  (|CallParentFunction)
  (Collision|SetCollisionResponsetoChannel (Variables|Default|GetCapsuleComponent) "ECC_Pawn" "ECR_Block")
  (bind _asbp_third_person_character (Utilities|Casting|CastToBP_ThirdPersonCharacter (Game|GetPlayerCharacter 0)))
  (Variables|Default|SetPlayerRef _asbp_third_person_character)
  (bind _returnvalue (Game|SpawnActorfromClass (Variables|Default|Getswordclassref) (Transformation|GetSocketTransform (Variables|Character|GetMesh) "Sword" "RTS_World") "Undefined" "MultiplyWithRoot" 0 0))
  (bind _output_get (Variables|Default|Setswordreference4 _returnvalue))
  (Transformation|AttachComponentToComponent _output_get (Variables|Character|GetMesh) "Sword" "SnapToTarget" "SnapToTarget" "SnapToTarget" true)
  (Variables|/Game/ThirdPerson/Equipment/TraceComponent.TraceComponent_C|Setswordref (Variables|Default|GetTraceComponent_Jackal) (Variables|Default|Getswordreference4))
  (bind _outactors (Actor|GetAllActorswithTag "enemy"))
  (Variables|/Game/ThirdPerson/Equipment/TraceComponent.TraceComponent_C|Setenemy (Variables|Default|GetTraceComponent_Jackal) _outactors))

(event Collision|EventActorBeginOverlap
  (params (OtherActor :type Actor%20Object%20Reference)))

(event EventTick
  (params (DeltaSeconds :type Float%20%28single-precision%29)))

(fn ConstructionScript
  (|CallParentFunction))

(fn SetMovementSpeed
  (params (Speed :type E_MoveSpeed%20Enum :default "NewEnumerator0"))
  (bind _output_get (Variables|/Script/Engine.CharacterMovementComponent|SetMaxWalkSpeed (Variables|Character|GetCharacterMovement) (Utilities|Select :Index Speed :NewEnumerator0 (Variables|Default|GetIdle) :NewEnumerator1 (Variables|Default|GetWalking) :NewEnumerator2 (Variables|Default|GetJogging) :NewEnumerator3 (Variables|Default|GetSprinting))))
  (return _output_get))

(fn GetIdealRange
  (return (Variables|Default|GetAttack%20Rad_0) (Variables|Default|GetDefend%20Rad_0)))

(fn IsDead
  (return (Variables|Default|GetEnemyDead?)))

(fn DeathFunc
  (|CallParentFunction))

(fn ReportDamage
  (params (Damage%20Amount%20Taken :type Float%20%28single-precision%29) (Instigator :type Actor%20Object%20Reference))
  (bind _damage_taken (|CallParentFunction Damage%20Amount%20Taken Instigator))
  (bind _output_get (Variables|Default|SetDamage%20Taken _damage_taken))
  (CallFunction|TakeDamage)
  (return _output_get))