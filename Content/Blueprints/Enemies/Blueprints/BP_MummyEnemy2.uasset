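; Mummy enemy Blueprint that wields a sword and handles its own death.
; BeginPlay spawns the sword on a mesh socket and passes it, plus actors tagged "enemy", to a trace component whose ignore list ClearHitActors empties.
; TakeDamage at zero health stops AI logic.
; Only if it is the player's lock-on target does it then release lock-on, expire with its sword, ragdoll and dissolve via a looping timer.
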(event Custom|TakeDamage
  (bind _playerref (Variables|Default|GetPlayerRef))
  (bind _targetactor (Variables|/Game/ThirdPerson/Blueprints/BP_ThirdPersonCharacter.BP_ThirdPersonCharacter_C|GetTargetActor _playerref))
  (if (<= (Variables|Default|GetHealth) 0.0)
    (Variables|Default|SetIsDead? true)
    (Collision|SetCollisionEnabled (Variables|Character|GetMesh) "QueryAndPhysics")
    (Collision|SetCollisionEnabled (Variables|Default|GetCapsuleComponent) "NoCollision")
    (Utilities|FlowControl|DoOnce false
      (:Completed
        (AI|Logic|StopLogic (Variables|/Script/AIModule.AIController|GetBrainComponent (AI|GetAIController self)) "die")
        (Variables|Default|SetEnemyDead? true)
        (Utilities|IsValid _targetactor
          (:Is%20Valid
            (if (== _targetactor self)
              (Default|DisengageLock-on (Variables|Default|GetPlayerRef))
              (Actor|SetLifeSpan 4.0)
              (Actor|SetLifeSpan (Variables|Default|Getswordreference5) 4.0)
              (Collision|SetCollisionResponsetoChannel (Variables|Character|GetMesh) "ECC_Pawn" "ECR_Ignore")
              (Utilities|FlowControl|RetriggerableDelay 2.2)
              (Physics|SetSimulatePhysics (Variables|Character|GetMesh) true)
              (Utilities|Time|SetTimerbyEvent (delegate Custom|CustomEvent) 0.01 true))))))))

(event Custom|Clear%20Hit%20Actors
  (Utilities|Array|Clear (Variables|/Game/ThirdPerson/Equipment/TraceComponent.TraceComponent_C|GetActorsToIgnore (Variables|Default|GetTraceComponent_Mummy))))

(event Custom|CustomEvent
  (bind _output_get (Variables|Default|SetValue (+ (Variables|Default|GetValue) 0.01)))
  (Rendering|Material|SetScalarParameterValueonMaterials (Variables|Character|GetMesh) "Dissolve" (Math|Interpolation|Ease "EaseIn" _output_get (Math|Float|MakeLiteralFloat -0.4) 0.0 2.0)))

(event EventBeginPlay
  (|CallParentFunction)
  (Collision|SetCollisionResponsetoChannel (Variables|Default|GetCapsuleComponent) "ECC_Pawn" "ECR_Block")
  (bind _asbp_third_person_character (Utilities|Casting|CastToBP_ThirdPersonCharacter (Game|GetPlayerCharacter 0)))
  (Variables|Default|SetPlayerRef _asbp_third_person_character)
  (bind _returnvalue (Game|SpawnActorfromClass (Variables|Default|Getswordclassref) (Transformation|GetSocketTransform (Variables|Character|GetMesh) "Sword" "RTS_World") "Undefined" "MultiplyWithRoot" 0 0))
  (bind _output_get (Variables|Default|Setswordreference5 _returnvalue))
  (Transformation|AttachComponentToComponent _output_get (Variables|Character|GetMesh) "sword" "SnapToTarget" "SnapToTarget" "SnapToTarget" true)
  (Variables|/Game/ThirdPerson/Equipment/TraceComponent.TraceComponent_C|Setswordref (Variables|Default|GetTraceComponent_Mummy) (Variables|Default|Getswordreference5))
  (bind _outactors (Actor|GetAllActorswithTag "enemy"))
  (Variables|/Game/ThirdPerson/Equipment/TraceComponent.TraceComponent_C|Setenemy (Variables|Default|GetTraceComponent_Mummy) _outactors))

(event Collision|EventActorBeginOverlap
  (params (OtherActor :type Actor%20Object%20Reference)))

(event EventTick
  (params (DeltaSeconds :type Float%20%28single-precision%29)))

(fn ConstructionScript
  (|CallParentFunction))