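; BP_PatrolRoute is a spline-based patrol path for the RockThrower enemy AI.
; It tracks a current spline point index and exposes that point as a world position.
; IncrementPatrolRoute steps the index by a direction value that flips at the first and last points, so the route ping-pongs back and forth rather than looping.
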(event Custom|IncrementPatrolRoute
  (bind _output_get (Variables|Default|SetPatrolIndex (+ (Variables|Default|GetPatrolIndex) (Variables|Default|GetDirections))))
  (if (== _output_get (- (Spline|GetNumberOfSplinePoints (Variables|Default|GetSpline)) 1))
    (Variables|Default|SetDirections -1)
    (elif (== (Variables|Default|GetPatrolIndex) 0)
      (Variables|Default|SetDirections 1))))

(fn ConstructionScript)

(fn GetSplinePointasWorldPos
  (return (Spline|GetLocationatSplinePoint (Variables|Default|GetSpline) (Variables|Default|GetPatrolIndex) "World")))