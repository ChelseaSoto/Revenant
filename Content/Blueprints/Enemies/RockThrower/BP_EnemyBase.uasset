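; Base enemy character with health, lock-on indicator, patrol route access and selectable walk speeds.
; Damage triggers player hit stop and camera shake when the causer's name contains "ThirdPerson", then reduces health.
; Surviving hits freeze the enemy through time dilation; health exactly at zero stops AI logic, ragdolls the mesh and expires the actor.
; Attack only waits before signalling its end, as the montage playback is disconnected.
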(event Custom|Attack
  (Utilities|FlowControl|Delay 2.0)
  (Default|CallOnAttackEnd))

(event EventOnDeselected
  (Rendering|SetVisibility (Variables|Default|GetLockOn) false false))

(event EventOnSelected
  (Rendering|SetVisibility (Variables|Default|GetLockOn) true false))

(event Game|Damage|EventAnyDamage
  (params (Damage :type Float%20%28single-precision%29) (DamageType :type Damage%20Type%20Object%20Reference) (InstigatedBy :type Controller%20Object%20Reference) (DamageCauser :type Actor%20Object%20Reference))
  (bind _my_player_character (CallFunction|GetMyPlayerCharacter))
  (if (Utilities|String|Contains (Utilities|GetDisplayName DamageCauser) "ThirdPerson")
    (Default|StartHitStop _my_player_character 0.1)
    (Default|CameraShake _my_player_character false))
  (bind _output_get (Variables|Default|SetHealth (- (Variables|Default|GetHealth) Damage)))
  (if (== _output_get 0.0)
    (Variables|Default|SetIsDead? true)
    (AI|Logic|StopLogic (Variables|/Script/AIModule.AIController|GetBrainComponent (AI|GetAIController self)) "death")
    (Physics|SetSimulatePhysics (Variables|Character|GetMesh) true)
    (Collision|SetCollisionEnabled (Variables|Collision|GetCapsuleComponent) "NoCollision")
    (Actor|SetLifeSpan 4.0)
    (else
      (CallFunction|StartHitStop 0.1))))

(fn ConstructionScript)

(fn StartHitStop
  (params (Time%20stop :type Float%20%28double-precision%29))
  (Camera|PlayWorldCameraShake "/Game/Blueprints/Player/Effects/BP_CamShakeSmall.BP_CamShakeSmall_C" (Transformation|GetWorldLocation (Variables|/Script/Engine.Character|GetMesh (CallFunction|GetMyPlayerCharacter))) 0.0 1e+03)
  (Variables|Default|SetCustomTimeDilation 0.0)
  (Utilities|Time|SetTimerbyFunctionName 0 "End Hit Stop" Time%20stop false 0.1 0.08))

(fn EndHitStop
  (Variables|Default|SetCustomTimeDilation 1.0))

(fn GetPatrolRoute
  (return (Variables|Default|GetPatrolRoute)))

(fn IsDead
  (return (Variables|Default|GetIsDead?)))

(fn SetMovementSpeed
  (params (Speed :type E_MoveSpeed%20Enum :default "NewEnumerator0"))
  (bind _output_get (Variables|/Script/Engine.CharacterMovementComponent|SetMaxWalkSpeed (Variables|Character|GetCharacterMovement) (Utilities|Select :Index Speed :NewEnumerator0 (Variables|Default|GetIdle) :NewEnumerator1 (Variables|Default|GetWalking) :NewEnumerator2 (Variables|Default|GetJogging) :NewEnumerator3 (Variables|Default|GetSprinting))))
  (return _output_get))