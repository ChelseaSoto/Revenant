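; BP_EnemySpawner is an actor that spawns an enemy of a configurable class, either automatically on BeginPlay when enabled or through its Spawn event.
; Each spawn picks a random reachable navmesh point within a radius of the spawner and applies a configurable yaw for facing.
; It stores the new actor and calls Spawned to signal that the spawn has happened.
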(event Custom|Spawn
  (bind _returnvalue (Game|SpawnActorfromClass (Variables|Default|GetEnemyToSpawn) (Math|Transform|MakeTransform (.RandomLocation (AI|Navigation|GetRandomReachablePointinRadius (Transformation|GetActorLocation) (Variables|Default|GetSpawnRadius) 0 0)) (Math|Rotator|MakeRotator 0.0 0.0 (Variables|Default|GetEnemySpawnDirection)) "1.000000,1.000000,1.000000") "Undefined" "MultiplyWithRoot" 0 0))
  (Variables|Default|SetSpawnedActor _returnvalue)
  (Default|CallSpawned))

(event EventBeginPlay
  (if (Variables|Default|GetSpawn%20on%20Play?)
    (CallFunction|Spawn)))

(fn ConstructionScript)