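; BP_RayOfFeathers is a damage-zone attack actor, attributed to the Bird Vessel enemy, that hurts the player while they overlap it.
; Its box ignores collision on spawn, then switches to overlap after a short delay.
; Player overlap applies damage immediately and starts a looping timer that repeats it until overlap ends.
; The damage causer is looked up by class, not passed in by a spawner.
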(event Custom|StartDamageOverTime
  (bind _returnvalue (Utilities|Time|SetTimerbyEvent (delegate Custom|DamageOverTime) 1.0 true))
  (Variables|Default|SetDamageOverTime_Timer _returnvalue))

(event Custom|DamageOverTime
  (bind _returnvalue (Actor|GetActorOfClass "/Game/Blueprints/Enemies/Blueprints/BP_BirdVesselEnemy_New.BP_BirdVesselEnemy_New_C"))
  (Game|Damage|ApplyDamage (Game|GetPlayerCharacter 0) 5.0 0 _returnvalue))

(event Custom|EndDamageOverTime
  (Utilities|Time|ClearandInvalidateTimerbyHandle (Variables|Default|GetDamageOverTime_Timer)))

(event EventBeginPlay
  (Collision|SetCollisionResponsetoAllChannels (Variables|Default|GetBox) "ECR_Ignore")
  (Utilities|FlowControl|Delay 2.5)
  (Collision|SetCollisionResponsetoAllChannels (Variables|Default|GetBox) "ECR_Overlap"))

(event EventTick
  (params (DeltaSeconds :type Float%20%28single-precision%29)))

(event Collision|EventActorBeginOverlap
  (params (OtherActor :type Actor%20Object%20Reference))
  (if (== OtherActor (Game|GetPlayerCharacter 0))
    (CallFunction|DamageOverTime)
    (CallFunction|StartDamageOverTime)))

(event Collision|EventActorEndOverlap
  (params (OtherActor :type Actor%20Object%20Reference))
  (if (== OtherActor (Game|GetPlayerCharacter 0))
    (CallFunction|EndDamageOverTime)))

(fn ConstructionScript)