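; Companion actor (Bastet) that walks along a spline while the player overlaps it, then fades and destroys itself at the path's end.
; Delayed overlap events toggle movement and the IsWalking flag, and BeginPlay hands the anim blueprint a self-reference.
; Tick advances spline distance by a per-frame speed, not delta-scaled, with offset location and yaw.
; Reaching EndPoint runs a material-parameter fade timeline, then calls CallReachedEndOfPath before destruction.
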(event OnComponentBeginOverlap(EndPoint)
  (params (OverlappedComponent :type Primitive%20Component%20Object%20Reference) (OtherActor :type Actor%20Object%20Reference) (OtherComp :type Primitive%20Component%20Object%20Reference) (OtherBodyIndex :type Integer) (bFromSweep :type Boolean) (SweepResult :type Hit%20Result%20Structure%20%28by%20ref%29))
  ;[1 1 1] Destroy entire actor once the colliders overlap at the end of the spline path
  (if (== OtherComp (Variables|Default|GetSphere))
    (CallFunction|FadeTimer)
    (Utilities|FlowControl|Delay 2.0)
    (Development|PrintString "Companion has reached end of spline path")
    (Default|CallReachedEndOfPath)
    (Actor|DestroyActor)))

(event Custom|FadeTimer
  (Utilities|FlowControl|FlipFlop
    (:A
      (bind _newtrack_0 (Timeline|Fade PlayFromStart)
        (:Update
          (Rendering|Material|SetScalarParameterValueonMaterials (Variables|Default|GetCharacter) "Fade" _newtrack_0))))
    (:B
      (Timeline|Fade ReverseFromEnd))))

(event EventBeginPlay
  ;[1 1 1] Animation is playing by default, so this stops it
  (Variables|Default|SetisWalking false)
  (bind _asabp_bastet (Utilities|Casting|CastToABP_Bastet (Components|SkeletalMesh|GetAnimInstance (Variables|Default|GetCharacter)))
    (:then
      (Variables|/Game/ArtPrototype/Rigs/Bastet_New/ABP_Bastet.ABP_Bastet_C|SetAs%20BP%20New%20Companion _asabp_bastet self)
      (Rendering|Material|SetScalarParameterValueonMaterials (Variables|Default|GetCharacter) "Fade" 0.0))
    (:CastFailed
      (Development|PrintString "ABP not found (Bastet walking)"))))

(event EventTick
  (params (DeltaSeconds :type Float%20%28single-precision%29))
  ;[1 1 1] While player is overlapping companion trigger, move the companion along their spline. Their movement is based on spline speed / distance along spline
  (if (Variables|Default|GetisOverlapping)
    (Variables|Default|SetdistanceAlongSpline (+ (* 1.0 (Variables|Default|GetsplineSpeed)) (Variables|Default|GetdistanceAlongSpline)))
    (Transformation|SetRelativeTransform (Variables|Default|GetCharacter) (Math|Transform|MakeTransform (Math|Vector|MakeVector (.x (.location (Spline|GetTransformatDistanceAlongSpline (Variables|Default|GetSpline) (Variables|Default|GetdistanceAlongSpline) "Local" false))) (.y (.location (Spline|GetTransformatDistanceAlongSpline (Variables|Default|GetSpline) (Variables|Default|GetdistanceAlongSpline) "Local" false))) (+ (.z (.location (Spline|GetTransformatDistanceAlongSpline (Variables|Default|GetSpline) (Variables|Default|GetdistanceAlongSpline) "Local" false))) -89.0)) (Math|Rotator|MakeRotator (.roll (.rotation (Spline|GetTransformatDistanceAlongSpline (Variables|Default|GetSpline) (Variables|Default|GetdistanceAlongSpline) "Local" false))) (.pitch (.rotation (Spline|GetTransformatDistanceAlongSpline (Variables|Default|GetSpline) (Variables|Default|GetdistanceAlongSpline) "Local" false))) (- (.yaw (.rotation (Spline|GetTransformatDistanceAlongSpline (Variables|Default|GetSpline) (Variables|Default|GetdistanceAlongSpline) "Local" false))) 89.0)) (Variables|/Script/Engine.SceneComponent|GetRelativeScale3D (Variables|Default|GetCharacter))) false false)))

(event Collision|EventActorBeginOverlap
  (params (OtherActor :type Actor%20Object%20Reference))
  ;[1 1 1] When player overlaps with companion trigger, start companion animation
  (if (== OtherActor (Game|Player|GetPlayerPawn 0))
    (Utilities|FlowControl|Delay 0.2)
    (Variables|Default|SetisOverlapping true)
    (Variables|Default|SetisWalking true)))

(event Collision|EventActorEndOverlap
  (params (OtherActor :type Actor%20Object%20Reference))
  ;[1 1 1] When player no longer overlaps with companion trigger, stop companion animation
  (if (== OtherActor (Game|Player|GetPlayerPawn 0))
    (Utilities|FlowControl|Delay 0.6)
    (Variables|Default|SetisOverlapping false)
    (Variables|Default|SetisWalking false)))

(fn ConstructionScript)