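; BP_MainCam is a camera director actor that plays short scripted camera shots for the West, South and East doors.
; Each door event cuts the first player's view to that side's first camera reference, blends to the second, then cuts back to the controlled pawn.
; The sequence is timed with Delay nodes and SetViewTargetWithBlend, and the actor enables input on BeginPlay.
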(event Custom|DoorCamEastEvent
  (Game|Player|SetViewTargetwithBlend (Game|GetPlayerController 0) (Variables|Default|GetCamRefEast1) 0.0 "VTBlend_Linear" 0.0 false)
  (Utilities|FlowControl|Delay 0.2)
  (Game|Player|SetViewTargetwithBlend (Game|GetPlayerController 0) (Variables|Default|GetCamRefEast2) 1.0 "VTBlend_Linear" 0.0 false)
  (Utilities|FlowControl|Delay 3.0)
  (Game|Player|SetViewTargetwithBlend (Game|GetPlayerController 0) (Pawn|GetControlledPawn (Game|GetPlayerController 0)) 0.0 "VTBlend_Linear" 0.0 true))

(event Custom|DoorCamWestEvent
  (Game|Player|SetViewTargetwithBlend (Game|GetPlayerController 0) (Variables|Default|GetCamRefWest1) 0.0 "VTBlend_Linear" 0.0 false)
  (Utilities|FlowControl|Delay 0.2)
  (Game|Player|SetViewTargetwithBlend (Game|GetPlayerController 0) (Variables|Default|GetCamRefWest2) 1.0 "VTBlend_Linear" 0.0 false)
  (Utilities|FlowControl|Delay 3.0)
  (Game|Player|SetViewTargetwithBlend (Game|GetPlayerController 0) (Pawn|GetControlledPawn (Game|GetPlayerController 0)) 0.0 "VTBlend_Linear" 0.0 true))

(event Custom|DoorCamSouthEvent
  (Game|Player|SetViewTargetwithBlend (Game|GetPlayerController 0) (Variables|Default|GetCamRefSouth1) 0.0 "VTBlend_Linear" 0.0 false)
  (Utilities|FlowControl|Delay 0.2)
  (Game|Player|SetViewTargetwithBlend (Game|GetPlayerController 0) (Variables|Default|GetCamRefSouth2) 1.0 "VTBlend_Linear" 0.0 false)
  (Utilities|FlowControl|Delay 3.0)
  (Game|Player|SetViewTargetwithBlend (Game|GetPlayerController 0) (Pawn|GetControlledPawn (Game|GetPlayerController 0)) 0.0 "VTBlend_Linear" 0.0 true))

(event EventBeginPlay
  (Input|EnableInput (Game|GetPlayerController 0)))

(event Collision|EventActorBeginOverlap
  (params (OtherActor :type Actor%20Object%20Reference)))

(event EventTick
  (params (DeltaSeconds :type Float%20%28single-precision%29)))

(fn ConstructionScript)