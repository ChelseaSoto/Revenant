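; BP_PyramidCam is a trigger that plays a short one-time camera cutaway, presumably of a pyramid, when the player character enters its Box.
; The first overlap passes a DoOnce and starts SwitchToCinematicCamera, which disables player input and blends the view to Cam1.
; After a timed hold, it blends back to the controlled pawn with the outgoing view locked, then re-enables input when that blend finishes.
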(event OnComponentBeginOverlap(Box)
  (params (OverlappedComponent :type Primitive%20Component%20Object%20Reference) (OtherActor :type Actor%20Object%20Reference) (OtherComp :type Primitive%20Component%20Object%20Reference) (OtherBodyIndex :type Integer) (bFromSweep :type Boolean) (SweepResult :type Hit%20Result%20Structure%20%28by%20ref%29))
  (if (== OtherActor (Game|GetPlayerCharacter 0))
    (Utilities|FlowControl|DoOnce false
      (:Completed
        (CallFunction|SwitchtoCinematicCamera)))))

(event Custom|Switch%20to%20Cinematic%20Camera
  (Input|DisableInput (Game|GetPlayerCharacter 0) (Game|GetPlayerController 0))
  (Game|Player|SetViewTargetwithBlend (Game|GetPlayerController 0) (Variables|Default|GetCam1) 2.8 "VTBlend_Linear" 0.2 false)
  (Utilities|FlowControl|Delay 3.6)
  (Game|Player|SetViewTargetwithBlend (Game|GetPlayerController 0) (Pawn|GetControlledPawn (Game|GetPlayerController 0)) 2.8 "VTBlend_Linear" 0.2 true)
  (Utilities|FlowControl|Delay 2.8)
  (Input|EnableInput (Game|GetPlayerCharacter 0) (Game|GetPlayerController 0)))

(event EventBeginPlay)

(event Collision|EventActorBeginOverlap
  (params (OtherActor :type Actor%20Object%20Reference)))

(event EventTick
  (params (DeltaSeconds :type Float%20%28single-precision%29)))

(fn ConstructionScript)