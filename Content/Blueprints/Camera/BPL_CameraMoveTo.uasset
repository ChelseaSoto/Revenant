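; Blueprint function library with a Cinematic function that switches the first player's view between a given camera actor and the player character.
; Play blends the view to the camera and enables cinematic mode, locking movement and turning while keeping the player visible.
; Otherwise it blends back to the character and turns cinematic mode off.
; Both paths return the blend time plus a fixed two-second margin.
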(fn Cinematic
  (params (Play :type Boolean) (Camera%20Actor%20to%20Look%20at :type Actor%20Object%20Reference) (Blend%20Time :type Float%20%28double-precision%29) (Blend%20Exp :type Float%20%28double-precision%29))
  (bind _returnvalue (Game|GetPlayerController 0))
  (bind _returnvalue_2 (Game|GetPlayerController 0))
  (if Play
    (Game|Player|SetViewTargetwithBlend _returnvalue_2 Camera%20Actor%20to%20Look%20at Blend%20Time "VTBlend_Linear" Blend%20Exp false)
    (Class|PlayerController|SetCinematicMode _returnvalue_2 true false true true true)
    (else
      (Game|Player|SetViewTargetwithBlend _returnvalue (Game|GetPlayerCharacter 0) Blend%20Time "VTBlend_Linear" Blend%20Exp false)
      (Class|PlayerController|SetCinematicMode _returnvalue false false true true true)))
  (return (+ Blend%20Time 2.0)))