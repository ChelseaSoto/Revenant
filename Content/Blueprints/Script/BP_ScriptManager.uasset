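; Script manager that drives visual-novel style dialogue, creating the player HUD and advancing through the story on interact input.
; A script DataTable, stepped by counter, supplies each event type and music; Dialogue events advance a separate dialogue table for name, line and SFX.
; The HUD dialogue widget displays each line; LineEnd shows the proceed prompt and enables input and cursor after the first line.
; Background and expression are stored but not applied here.
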(event Custom|Action
  (bind _hud (Variables|Default|GetHUD))
  (bind _chwb_dialogue1 (Variables|/Game/ThirdPerson/UI/WB_PlayerHUD.WB_PlayerHUD_C|GetchWB_Dialogue1 _hud))
  ;[1 1 1] Does the thing
  (Variables|Default|SetCanProceed? false)
  (Default|ClearText _chwb_dialogue1)
  (Default|ShowProceed _chwb_dialogue1 "Hidden")
  (CallFunction|NextLine)
  (CallFunction|GetScriptRow (Utilities|String|StringToName (Utilities|String|ToString(Integer) (Variables|Default|GetScript%20Counter))))
  (Utilities|FlowControl|Sequence
    (:then_0
      (switch Utilities|FlowControl|Switch|SwitchonE_Script (Variables|Default|GetSpecial%20Event)
        (:NewEnumerator0
          (CallFunction|PlayLine))))
    (:then_1
      ;;[1 1 1] If music is valid, then change the music.
      (if (not (== (Variables|Default|GetScript%20Counter) 1))
        (CallFunction|PlayMusic)))))

(event Custom|PlayLine
  ;[1 1 1] Play the line
  (CallFunction|NextDialogueRow)
  (CallFunction|FillDialogue)
  (Variables|Default|SetTyping true)
  (Utilities|FlowControl|Sequence
    (:then_0
      ;;[1 1 1] Play SFX if exists
      (Utilities|IsValid (Variables|Default|GetSFX)
        (:Is%20Valid
          (Audio|PlaySound2D (Variables|Default|GetSFX) 1.0 1.0 0.0 0 0))))
    (:then_1
      (Default|StartLine (Variables|/Game/ThirdPerson/UI/WB_PlayerHUD.WB_PlayerHUD_C|GetchWB_Dialogue1 (Variables|Default|GetHUD)) (Utilities|Text|ToText(String) (Variables|Default|GetLine)) (Variables|Default|GetNames)))))

(event Custom|LineEnd
  ;[1 1 1] End the line
  (Variables|Default|SetTyping false)
  (switch Utilities|FlowControl|Switch|SwitchonE_Script (Variables|Default|GetSpecial%20Event)
    (:NewEnumerator0
      (Default|ShowProceed (Variables|/Game/ThirdPerson/UI/WB_PlayerHUD.WB_PlayerHUD_C|GetchWB_Dialogue1 (Variables|Default|GetHUD)) "Visible")
      (CallFunction|EnableInputAfterFirstRun))))

(event Input|EnhancedActionEvents|EnhancedInputActionIA_Interact
  (params (ActionValue :type Boolean) (ElapsedSeconds :type Float%20%28double-precision%29) (TriggeredSeconds :type Float%20%28double-precision%29) (InputAction :type Input%20Action%20Object%20Reference :default "/Game/ThirdPerson/Input/Actions/IA_Interact.IA_Interact"))
  ;[1 1 1] When receiving input, it does the thing
  (:Completed
    (if (Variables|Default|GetCanProceed?)
      (CallFunction|Action))))

(event EventBeginPlay
  (bind _returnvalue (UserInterface|CreateWidget "/Game/ThirdPerson/UI/WB_PlayerHUD.WB_PlayerHUD_C" (Game|GetPlayerController 0) self))
  (bind _output_get (Variables|Default|SetHUD _returnvalue))
  (UserInterface|Viewport|AddtoViewport _output_get 0)
  (CallFunction|GetScriptRow (Utilities|String|StringToName (Utilities|String|ToString(Integer) (Variables|Default|GetScript%20Counter))))
  (Utilities|FlowControl|Sequence
    (:then_0
      (CallFunction|PlayMusic))
    (:then_1
      (Utilities|FlowControl|Delay 1.0)
      (Default|ShowDialogue (Variables|/Game/ThirdPerson/UI/WB_PlayerHUD.WB_PlayerHUD_C|GetchWB_Dialogue1 (Variables|Default|GetHUD))))))

(fn ConstructionScript)

(fn GetScriptRow
  (params (RowName :type Name))
  (bind _returnvalue (Utilities|GetDataTableRow (Variables|Default|GetDT_Script) RowName)
    (:then
      (Variables|Default|SetSpecial%20Event (.EpecialEvent (Utilities|Struct|BreakST_Script _returnvalue)))
      (Variables|Default|SetMusic (.Music (Utilities|Struct|BreakST_Script _returnvalue)))
      (Variables|Default|SetBackground (.Background (Utilities|Struct|BreakST_Script _returnvalue))))))

(fn PlayMusic
  (bind _backgroundmusic (Variables|Default|GetBackgroundMusic))
  (Utilities|IsValid (Variables|Default|GetMusic)
    (:Is%20Valid
      (Audio|Components|Audio|SetSound _backgroundmusic (Variables|Default|GetMusic))
      (Audio|Components|Audio|FadeIn _backgroundmusic 1.0 1.0 0.0 "Linear" :!class /Script/Engine.AudioComponent))))

(fn NextLine
  (Variables|Default|SetScript%20Counter (+ (Variables|Default|GetScript%20Counter) 1)))

(fn NextDialogueRow
  (Variables|Default|SetDialogue%20Counter (+ (Variables|Default|GetDialogue%20Counter) 1)))

(fn FillDialogue
  (bind _returnvalue (Utilities|GetDataTableRow (Variables|Default|GetDT_Dialogue) (Utilities|String|StringToName (Utilities|String|ToString(Integer) (Variables|Default|GetDialogue%20Counter))))
    (:then
      (Variables|Default|SetNames (.Names (Utilities|Struct|BreakST_Dialogue _returnvalue)))
      (Variables|Default|SetExpression (.Expression (Utilities|Struct|BreakST_Dialogue _returnvalue)))
      (Variables|Default|SetSFX (.SFX (Utilities|Struct|BreakST_Dialogue _returnvalue)))
      (Variables|Default|SetLine (.Line (Utilities|Struct|BreakST_Dialogue _returnvalue))))))

(fn EnableInputAfterFirstRun
  (bind _returnvalue (Game|GetPlayerController 0))
  (if (== (Variables|Default|GetScript%20Counter) 1)
    (Input|EnableInput _returnvalue)
    (Variables|/Script/Engine.PlayerController|SetbShowMouseCursor _returnvalue true)))