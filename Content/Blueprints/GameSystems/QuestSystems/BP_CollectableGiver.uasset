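; BP_CollectableGiver is a quest-system Blueprint that processes a list of quest data table rows at BeginPlay.
; It skips quests already active in the player character's BPCQuestLogComponent and looks up the data row for each remaining one.
; It creates a WB_QuestGiver widget with that quest's details and ID, then adds it to the viewport and immediately removes it, without waiting for player input.
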(event EventBeginPlay
  (for _array_element (Variables|Default|GetQuestData)
    (if (not (Default|QueryActiveQuest (Variables|/Game/ThirdPerson/Blueprints/BP_ThirdPersonCharacter.BP_ThirdPersonCharacter_C|GetBPC_QuestLogComponent (CallFunction|GetMyPlayerCharacter)) (.RowName (Utilities|Struct|BreakDataTableRowHandle _array_element))))
      (bind _returnvalue (Utilities|GetDataTableRow (.DataTable (Utilities|Struct|BreakDataTableRowHandle _array_element)) (.RowName (Utilities|Struct|BreakDataTableRowHandle _array_element)))
        (:then
          (bind _returnvalue_2 (UserInterface|CreateWidget "/Game/UI/QuestUI/WB_QuestGiver.WB_QuestGiver_C" 0 _returnvalue (.RowName (Utilities|Struct|BreakDataTableRowHandle _array_element))))
          (UserInterface|Viewport|AddtoViewport _returnvalue_2 0)
          (Widget|RemovefromParent _returnvalue_2))))))

(fn ConstructionScript)