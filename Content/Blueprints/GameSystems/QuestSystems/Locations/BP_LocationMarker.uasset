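; BP_LocationMarker is a quest location trigger that registers the player's arrival and announces the location.
; On the first overlap by the player character, it calls CallOnObjectIDCalled on BP_ThirdPersonCharacter with its ObjectiveId and a value of 1.
; It then shows a WB_LocationNotify widget with the location name and description and destroys itself, making the marker single-use.
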(event Collision|EventActorBeginOverlap
  (params (OtherActor :type Actor%20Object%20Reference))
  (if (== OtherActor (CallFunction|GetMyPlayerCharacter))
    (Utilities|FlowControl|DoOnce false
      (:Completed
        (bind _asbp_third_person_character (Utilities|Casting|CastToBP_ThirdPersonCharacter OtherActor))
        (Default|CallOnObjectIDCalled _asbp_third_person_character (Variables|Default|GetObjectiveId) 1)
        (bind _returnvalue (UserInterface|CreateWidget "/Game/UI/QuestUI/WB_LocationNotify.WB_LocationNotify_C" 0 (Variables|Default|GetLocationName) (Variables|Default|GetDesc)))
        (UserInterface|Viewport|AddtoViewport _returnvalue 0)
        (Actor|DestroyActor)))))

(fn ConstructionScript)