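; Quest giver component that offers its configured quest to the player on interaction or trigger entry.
; Interact asks the player's quest log component whether the quest is active; if not, it shows the quest and returns the owner's display name, otherwise an empty string.
; ShowQuest looks up the quest's data table row and passes its details and ID to a WB_QuestGiver widget added to the viewport.
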(event EventBeginPlay)

(event EventTick
  (params (DeltaSeconds :type Float%20%28single-precision%29)))

(fn ShowQuest
  (bind _questdata (Variables|Default|GetQuestData))
  (bind _returnvalue (Utilities|GetDataTableRow (.datatable _questdata) (.rowname _questdata))
    (:then
      (bind _returnvalue_2 (UserInterface|CreateWidget "/Game/UI/QuestUI/WB_QuestGiver.WB_QuestGiver_C" 0 _returnvalue (.rowname _questdata)))
      (UserInterface|Viewport|AddtoViewport _returnvalue_2 0))))

(fn TriggerEnter
  (CallFunction|Interact))

(fn Interact
  (if (not (Default|QueryActiveQuest (Variables|/Game/ThirdPerson/Blueprints/BP_ThirdPersonCharacter.BP_ThirdPersonCharacter_C|GetBPC_QuestLogComponent (CallFunction|GetMyPlayerCharacter)) (.rowname (Variables|Default|GetQuestData))))
    (CallFunction|ShowQuest)
    (return (Utilities|GetDisplayName (Components|GetOwner)))
    (else
      (return ""))))