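; BP_QuestBase is the base quest Blueprint that tracks one quest's staged objectives from start to completion.
; It loads its stages from a data table by QuestID and maps the current stage's objective IDs to progress counts.
; The player character's objective-ID event updates those counts, with increases limited to unfinished objectives.
; Completed objectives show a notification, finished stages load the next, and the last opens the quest complete widget.
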(event EventBeginPlay
  (CallFunction|GetQuestDetails)
  (EventDispatchers|BindEventtoOnObjectIDCalled (CallFunction|GetMyPlayerCharacter) (EventDispatchers|CreateEvent :!event OnObjectiveIDHeard)))

(fn ConstructionScript)

(fn OnObjectiveIDHeard
  (params (ObjectiveID :type String) (Value :type Integer))
  (bind _currentobjectiveprogress (Variables|Default|GetCurrentObjectiveProgress))
  (bind (_value _returnvalue) (Utilities|Map|Find _currentobjectiveprogress ObjectiveID))
  (if (> (Class|KismetMathLibrary|SignOfInteger Value) 0)
    (if _returnvalue
      (if (< _value (Utilities|Struct|BreakST_ObjectiveDetails (CallFunction|GetObjDatabyId ObjectiveID)))
        (Utilities|Map|Add (Variables|Default|GetCurrentObjectiveProgress) ObjectiveID (+ _value Value))
        (CallFunction|IsObjectiveComplete ObjectiveID)
        (Default|CallOnObjHeard)
        (return))
      (else
        (return)))
    (else
      (Utilities|Map|Add (Variables|Default|GetCurrentObjectiveProgress) ObjectiveID (+ (.Value (Utilities|Map|Find (Variables|Default|GetCurrentObjectiveProgress) ObjectiveID)) Value))
      (return))))

(fn GetQuestDetails
  (bind _returnvalue (Utilities|GetDataTableRow "/Game/Blueprints/GameSystems/QuestSystems/QuestData.QuestData" (Variables|Default|GetQuestID))
    (:then
      (bind _output_get (Variables|Default|SetQuestDetails _returnvalue))
      (bind _output_get_2 (Variables|Default|SetCurrentStageDetails (Utilities|Array|Get(acopy) (.Stages (Utilities|Struct|BreakST_QuestDetails _output_get)) (Variables|Default|GetCurrentStage))))
      (Utilities|Map|Clear (Variables|Default|GetCurrentObjectiveProgress))
      (for _array_element (.Objectives (Utilities|Struct|BreakST_StageDetails _output_get_2))
        (Utilities|Map|Add (Variables|Default|GetCurrentObjectiveProgress) (.ObjectiveID (Utilities|Struct|BreakST_ObjectiveDetails _array_element)) 0)))))

(fn GetObjDatabyId
  (params (ObjectiveID :type String))
  (for _array_element (.Objectives (Utilities|Struct|BreakST_StageDetails (Variables|Default|GetCurrentStageDetails)))
    (if (Utilities|Enum|Equal(Enum) (Utilities|Struct|BreakST_ObjectiveDetails _array_element) ObjectiveID)
      (return _array_element))))

(fn IsObjectiveComplete
  (params (ObjectiveID :type String))
  (bind _array_element (CallFunction|GetObjDatabyId ObjectiveID))
  (bind (_description _quantity) (Utilities|Struct|BreakST_ObjectiveDetails _array_element))
  (if (>= (.Value (Utilities|Map|Find (Variables|Default|GetCurrentObjectiveProgress) ObjectiveID)) _quantity)
    (bind _returnvalue (UserInterface|CreateWidget "/Game/UI/QuestUI/WB_QuestNotification.WB_QuestNotification_C" 0 _description))
    (UserInterface|Viewport|AddtoViewport _returnvalue 0)
    (bind _return (CallFunction|AreAllObjComplete))
    (if _return
      (bind _result (Math|Integer|IncrementInt (Variables|Default|GetCurrentStage))
        (:%20%20
          (if (Utilities|Array|IsValidIndex (.stages (Variables|Default|GetQuestDetails)) _result)
            (CallFunction|GetQuestDetails)
            (else
              (bind _output_get (Variables|Default|SetIsCompleted true))
              (if _output_get
                (Default|GetQuestActor (Variables|/Game/ThirdPerson/Blueprints/BP_ThirdPersonCharacter.BP_ThirdPersonCharacter_C|GetBPC_QuestLogComponent (CallFunction|GetMyPlayerCharacter)) (Variables|Default|GetQuestID))
                (CallFunction|DisplayRewards)))))))))

(fn AreAllObjComplete
  (for _array_element (.Objectives (Utilities|Struct|BreakST_StageDetails (Variables|Default|GetCurrentStageDetails)))
    (if (not (>= (.Value (Utilities|Map|Find (Variables|Default|GetCurrentObjectiveProgress) (.ObjectiveID (Utilities|Struct|BreakST_ObjectiveDetails _array_element)))) (.Quantity (Utilities|Struct|BreakST_ObjectiveDetails (CallFunction|GetObjDatabyId (.ObjectiveID (Utilities|Struct|BreakST_ObjectiveDetails _array_element)))))))
      (bind _output_get (LocalVariables|SetLocalAllComplete false))
      (return _output_get)))
  (return (LocalVariables|GetLocalAllComplete)))

(fn DisplayRewards
  (bind _returnvalue (UserInterface|CreateWidget "/Game/UI/QuestUI/WB_QuestComplete.WB_QuestComplete_C" 0 (Variables|Default|GetQuestDetails) (Variables|Default|GetQuestID)))
  (UserInterface|Viewport|AddtoViewport _returnvalue 0))