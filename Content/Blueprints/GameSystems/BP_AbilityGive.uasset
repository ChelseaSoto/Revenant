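; BP_AbilityGive is a pickup trigger that grants the player a configured set of abilities.
; When the player character overlaps its box, it writes the four ability flags (Laser, Time, Shock, Grapple) into the game instance's save data and saves to a fixed slot.
; It then updates the player HUD's ability visibility and destroys itself.
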(event OnComponentBeginOverlap(Box)
  (params (OverlappedComponent :type Primitive%20Component%20Object%20Reference) (OtherActor :type Actor%20Object%20Reference) (OtherComp :type Primitive%20Component%20Object%20Reference) (OtherBodyIndex :type Integer) (bFromSweep :type Boolean) (SweepResult :type Hit%20Result%20Structure%20%28by%20ref%29))
  (if (== OtherActor (Game|GetPlayerCharacter 0))
    (CallFunction|AbilityGive)))

(event Custom|AbilityGive
  (bind _asgi_my_game_instance (Utilities|Casting|CastToGI_MyGameInstance (Game|GetGameInstance)))
  (Default|ChangeAbilityDetails (Variables|/Game/Savegame/GI_MyGameInstance.GI_MyGameInstance_C|GetSaveData _asgi_my_game_instance) (Variables|Default|GetAbility%201) (Variables|Default|GetAbility%202) (Variables|Default|GetAbility%203) (Variables|Default|GetAbility%204))
  (SaveGame|SaveGametoSlot (Variables|/Game/Savegame/GI_MyGameInstance.GI_MyGameInstance_C|GetSaveData _asgi_my_game_instance) "slot1")
  (Default|SetAbilityVisible (Variables|/Game/ThirdPerson/Blueprints/BP_ThirdPersonCharacter.BP_ThirdPersonCharacter_C|GetPlayerHUD (CallFunction|GetMyPlayerCharacter)) (Variables|Default|GetAbility%201) (Variables|Default|GetAbility%202) (Variables|Default|GetAbility%203) (Variables|Default|GetAbility%204))
  (Actor|DestroyActor))

(fn ConstructionScript)