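; BP_CollectableDisplayUI is an interactable collectable actor that animates its model in the world until it is picked up.
; Tick spins CollectableModel around yaw at SpinSpeed, while a Timeline started on BeginPlay bobs it vertically through a lerp.
; Interact runs an Interact call, notifies the player character through CallOnObjectIDCalled with an empty ObjectiveID, then destroys the actor.
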(event EventTick
  (params (DeltaSeconds :type Float%20%28single-precision%29))
  ;[1 1 1] Spin the model
  (Transformation|AddLocalRotation (Variables|Default|GetCollectable%20Model) (Math|Rotator|MakeRotator 0.0 0.0 (* DeltaSeconds (Variables|Default|GetspinSpeed))) false false))

(event EventBeginPlay
  ;[1 1 1] Bob model up and down
  (bind _newtrack_1 (Timeline|Timeline Play)
    (:Update
      (Transformation|SetRelativeLocation (Variables|Default|GetCollectable%20Model) (Math|Vector|MakeVector 0.0 0.0 (Math|Float|Lerp 1e+01 -1e+01 _newtrack_1)) false false))))

(fn ConstructionScript)

(fn Interact
  (CallFunction|Interact)
  (Default|CallOnObjectIDCalled (CallFunction|GetMyPlayerCharacter) "" 1)
  (Actor|DestroyActor)
  (return ""))