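; Base collectable actor that the player interacts with to progress quest objectives.
; Player overlap shows an interact prompt widget, created with the player's gamepad state, and applies a highlight overlay material to the model, with both removed when overlap ends.
; Interact triggers the quest giver component, reports its objective ID to the player character, then destroys the actor.
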(event EventBeginPlay)

(event Collision|EventActorBeginOverlap
  (params (OtherActor :type Actor%20Object%20Reference))
  (bind _returnvalue (UserInterface|CreateWidget "/Game/UI/P_Interact.P_Interact_C" 0 (Variables|/Game/ThirdPerson/Blueprints/BP_ThirdPersonCharacter.BP_ThirdPersonCharacter_C|GetUsingGamepad (CallFunction|GetMyPlayerCharacter))))
  (if (== OtherActor (Game|GetPlayerCharacter 0))
    (UserInterface|Viewport|AddtoViewport _returnvalue 0)
    (Rendering|Material|SetOverlayMaterial (Variables|Default|GetCollectable%20Model) "/Game/Materials/M_OverlayMat.M_OverlayMat" :!class /Script/Engine.MeshComponent)))

(event Collision|EventActorEndOverlap
  (params (OtherActor :type Actor%20Object%20Reference))
  (if (== (Game|GetPlayerCharacter 0) OtherActor)
    (Widget|RemovefromParent (stale Collision|EventActorBeginOverlap _returnvalue))
    (Rendering|Material|SetOverlayMaterial (Variables|Default|GetCollectable%20Model) 0 :!class /Script/Engine.MeshComponent)))

(fn ConstructionScript)

(fn Interact
  (Default|Interact (Variables|Default|GetBPC_QuestGiver))
  (Default|CallOnObjectIDCalled (CallFunction|GetMyPlayerCharacter) (Variables|Default|GetObjectiveID) 1)
  (Actor|DestroyActor)
  (return ""))