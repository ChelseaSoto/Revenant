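; Actor that plays an assigned level sequence, either at level start or when the player pawn overlaps it.
; A Start flag plays the sequence on BeginPlay, with Loop selecting endless looping.
; The player's first overlap fires the Starting dispatcher, plays the sequence and binds its finish event to destroy the actor.
; The overlap path does not check Start, and only it binds that self-destruct.
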(event Custom|OnFinished_Event
  (Actor|DestroyActor))

(event EventBeginPlay
  (bind _sequence_to_play (Variables|Default|GetSequence%20To%20Play))
  (bind _sequenceplayer (Variables|/Script/LevelSequence.LevelSequenceActor|GetSequencePlayer _sequence_to_play))
  (if (Variables|Default|GetStart?)
    (if (Variables|Default|GetLoop?)
      (Class|MovieSceneSequencePlayer|PlayLooping _sequenceplayer -1)
      (else
        (Sequencer|Player|Play _sequenceplayer :!class /Script/MovieScene.MovieSceneSequencePlayer)))))

(event Collision|EventActorBeginOverlap
  (params (OtherActor :type Actor%20Object%20Reference))
  (bind _sequence_to_play (Variables|Default|GetSequence%20To%20Play))
  (bind _sequenceplayer (Variables|/Script/LevelSequence.LevelSequenceActor|GetSequencePlayer _sequence_to_play))
  (if (== OtherActor (Game|Player|GetPlayerPawn 0))
    (Utilities|FlowControl|DoOnce false
      (:Completed
        (Default|CallStarting)
        (Sequencer|Player|Play _sequenceplayer :!class /Script/MovieScene.MovieSceneSequencePlayer)
        (EventDispatchers|AssignOnFinished _sequenceplayer (delegate Custom|OnFinished_Event))))))

(fn ConstructionScript)