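; BP_AudioBase is a dialogue audio actor that plays a sequence of voice lines attached to the player character's mesh.
; StartDialouge reads the current numbered row of DT_ScriptAudio through GetDataInfo and spawns its sound.
; When the sound finishes, it increments the row, waits that line's delay and plays the next.
; The actor destroys itself on reaching RowEndBefore or a missing row.
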(event Custom|Start%20Dialouge
  (bind (_charater_names _dialouge_text _audiotoplay _delay_after_sound) (CallFunction|GetDataInfo))
  (bind _returnvalue (Audio|SpawnSoundAttached _audiotoplay (Variables|/Script/Engine.Character|GetMesh (Game|GetPlayerCharacter 0)) "None" "0, 0, 0" "0, 0, 0" "KeepRelativeOffset" false 1.0 1.0 0.0 0 0))
  (EventDispatchers|AssignOnAudioFinished _returnvalue (delegate Custom|Audio%20Done)))

(event Custom|Audio%20Done
  (bind _result (Math|Integer|IncrementInt (Variables|Default|GetRow%20Number))
    (:%20%20
      (Variables|Default|SetRow%20Number _result)
      (Utilities|FlowControl|Delay (stale Custom|Start%20Dialouge _delay_after_sound))
      (CallFunction|StartDialouge))))

(fn ConstructionScript)

(fn GetDataInfo
  (bind _row_number (Variables|Default|GetRow%20Number))
  (if (not (>= _row_number (Variables|Default|GetRow%20End%20Before)))
    (bind _returnvalue (Utilities|GetDataTableRow "/Game/Blueprints/GameSystems/DialogueSystem/DT_ScriptAudio.DT_ScriptAudio" (Utilities|String|StringToName (Utilities|String|ToString(Integer) _row_number)))
      (:then
        (return (.CharaterNames (Utilities|Struct|BreakS_DialougeAudio _returnvalue)) (.DialougeText (Utilities|Struct|BreakS_DialougeAudio _returnvalue)) (.AudioToPlay (Utilities|Struct|BreakS_DialougeAudio _returnvalue)) (.Delayaftersound (Utilities|Struct|BreakS_DialougeAudio _returnvalue))))
      (:RowNotFound
        _)))
  (Actor|DestroyActor))