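; BP_HeartVessel is an interactable pickup that counts toward an objective.
; A sphere overlap creates a gamepad-aware P_Interact prompt, shows it for the local player character and removes it when they leave.
; Interact fires the PickedUp dispatcher, destroys the actor and broadcasts its ObjectiveID with a value of 1 through the player character.
; The outline overlay material nodes are disconnected and never run.
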(event OnComponentBeginOverlap(Sphere)
  (params (OverlappedComponent :type Primitive%20Component%20Object%20Reference) (OtherActor :type Actor%20Object%20Reference) (OtherComp :type Primitive%20Component%20Object%20Reference) (OtherBodyIndex :type Integer) (bFromSweep :type Boolean) (SweepResult :type Hit%20Result%20Structure%20%28by%20ref%29))
  (bind _asbp_third_person_character (Utilities|Casting|CastToBP_ThirdPersonCharacter OtherActor))
  (bind _returnvalue (UserInterface|CreateWidget "/Game/UI/P_Interact.P_Interact_C" 0 (Variables|/Game/ThirdPerson/Blueprints/BP_ThirdPersonCharacter.BP_ThirdPersonCharacter_C|GetUsingGamepad _asbp_third_person_character)))
  (Variables|Default|SetInteractPrompt _returnvalue)
  (if (== OtherActor (Game|GetPlayerCharacter 0))
    (UserInterface|Viewport|AddtoViewport (Variables|Default|GetInteractPrompt) 0)))

(event OnComponentEndOverlap(Sphere)
  (params (OverlappedComponent :type Primitive%20Component%20Object%20Reference) (OtherActor :type Actor%20Object%20Reference) (OtherComp :type Primitive%20Component%20Object%20Reference) (OtherBodyIndex :type Integer))
  (if (== (Game|GetPlayerCharacter 0) OtherActor)
    (Widget|RemovefromParent (Variables|Default|GetInteractPrompt))))

(event EventBeginPlay)

(event Collision|EventActorBeginOverlap
  (params (OtherActor :type Actor%20Object%20Reference)))

(event EventTick
  (params (DeltaSeconds :type Float%20%28single-precision%29)))

(fn ConstructionScript)

(fn Interact
  (Default|CallPickedUp!)
  (Actor|DestroyActor)
  (Default|CallOnObjectIDCalled (CallFunction|GetMyPlayerCharacter) (Variables|Default|GetObjective%20ID) 1)
  (return ""))