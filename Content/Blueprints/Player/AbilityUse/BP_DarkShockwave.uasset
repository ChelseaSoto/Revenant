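; BP_DarkShockwave is a player ability actor that charges an expanding shockwave around its owner, then deals radial damage.
; On BeginPlay a looping timer calls Charge, which grows the area size each tick and draws a short-lived debug sphere as the only visual.
; At maximum size it clears the timer, applies radial damage at the owner's current location while ignoring the owner, and destroys itself.
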(event Custom|Charge
  (bind _actorowner (Variables|Default|GetActorOwner))
  (bind _output_get (Variables|Default|SetAoeSize (+ (Variables|Default|GetAoeSize) 5e+01)))
  (if (>= _output_get 5e+02)
    (Utilities|Time|ClearandInvalidateTimerbyHandle (stale EventBeginPlay _returnvalue))
    (Game|Damage|ApplyRadialDamage 1e+01 (Transformation|GetActorLocation _actorowner) 5e+02 "/Script/Engine.DamageType" (Utilities|Array|MakeArray _actorowner 0) _actorowner 0 false "ECC_Visibility")
    (Actor|DestroyActor)
    (else
      (Rendering|Debug|DrawDebugSphere (Transformation|GetActorLocation (Variables|Default|GetActorOwner)) _output_get 12 "(R=1.000000,G=0.047707,B=0.000000,A=1.000000)" 0.1))))

(event EventBeginPlay
  (bind _returnvalue (Utilities|Time|SetTimerbyEvent (delegate Custom|Charge) 0.1 true)))

(fn ConstructionScript)