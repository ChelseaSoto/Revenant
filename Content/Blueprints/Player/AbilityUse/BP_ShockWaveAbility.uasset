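; Player shockwave ability that charges a growing area around the character, then releases a radial blast.
; A looping timer, started on activation, grows the radius and previews it with debug spheres.
; At maximum size it stops, applies radial damage that ignores the player, and calls Broken on overlapped actors implementing BPI_Ability3.
; The size is never reset within this graph.
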(event Custom|Charge
  (bind _my_player_character (CallFunction|GetMyPlayerCharacter))
  (bind _returnvalue (Transformation|GetActorLocation _my_player_character))
  (bind _output_get (Variables|Default|SetAoeSize (+ (Variables|Default|GetAoeSize) 5e+01)))
  (if (>= _output_get 5e+02)
    (Utilities|Time|ClearandInvalidateTimerbyHandle (stale Ability|EventActivateAbility _returnvalue))
    (Game|Damage|ApplyRadialDamage 1e+01 _returnvalue 5e+02 "/Script/Engine.DamageType" (Utilities|Array|MakeArray _my_player_character 0) _my_player_character 0 false "ECC_Visibility")
    (bind _outactors (Collision|SphereOverlapActors _returnvalue 5e+02 (Variables|Default|GetObject%20Types) "/Script/Engine.Actor"))
    (for _array_element _outactors
      (if (Utilities|DoesObjectImplementInterface _array_element "/Game/Blueprints/Enviromental/BreakableLvl3/BPI_Ability3.BPI_Ability3_C")
        (bind _asbpi_ability_3 (Utilities|Casting|CastToBPI_Ability3 _array_element))
        (Default|Broken! _asbpi_ability_3)))
    (else
      (Rendering|Debug|DrawDebugSphere (Transformation|GetActorLocation (Game|GetPlayerCharacter 0)) _output_get 12 "(R=1.000000,G=0.047707,B=0.000000,A=1.000000)" 0.1))))

(event Ability|EventActivateAbility
  (bind _returnvalue (Utilities|Time|SetTimerbyEvent (delegate Custom|Charge) 0.1 true 0.4)))