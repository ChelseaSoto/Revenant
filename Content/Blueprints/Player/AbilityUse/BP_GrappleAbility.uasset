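; Player grapple ability that pulls the character toward whatever point the camera is aimed at.
; On activation it plays a sound and line-traces on the Camera channel from the ability spawn point along the camera's forward vector.
; A hit fires the hook visual, hops the character upward, then after a short delay launches it with velocity proportional to the offset to the hit.
; A miss resets the hook.
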(event Ability|EventActivateAbility
  (bind _my_player_character (CallFunction|GetMyPlayerCharacter))
  (bind _my_player_character_2 (CallFunction|GetMyPlayerCharacter))
  (bind _my_player_character_3 (CallFunction|GetMyPlayerCharacter))
  (bind _abilityspawn (Variables|/Game/ThirdPerson/Blueprints/BP_ThirdPersonCharacter.BP_ThirdPersonCharacter_C|GetAbilitySpawn _my_player_character))
  (bind _returnvalue (Transformation|GetWorldLocation _abilityspawn))
  (Audio|PlaySoundatLocation "/Game/Audio/SFX/PlayerAudio/Grapple/SQ_Grapple.SQ_Grapple" _returnvalue "0, 0, 0" 1.0 1.0 0.0 0 0 0 0)
  (bind (_outhit _returnvalue_2) (Collision|LineTraceByChannel _returnvalue (+ _returnvalue (* (Math|Vector|GetForwardVector (Variables|/Game/ThirdPerson/Blueprints/BP_ThirdPersonCharacter.BP_ThirdPersonCharacter_C|GetFollowCamera _my_player_character)) (Variables|Default|GetGrappleDistance))) "TraceTypeQuery2" false 0 "None"))
  (if _returnvalue_2
    (bind _output_get (Variables|Default|SetHitLocation (.Location (Collision|BreakHitResult _outhit))))
    (Default|GrappleHookVisualShoot _my_player_character_3 _output_get)
    (Character|LaunchCharacter _my_player_character_3 "0.000000,0.000000,700.000000" false true)
    (Utilities|FlowControl|Delay 0.2)
    (Character|LaunchCharacter _my_player_character_2 (* (- (Variables|Default|GetHitLocation) (Transformation|GetActorLocation _my_player_character_2)) (Variables|Default|GetLaunchForce)) false true)
    (else
      (Default|ResetGrappleHook (CallFunction|GetMyPlayerCharacter)))))