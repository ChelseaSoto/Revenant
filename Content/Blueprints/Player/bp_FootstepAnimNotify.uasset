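; Anim notify that plays surface-dependent footstep sounds at the owning actor's location during animations.
; On each notify, it line traces downward from the actor on the Visibility channel to read the physical surface underfoot.
; Gravel gets its own cue, while Stone and all other surfaces share a custom footstep cue.
; Volume scales in three tiers based on the owner's current speed.
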(fn ReceivedNotify
  (params (MeshComp :type Skeletal%20Mesh%20Component%20Object%20Reference) (Animation :type Anim%20Sequence%20Base%20Object%20Reference) (EventReference :type Anim%20Notify%20Event%20Reference%20Structure%20%28by%20ref%29))
  (bind _returnvalue (Components|GetOwner MeshComp))
  (bind _returnvalue_2 (Transformation|GetActorLocation _returnvalue))
  (LocalVariables|SetcurrentSpeed (Math|Vector|VectorLength (Transformation|GetVelocity _returnvalue)))
  (bind (_outhit _returnvalue_3) (Collision|LineTraceByChannel _returnvalue_2 (+ _returnvalue_2 (* (Transformation|GetActorUpVector _returnvalue) -2e+02)) "TraceTypeQuery1" false (Utilities|Array|MakeArray _returnvalue) "None" true "(R=1.000000,G=0.000000,B=0.000000,A=1.000000)" "(R=0.000000,G=1.000000,B=0.000000,A=1.000000)" 1.5))
  (if _returnvalue_3
    ;[1 1 1] Change the step volume based on how fast the player is moving
    (if (<= (LocalVariables|GetcurrentSpeed) 4.5e+02)
      (LocalVariables|SetstepVolume 0.25)
      (elif (>= (LocalVariables|GetcurrentSpeed) 6e+02)
        (LocalVariables|SetstepVolume 1.0)
        (else
          (LocalVariables|SetstepVolume 0.6))))
    ;[1 1 1] Change sound of footstep depending on pm being stepped on. To add more materials Edit->Project Settings->Search "Surface"->Add new material
    (switch Utilities|FlowControl|Switch|SwitchonEPhysicalSurface (Collision|GetSurfaceType _outhit)
      (:SurfaceType_Default
        (Audio|PlaySoundatLocation "/Game/Audio/FootStepCustom_Cue.FootStepCustom_Cue" _returnvalue_2 "0, 0, 0" (LocalVariables|GetstepVolume) 1.0 0.0 0 0 0 0))
      (:SurfaceType1
        (Audio|PlaySoundatLocation "/Game/Audio/FootStepCustom_Cue.FootStepCustom_Cue" _returnvalue_2 "0, 0, 0" (LocalVariables|GetstepVolume) 1.0 0.0 0 0 0 0))
      (:SurfaceType2
        (Audio|PlaySoundatLocation "/Game/Audio/gravelFootstepCue.gravelFootstepCue" _returnvalue_2 "0, 0, 0" (LocalVariables|GetstepVolume) 1.0 0.0 0 0 0 0))))
  (return false))