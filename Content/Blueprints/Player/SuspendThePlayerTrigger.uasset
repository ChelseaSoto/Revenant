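; Trigger actor that briefly freezes the player's movement when the player character overlaps it.
; On overlap it deactivates the CharacterMovement component of BP_ThirdPersonCharacter, waits for the Duration variable, then reactivates it.
; A DoOnce gate blocks re-triggering during the suspension and resets afterward, so the trigger can fire again.
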(event EventBeginPlay)

(event EventTick
  (params (DeltaSeconds :type Float%20%28single-precision%29)))

(event Collision|EventActorBeginOverlap
  (params (OtherActor :type Actor%20Object%20Reference))
  (if (== OtherActor (Game|GetPlayerCharacter 0))
    (Utilities|FlowControl|DoOnce false :!label _label
      (:Completed
        (bind _asbp_third_person_character (Utilities|Casting|CastToBP_ThirdPersonCharacter (Game|GetPlayerCharacter 0)))
        (Components|Activation|Deactivate (Variables|/Script/Engine.Character|GetCharacterMovement _asbp_third_person_character))
        (Utilities|FlowControl|Delay (Variables|Default|GetDuration))
        (Components|Activation|Activate (Variables|/Script/Engine.Character|GetCharacterMovement _asbp_third_person_character) false)
        (goto _label Reset)))))

(fn ConstructionScript)