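; BP_Dissolve is a volume Blueprint that feeds the position and size of its Cube to dissolve materials through the PC_Dissolve parameter collection.
; The construction script writes the Cube's world location and scale to the Location and Bounds parameters.
; At runtime it starts inactive; once MakeActive is called, Tick rewrites both parameters every frame and prints a debug "Hello".
; The collection is shared, so multiple instances overwrite each other's values.
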(event Custom|Make%20Active
  ;[1 1 1] Dissolve is disabled by default. When you want to use it give the other blueprint a child of it and have that child cast here and enable 'active' //Julian
  (Variables|Default|Setactive true))

(event EventBeginPlay
  ;[1 1 1] Dissolve is disabled by default. When you want to use it give the other blueprint a child of it and have that child cast here and enable 'active' //Julian
  (Variables|Default|Setactive false))

(event EventTick
  (params (DeltaSeconds :type Float%20%28single-precision%29))
  (bind _cube (Variables|Default|GetCube))
  ;[1 1 1] Dissolve is disabled by default. When you want to use it give the other blueprint a child of it and have that child cast here and enable 'active' //Julian
  (if (Variables|Default|Getactive)
    (Rendering|Material|SetVectorParameterValue "/Game/VFX/ShadersandMaterials/DissolveAssets/PC_Dissolve.PC_Dissolve" "Location" (Math|Conversions|ToLinearColor(Vector) (Transformation|GetWorldLocation _cube)) :!class /Script/Engine.KismetMaterialLibrary)
    (Rendering|Material|SetVectorParameterValue "/Game/VFX/ShadersandMaterials/DissolveAssets/PC_Dissolve.PC_Dissolve" "Bounds" (Math|Conversions|ToLinearColor(Vector) (Transformation|GetWorldScale _cube)) :!class /Script/Engine.KismetMaterialLibrary)
    (Development|PrintString "Hello")))

(fn ConstructionScript
  (bind _cube (Variables|Default|GetCube))
  (Rendering|Material|SetVectorParameterValue "/Game/VFX/ShadersandMaterials/DissolveAssets/PC_Dissolve.PC_Dissolve" "Location" (Math|Conversions|ToLinearColor(Vector) (Transformation|GetWorldLocation _cube)) :!class /Script/Engine.KismetMaterialLibrary)
  (Rendering|Material|SetVectorParameterValue "/Game/VFX/ShadersandMaterials/DissolveAssets/PC_Dissolve.PC_Dissolve" "Bounds" (Math|Conversions|ToLinearColor(Vector) (Transformation|GetWorldScale _cube)) :!class /Script/Engine.KismetMaterialLibrary))