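; Actor component that manages a character's locomotion gait, starting in a default gait on BeginPlay.
; UpdateGait records the last and current gait, then sends the new one to the mesh's anim instance through ReciveGaitDataMessage.
; If that call returns true, it copies the gait's GaitSettings entry onto the owner's CharacterMovementComponent, setting speed, acceleration and braking behavior.
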(event EventBeginPlay
  (CallFunction|UpdateGait "NewEnumerator1"))

(fn UpdateGait
  (params (Desired%20Gait :type E_Gait%20Enum :default "NewEnumerator0"))
  (bind _returnvalue (Components|GetOwner))
  (bind _gait_settings (Variables|Default|GetGait%20Settings))
  (bind _value (Utilities|Map|Find _gait_settings Desired%20Gait))
  (bind _returnvalue_2 (Actor|GetComponentbyClass _returnvalue "/Script/Engine.CharacterMovementComponent"))
  (bind (_movementspeed _maxacceleration _brakingdecleration _brakingfrictionfactor _useseperatebreakingfriction _brakingfriction) (Utilities|Struct|BreakSC_GaitSettings _value))
  (Variables|Default|SetLast%20Gait (Variables|Default|GetCurrent%20Gait))
  (Variables|Default|SetCurrent%20Gait Desired%20Gait)
  (bind _success_ (Class|BPIGaitData|ReciveGaitData(Message) (CallFunction|GetAnimInstance) Desired%20Gait))
  (if _success_
    (Variables|/Script/Engine.CharacterMovementComponent|SetMaxWalkSpeed _returnvalue_2 _movementspeed)
    (Variables|/Script/Engine.CharacterMovementComponent|SetMaxAcceleration _returnvalue_2 _maxacceleration)
    (Variables|/Script/Engine.CharacterMovementComponent|SetBrakingDecelerationWalking _returnvalue_2 _brakingdecleration)
    (Variables|/Script/Engine.CharacterMovementComponent|SetBrakingFrictionFactor _returnvalue_2 _brakingfrictionfactor)
    (Variables|/Script/Engine.CharacterMovementComponent|SetbUseSeparateBrakingFriction _returnvalue_2 _useseperatebreakingfriction)
    (Variables|/Script/Engine.CharacterMovementComponent|SetBrakingFriction _returnvalue_2 _brakingfriction)))

(fn GetAnimInstance
  (return (Components|SkeletalMesh|GetAnimInstance (Variables|/Script/Engine.Character|GetMesh (.AsCharacter (Utilities|Casting|CastToCharacter (Components|GetOwner)))))))