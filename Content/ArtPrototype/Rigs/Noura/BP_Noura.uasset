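; BP_Noura is the interactable Noura character, offering either dialogue or a hug with the player.
; A sphere overlap shows a widget, removed on exit or interaction.
; The hug hides the sword, locks input, snaps the player to an Arrow and plays a montage until a notify restores both and calls Fade.
; Dialogue completion also calls Fade, a FlipFlop timeline driving a material parameter, then unhides a linked actor.
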(event OnComponentBeginOverlap(Sphere)
  (params (OverlappedComponent :type Primitive%20Component%20Object%20Reference) (OtherActor :type Actor%20Object%20Reference) (OtherComp :type Primitive%20Component%20Object%20Reference) (OtherBodyIndex :type Integer) (bFromSweep :type Boolean) (SweepResult :type Hit%20Result%20Structure%20%28by%20ref%29))
  (bind _returnvalue (Game|GetPlayerCharacter 0))
  (bind _returnvalue_2 (== OtherActor _returnvalue))
  (if _returnvalue_2
    (bind _returnvalue_3 (UserInterface|CreateWidget (Variables|Default|GetClass)))
    (Variables|Default|SetNewVar _returnvalue_3)
    (if _returnvalue_2
      (UserInterface|Viewport|AddtoViewport (Variables|Default|GetNewVar) 0))))

(event OnComponentEndOverlap(Sphere)
  (params (OverlappedComponent :type Primitive%20Component%20Object%20Reference) (OtherActor :type Actor%20Object%20Reference) (OtherComp :type Primitive%20Component%20Object%20Reference) (OtherBodyIndex :type Integer))
  (if (== (Game|GetPlayerCharacter 0) OtherActor)
    (Widget|RemovefromParent (Variables|Default|GetNewVar))))

(event Custom|HAHA
  (Widget|RemovefromParent (Variables|Default|GetNewVar)))

(event Custom|Fade
  (Utilities|FlowControl|FlipFlop
    (:A
      (bind _newtrack_0 (Timeline|Timeline PlayFromStart)
        (:Update
          (Rendering|Material|SetScalarParameterValueonMaterials (Variables|Default|GetNoura) "Text" _newtrack_0))))
    (:B
      (Timeline|Timeline Reverse))))

(event Custom|Bind
  (params (Binding :type WB%20Dialogue%20Base%20Object%20Reference))
  (EventDispatchers|BindEventtoFinished Binding (delegate Custom|Dialouge%20Ended)))

(event Custom|Dialouge%20Ended
  (CallFunction|Fade)
  (Rendering|SetActorHiddenInGame (Variables|Default|GetActorToUnhide) false))

(event Custom|HUG!
  (bind _my_player_character (CallFunction|GetMyPlayerCharacter))
  (Rendering|SetActorHiddenInGame (Variables|/Game/ThirdPerson/Blueprints/BP_ThirdPersonCharacter.BP_ThirdPersonCharacter_C|GetSwordReference _my_player_character) true)
  (Input|DisableInput _my_player_character (Game|GetPlayerController 0))
  (|MovePlayertocorrectLocation _my_player_character)
  (Animation|Montage|PlayMontage (Variables|/Script/Engine.Character|GetMesh _my_player_character) "/Game/ArtPrototype/Rigs/Hossam/Animations/New/AM_Hug.AM_Hug"
    (:OnNotifyBegin
      (Input|EnableInput _my_player_character (Game|GetPlayerController 0))
      (Rendering|SetActorHiddenInGame (Variables|/Game/ThirdPerson/Blueprints/BP_ThirdPersonCharacter.BP_ThirdPersonCharacter_C|GetSwordReference _my_player_character) false)
      (CallFunction|Fade))))

(event EventBeginPlay
  (EventDispatchers|BindEventtoInteract! (delegate Custom|HAHA)))

(event Collision|EventActorBeginOverlap
  (params (OtherActor :type Actor%20Object%20Reference)))

(event EventTick
  (params (DeltaSeconds :type Float%20%28single-precision%29)))

(fn ConstructionScript)

(fn Interact
  (Default|CallInteract!)
  (if (Variables|Default|GetHasDialouge?)
    (bind _returnvalue (Default|ActivateDialouge (Variables|Default|GetDialouge)))
    (bind _output_get (Variables|Default|SetBind%20to%20event _returnvalue))
    (CallFunction|Bind _output_get)
    (else
      (CallFunction|HUG!)))
  (return ""))